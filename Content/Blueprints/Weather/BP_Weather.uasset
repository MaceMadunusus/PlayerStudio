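; BP_Weather is a day-night sky actor with sun, moon, stars, particle clouds, a calendar and an optional clock/compass widget.
; Construction scales timeline play rates by global speed, seeks them to TimeOfDay and scatters clouds within bounds.
; Four timelines drive light rotation and intensity, sky dome material colors and skylight recapture.
; The sun timeline's playback position becomes clock time, its New Day event advances the date, and day count steps moon phases.
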(fn ConstructionScript
  (CallFunction|ConstructorWidget)
  (CallFunction|SetSpeed)
  (CallFunction|ConstructorSkyDome)
  (CallFunction|ConstructorMoon)
  (Transformation|SetWorldRotation (Variables|Default|GetCompassRoseSM) (Math|Rotator|MakeRotator 0.0 (Variables|Global|GetGlobalAngle) 0.0) false)
  (CallFunction|ConstructTL (Variables|Default|GetSunTL) (Variables|Default|GetSpeed) (Variables|Global|GetTimeOfDay) false)
  (CallFunction|ConstructTL (Variables|Default|GetUpdaterTL) (Variables|Default|GetSpeed) (Variables|Global|GetTimeOfDay) true)
  (CallFunction|ConstructTL (Variables|Default|GetMoonTL) (Variables|Default|GetSpeed) (Variables|Global|GetTimeOfDay) false)
  (CallFunction|ConstructTL (Variables|Default|GetSkyTL) (Variables|Default|GetSpeed) (Variables|Global|GetTimeOfDay) true)
  (CallFunction|UpdateMoonPhaseMaterial)
  (CallFunction|ConstructClouds))

(fn ConstructTL
  (params (TL :type Timeline%20Component%20Object%20Reference) (Speed :type Float%20%28single-precision%29) (Position :type Float%20%28single-precision%29) (FireEvents :type Boolean))
  (Components|Timeline|SetPlayRate TL Speed)
  (Components|Timeline|SetPlaybackPosition TL Position FireEvents))

(fn DayCounter
  ;[1 1 1] Checking if day is equal to last day of month
  (if (== (Variables|Calendar|GetDays) (Utilities|Array|Get(acopy) (Variables|Calendar|GetCollectionDaysPerMonth) (- (Variables|Calendar|GetMonth) 1)))
    (Variables|Calendar|SetDays 1)
    ;[1 1 1] Checking if month will be reset
    (if (== (Variables|Calendar|GetMonth) 12)
      (Variables|Calendar|SetMonth 1)
      ;[1 1 1] Change Year
      (Variables|Calendar|SetYear (+ (Variables|Calendar|GetYear) 1))
      (else
        ;[1 1 1] Change Month
        (Variables|Calendar|SetMonth (+ (Variables|Calendar|GetMonth) 1))))
    (else
      ;[1 1 1] Change day
      (Variables|Calendar|SetDays (+ (Variables|Calendar|GetDays) 1)))))

(fn UpdateClock
  ;[1 1 1] UpdateTimeOfDay
  (Variables|Global|SetTimeOfDay (Components|Timeline|GetPlaybackPosition (Variables|Default|GetSunTL)))
  ;[1 1 1] Set Hour
  (Variables|Clock|SetHours (Math|Float|Floor (Variables|Global|GetTimeOfDay)))
  ;[1 1 1] Set Minutes
  (Variables|Clock|SetMinutes (Math|Float|Floor (* 60 (- (Variables|Global|GetTimeOfDay) (Math|Conversions|ToFloat(Integer) (Math|Float|Floor (Variables|Global|GetTimeOfDay)))))))
  ;[1 1 1] Set Seconds
  (Variables|Clock|SetSeconds (Math|Float|Floor (* 60 (- (* 60 (- (Variables|Global|GetTimeOfDay) (Math|Conversions|ToFloat(Integer) (Math|Float|Floor (Variables|Global|GetTimeOfDay))))) (Math|Conversions|ToFloat(Integer) (Math|Float|Floor (* 60 (- (Variables|Global|GetTimeOfDay) (Math|Conversions|ToFloat(Integer) (Math|Float|Floor (Variables|Global|GetTimeOfDay)))))))))))
  (CallFunction|UpdateClockPointers)
  (return))

(fn SetSpeed
  (Variables|Default|SetSpeed (* (Variables|Global|GetGlobalSpeed) 0.00027))
  (return))

(fn ConstructorSkyDome
  (bind _returnvalue (Rendering|Material|CreateDynamicMaterialInstance (Variables|Default|GetSkydomeSM) 0 "/Game/BluePrints/Weather/Material/M_Sky_Inst.M_Sky_Inst" :!class /Script/Engine.PrimitiveComponent))
  (Variables|Default|SetSkyDomeMaterial _returnvalue)
  (Rendering|Material|SetScalarParameterValue (Variables|Default|GetSkyDomeMaterial) "StarsRotationSpeed" (Variables|Default|GetSpeed) :!class /Script/Engine.MaterialInstanceDynamic)
  (return))

(fn UpdateMoonPhaseMaterial
  (Rendering|Material|SetScalarParameterValue (Variables|Default|GetMoonMaterial) "MoonPhase" (Math|Conversions|ToFloat(Integer) (Variables|Moon|GetMoonPhase)) :!class /Script/Engine.MaterialInstanceDynamic)
  (if (Variables|Global|GetShowWidget)
    (Rendering|Material|SetScalarParameterValue (Variables|Default|GetMoonMaterial) "MoonPhase" (Math|Conversions|ToFloat(Integer) (Variables|Moon|GetMoonPhase)) :!class /Script/Engine.MaterialInstanceDynamic))
  (return))

(fn UpdateSunDisk
  (Rendering|Material|SetVectorParameterValue (Variables|Default|GetSkyDomeMaterial) "SunDirection" (Math|Conversions|ToLinearColor(Vector) (Math|Vector|GetForwardVector (Variables|Default|GetSunLight))) :!class /Script/Engine.MaterialInstanceDynamic)
  (return ""))

(fn UpdateStars
  (params (StarsBrighness :type Float%20%28single-precision%29))
  (Rendering|Material|SetScalarParameterValue (Variables|Default|GetSkyDomeMaterial) "StarBrighness" (* StarsBrighness (Variables|Sky|GetStarBrighness)) :!class /Script/Engine.MaterialInstanceDynamic)
  (return))

(fn UpdateSkyColor
  (params (SkyBrighness :type Float%20%28single-precision%29) (SunCorona :type Linear%20Color%20Structure) (Zenith%20Color :type Linear%20Color%20Structure) (Horizon%20Color :type Linear%20Color%20Structure))
  (bind _skydomematerial (Variables|Default|GetSkyDomeMaterial))
  (Rendering|Material|SetVectorParameterValue _skydomematerial "Zenith" Zenith%20Color :!class /Script/Engine.MaterialInstanceDynamic)
  (Rendering|Material|SetVectorParameterValue _skydomematerial "Horizon" Horizon%20Color :!class /Script/Engine.MaterialInstanceDynamic)
  (Rendering|Material|SetVectorParameterValue _skydomematerial "SunCorona" SunCorona :!class /Script/Engine.MaterialInstanceDynamic)
  (Rendering|Components|Light|SetIntensity (Variables|Default|GetSkyLight) (* SkyBrighness (Variables|Sky|GetSkyLightMultiplier)))
  (return))

(fn ClockFormat
  (params (In :type Integer) (Append%20:? :type Boolean))
  (bind _returnvalue (Utilities|String|ToString(Integer) In))
  (bind _returnvalue_2 (Utilities|String|Len _returnvalue))
  (bind _returnvalue_3 (Utilities|String|Append "0" _returnvalue))
  (bind _returnvalue_4 (== _returnvalue_2 1))
  (bind _returnvalue_5 (Utilities|String|SelectString _returnvalue_3 _returnvalue _returnvalue_4))
  (return (Utilities|String|SelectString (Utilities|String|Append _returnvalue_5 ":") _returnvalue_5 Append%20:?)))

(fn ClocktoString
  (return (Utilities|String|Append (Utilities|String|Append (CallFunction|ClockFormat (Variables|Clock|GetHours) true) (CallFunction|ClockFormat (Variables|Clock|GetMinutes) true)) (CallFunction|ClockFormat (Variables|Clock|GetSeconds) false))))

(fn UpdateClockPointers
  (if (Variables|Global|GetShowWidget)
    (Transformation|SetRelativeRotation (Variables|Default|GetHourSM) (Math|Rotator|MakeRotator 0.0 (* (Variables|Global|GetTimeOfDay) 3e+01) 0.0) false)
    (Transformation|SetRelativeRotation (Variables|Default|GetMinuteSM) (Math|Rotator|MakeRotator 0.0 (Math|Conversions|ToFloat(Integer) (* (Variables|Clock|GetMinutes) 6)) 0.0) false)
    (Transformation|SetRelativeRotation (Variables|Default|GetSecondSM) (Math|Rotator|MakeRotator 0.0 (Math|Conversions|ToFloat(Integer) (* (Variables|Clock|GetSeconds) 6)) 0.0) false))
  (return))

(fn ConstructorWidget
  (Rendering|SetVisibility (Variables|Default|GetSecondSM) (Variables|Global|GetShowWidget) false)
  (return))

(fn UpdateSunWidget
  (if (Variables|Global|GetShowWidget)
    (Transformation|SetRelativeRotation (Variables|Default|GetSunIconSM) (Variables|/Script/Engine.SceneComponent|GetRelativeRotation (Variables|Default|GetSunContainer)) false))
  (return))

(fn UpdateMoonPhase
  (if (== (Math|Integer|%(Integer) (Variables|Calendar|GetDays) (Variables|Moon|GetPerDayMoonPhases)) 0)
    (Variables|Moon|SetMoonPhase (+ (Variables|Moon|GetMoonPhase) 1))
    (if (> (Variables|Moon|GetMoonPhase) 7)
      (Variables|Moon|SetMoonPhase 0)))
  (return))

(fn UpdateMoonWidget
  (if (Variables|Global|GetShowWidget)
    (Transformation|SetRelativeRotation (Variables|Default|GetMoonIconSM) (Variables|/Script/Engine.SceneComponent|GetRelativeRotation (Variables|Default|GetMoonSM)) false))
  (return))

(fn UpdateMoonRotation
  (params (Rotation :type Float%20%28single-precision%29))
  (Transformation|SetRelativeRotation (Variables|Default|GetMoonSM) (Math|Rotator|MakeRotator (Variables|Moon|GetMoonLongitude) 9e+01 (+ Rotation 1.8e+02)) false)
  (return))

(fn UpdateSunRotation
  (params (Rotation :type Float%20%28single-precision%29))
  (Transformation|SetRelativeRotation (Variables|Default|GetSunContainer) (Math|Rotator|MakeRotator (Variables|Sun|GetSunLongitude) 9e+01 Rotation) false)
  (return))

(fn UpdateSunBrighness
  (params (NewBrightness :type Float%20%28single-precision%29))
  (bind _sunlightmultiplier (Variables|Sun|GetSunLightMultiplier))
  (bind _returnvalue (* NewBrightness _sunlightmultiplier))
  (Rendering|Components|Light|SetIntensity (Variables|Default|GetSunLight) _returnvalue)
  (Rendering|Components|Light|SetCastShadows (Variables|Default|GetSunLight) (>= _returnvalue 0.0))
  (return))

(fn ConstructorMoon
  (bind _returnvalue (Rendering|Material|CreateDynamicMaterialInstance (Variables|Default|GetMoonSM) 0 "/Game/BluePrints/Weather/Material/M_Moon_Inst.M_Moon_Inst" :!class /Script/Engine.PrimitiveComponent))
  (Variables|Default|SetMoonMaterial _returnvalue)
  (Rendering|Material|SetMaterial (Variables|Default|GetMoonIconSM) 0 (Variables|Default|GetMoonMaterial))
  (return))

(fn UpdateMoonDisk
  (Rendering|Material|SetVectorParameterValue (Variables|Default|GetSkyDomeMaterial) "MoonDirection" (Math|Conversions|ToLinearColor(Vector) (Math|Vector|GetUpVector (Variables|Default|GetMoonSM))) :!class /Script/Engine.MaterialInstanceDynamic)
  (return ""))

(fn AddClouds
  (bind _basestream (Variables|Clouds|GetBaseStream))
  (bind _cloudsmaxbounds (Variables|Clouds|GetCloudsMaxBounds))
  (bind _returnvalue (AddComponent|AddParticleSystemComponent true (Math|Transform|MakeTransform (Math|Vector|MakeVector (Math|Random|RandomFloatinRangefromStream (* (.x _cloudsmaxbounds) -1.0) (.x _cloudsmaxbounds) _basestream) (Math|Random|RandomFloatinRangefromStream (* (.y _cloudsmaxbounds) -1.0) (.y _cloudsmaxbounds) _basestream) (Math|Random|RandomFloatinRangefromStream (.z _cloudsmaxbounds) (+ (.z _cloudsmaxbounds) (Variables|Clouds|GetCloudsVariationOffsetZ)) _basestream)) "0, 0, 0" "1,1,1")))
  (Class|SceneComponent|Attachto _returnvalue 0 "None" "KeepRelativeOffset" true)
  (Utilities|Array|Add (Variables|Default|GetCollectionClouds) _returnvalue)
  (CallFunction|UpdateCloudParameters _returnvalue))

(fn ConstructClouds
  (for _index (range 1 (Variables|Clouds|GetMaxClouds))
    (CallFunction|AddClouds)
    (return))
  (return))

(fn UpdateCloudParameters
  (params (Particle :type Particle%20System%20Component%20Object%20Reference))
  (bind _cloudspeed (Variables|Clouds|GetCloudSpeed))
  (LocalVariables|Set_Particle Particle)
  (Effects|Components|ParticleSystem|SetFloatParameter (LocalVariables|Get_Particle) "Scale" (Variables|Clouds|GetCloudScale))
  (Effects|Components|ParticleSystem|SetFloatParameter (LocalVariables|Get_Particle) "LifeTime" (Variables|Clouds|GetCloudLifeTime))
  (Effects|Components|ParticleSystem|SetFloatParameter (LocalVariables|Get_Particle) "Density" (Variables|Clouds|GetCloudDensity))
  (Effects|Components|ParticleSystem|SetVectorParameter (LocalVariables|Get_Particle) "Direction" (* (Variables|Clouds|GetCloudDirection) (Math|Random|RandomFloatinRange (/ _cloudspeed 2.0) _cloudspeed)))
  (bind _returnvalue (Rendering|Material|CreateDynamicMaterialInstance (LocalVariables|Get_Particle) 0 0 :!class /Script/Engine.PrimitiveComponent))
  (LocalVariables|Set_CloudMaterial _returnvalue)
  (Rendering|Material|SetScalarParameterValue (LocalVariables|Get_CloudMaterial) "Opacity" (Variables|Clouds|GetCloudOpacity) :!class /Script/Engine.MaterialInstanceDynamic)
  (Rendering|Material|SetScalarParameterValue (LocalVariables|Get_CloudMaterial) "Color" (Variables|Clouds|GetCloudBrighness) :!class /Script/Engine.MaterialInstanceDynamic)
  (return))

(fn UpdateMoonBrighness
  (params (MoonBrighness :type Float%20%28single-precision%29))
  (bind _moonlightmultiplier (Variables|Moon|GetMoonLightMultiplier))
  (bind _returnvalue (* MoonBrighness _moonlightmultiplier))
  (Rendering|Components|Light|SetIntensity (Variables|Default|GetMoonLight) _returnvalue)
  (Rendering|Components|Light|SetCastShadows (Variables|Default|GetMoonLight) (>= _returnvalue 0.0))
  (return))