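; Light tower actor with two spotlights and an emissive mesh that share a switchable, recolorable light.
; Construction creates a dynamic material instance and applies the configured color and on/off state to spotlights and material.
; While something overlaps the Area component, left click sets a random color and right click resets it to white.
; The LightsOn/Off event toggles spotlight visibility and the material's Bloom.
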(event OnComponentBeginOverlap(Area)
  (params (OtherActor :type Actor%20Object%20Reference) (OtherComp :type Primitive%20Component%20Object%20Reference) (OtherBodyIndex :type Integer))
  (Variables|Default|SetMouse%20Over true))

(event OnComponentEndOverlap(Area)
  (params (OtherActor :type Actor%20Object%20Reference) (OtherComp :type Primitive%20Component%20Object%20Reference) (OtherBodyIndex :type Integer))
  (Variables|Default|SetMouse%20Over false))

(event Custom|Lights%20On/Off
  (params (Lights%20Enabled :type Boolean))
  (bind _bloom (Variables|Default|GetBloom))
  (bind _light_tower_dynamic_material (Variables|Default|GetLight%20Tower%20Dynamic%20Material))
  (Variables|Default|SetLights%20Enabled Lights%20Enabled)
  (Rendering|SetVisibility (Variables|Default|GetSpotLight13) (Variables|Default|GetLights%20Enabled) false)
  (if (Variables|Default|GetLights%20Enabled)
    (Rendering|Material|SetScalarParameterValue _light_tower_dynamic_material _bloom 1e+02 :!class /Script/Engine.MaterialInstanceDynamic)
    (else
      (Rendering|Material|SetScalarParameterValue _light_tower_dynamic_material _bloom 0.0 :!class /Script/Engine.MaterialInstanceDynamic))))

(event Input|MouseEvents|RightMouseButton
  (:Pressed
    (if (Variables|Default|GetMouse%20Over)
      (Variables|Default|SetLight%20Color "(R=1.000000,G=1.000000,B=1.000000,A=1.000000)")
      (Rendering|Components|Light|SetLightColor (Variables|Default|GetSpotLight13) (Variables|Default|GetLight%20Color))
      (Rendering|Material|SetVectorParameterValue (Variables|Default|GetLight%20Tower%20Dynamic%20Material) "Color" (Variables|Default|GetLight%20Color) :!class /Script/Engine.MaterialInstanceDynamic))))

(event Input|MouseEvents|LeftMouseButton
  (:Pressed
    (if (Variables|Default|GetMouse%20Over)
      (Variables|Default|SetLight%20Color (Math|Conversions|ToLinearColor(Vector) (Math|Random|RandomUnitVector)))
      (Rendering|Components|Light|SetLightColor (Variables|Default|GetSpotLight13) (Variables|Default|GetLight%20Color))
      (Rendering|Material|SetVectorParameterValue (Variables|Default|GetLight%20Tower%20Dynamic%20Material) "Color" (Variables|Default|GetLight%20Color) :!class /Script/Engine.MaterialInstanceDynamic))))

(fn ConstructionScript
  (bind _lights_enabled (Variables|Default|GetLights%20Enabled))
  (bind _bloom (Variables|Default|GetBloom))
  (bind _light_color (Variables|Default|GetLight%20Color))
  (bind _spotlight14 (Variables|Default|GetSpotLight14))
  (bind _returnvalue (Rendering|Material|CreateDynamicMaterialInstance "/Game/PlanetSide_2/World/Materials/LightTower_Inst.LightTower_Inst" :!class /Script/Engine.KismetMaterialLibrary))
  (Variables|Default|SetLight%20Tower%20Dynamic%20Material _returnvalue)
  (Rendering|Material|SetMaterial (Variables|Default|GetLightTower) 0 (Variables|Default|GetLight%20Tower%20Dynamic%20Material))
  (Rendering|SetVisibility _spotlight14 _lights_enabled false)
  (Rendering|Components|Light|SetLightColor _spotlight14 _light_color)
  (Rendering|Material|SetVectorParameterValue (Variables|Default|GetLight%20Tower%20Dynamic%20Material) (Variables|Default|GetColor) _light_color :!class /Script/Engine.MaterialInstanceDynamic)
  (if _lights_enabled
    (Rendering|Material|SetScalarParameterValue (Variables|Default|GetLight%20Tower%20Dynamic%20Material) _bloom 1e+02 :!class /Script/Engine.MaterialInstanceDynamic)
    (else
      (Rendering|Material|SetScalarParameterValue (Variables|Default|GetLight%20Tower%20Dynamic%20Material) _bloom 0.0 :!class /Script/Engine.MaterialInstanceDynamic))))