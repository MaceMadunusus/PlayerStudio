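; Magrider vehicle Blueprint that configures its primary and secondary weapon appearance at construction time.
; The construction script applies the selected static meshes for both weapons.
; It rotates the Weapon component on roll by the negated primary rotation value and the TopWeapon component on yaw by the secondary rotation value.
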(fn ConstructionScript
  (Components|StaticMesh|SetStaticMesh (Variables|Weapons|GetPrimary%20Weapon))
  (Transformation|SetRelativeRotation (Variables|Default|GetWeapon) (Class|KismetMathLibrary|MakeRot 0.0 0.0 (* (Variables|Weapons|GetPrimary%20Weapon%20Rotation) -1.0)) false)
  (Components|StaticMesh|SetStaticMesh (Variables|Weapons|GetSecondary%20Weapon))
  (Transformation|SetRelativeRotation (Variables|Default|GetTop%20Weapon) (Class|KismetMathLibrary|MakeRot 0.0 (Variables|Weapons|GetSecondary%20Weapon%20Rotation) 0.0) false))