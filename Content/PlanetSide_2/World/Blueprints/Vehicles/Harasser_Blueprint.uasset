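; Harasser vehicle Blueprint from a PlanetSide 2 project that assembles a customizable vehicle in its construction script.
; Exposed meshes and toggles set the weapon, cosmetic attachments, composite armor and an optional decal.
; Lumifiber gets a dynamic material for color and bloom, while light settings drive light components and the four faction materials (TR, VS, NC, NS).
; A camouflage texture, tiling and color branch exists but is disconnected, so it never runs.
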(fn ConstructionScript
  (bind _headlights_on_off (Variables|Lights|GetHeadlights%20On/Off))
  (bind _headlight_4 (Variables|Lights|GetHeadlight%204))
  (bind _bumper_mesh (Variables|Cosmetics|GetBumper%20Mesh))
  (bind _windshield_mesh (Variables|Cosmetics|GetWindshield%20Mesh))
  (bind _tirespikes_mesh (Variables|Cosmetics|GetTirespikes%20Mesh))
  (bind _hubcaps_mesh (Variables|Cosmetics|GetHubcaps%20Mesh))
  (bind _headlight_color (Variables|Lights|GetHeadlight%20Color))
  (bind _tr_material (Variables|FactionColors|GetTR%20Material))
  (bind _taillight_1 (Variables|Lights|GetTaillight%201))
  (bind _underglow_light (Variables|Lights|GetUnderglow%20Light))
  (bind _hood_ornament_mesh (Variables|Cosmetics|GetHood%20Ornament%20Mesh))
  (bind _lumifiber_mesh (Variables|Cosmetics|GetLumifiber%20Mesh))
  (bind _bloom (Variables|Lights|GetBloom))
  (Utilities|FlowControl|Sequence
    (:then_1
      ;[1 1 1] Weapon
      (Components|StaticMesh|SetStaticMesh (Variables|Weapon|GetWeapon%20Mesh) (Variables|Weapon|GetWeapon)))
    (:then_2
      (Utilities|FlowControl|Sequence
        (:then_0
          ;[1 1 1] Bumper
          (Rendering|SetVisibility _bumper_mesh (Variables|Cosmetics|GetBumper%20On/Off) false)
          (Components|StaticMesh|SetStaticMesh _bumper_mesh (Variables|Cosmetics|GetBumper)))
        (:then_1
          ;[1 1 1] Windshield
          (Rendering|SetVisibility _windshield_mesh (Variables|Cosmetics|GetWindshield%20On/Off) false)
          (Components|StaticMesh|SetStaticMesh _windshield_mesh (Variables|Cosmetics|GetWindshield)))
        (:then_2
          ;[1 1 1] Tirespikes
          (Rendering|SetVisibility _tirespikes_mesh (Variables|Cosmetics|GetTirespikes%20On/Off) false)
          (Components|StaticMesh|SetStaticMesh _tirespikes_mesh (Variables|Cosmetics|GetTirespikes)))
        (:then_3
          ;[1 1 1] Hubcaps
          (Rendering|SetVisibility _hubcaps_mesh (Variables|Cosmetics|GetHubcaps%20On/Off) false)
          (Components|StaticMesh|SetStaticMesh _hubcaps_mesh (Variables|Cosmetics|GetHubcaps)))
        (:then_4
          ;[1 1 1] Hood Ornaments
          (Rendering|SetVisibility _hood_ornament_mesh (Variables|Cosmetics|GetHood%20Ornament%20On/Off) false)
          (Components|StaticMesh|SetStaticMesh _hood_ornament_mesh (Variables|Cosmetics|GetHood%20Ornament)))
        (:then_5
          ;[1 1 1] Decal
          (if (Variables|Decal|GetDecal%20On/Off)
            (bind _returnvalue (AddComponent|AddDecalComponent false))
            (Rendering|Components|Decal|SetDecalMaterial _returnvalue (Variables|Decal|GetDecal))))
        (:then_6
          ;[1 1 1] Lumifiber
          (Rendering|SetVisibility _lumifiber_mesh (Variables|Cosmetics|GetLumifiber%20On/Off) false)
          (Components|StaticMesh|SetStaticMesh _lumifiber_mesh (Variables|Cosmetics|GetLumifiber))
          (bind _returnvalue_2 (Rendering|Material|CreateDynamicMaterialInstance "/Game/PlanetSide_2/Vehicles/Harasser/Attachments/Lumifiber/Lumifiber_C_Inst.Lumifiber_C_Inst" :!class /Script/Engine.KismetMaterialLibrary))
          (Rendering|Material|SetMaterial _lumifiber_mesh 0 _returnvalue_2)
          (Rendering|Material|SetVectorParameterValue _returnvalue_2 (Variables|Cosmetics|GetLumifiber%20Color%20Variable) (Variables|Cosmetics|GetLumifiber%20Color) :!class /Script/Engine.MaterialInstanceDynamic)
          (Rendering|Material|SetScalarParameterValue _returnvalue_2 (Variables|Lights|GetBloom) (Variables|Cosmetics|GetLumifiber%20Bloom%20Intensity) :!class /Script/Engine.MaterialInstanceDynamic))))
    (:then_3
      ;[1 1 1] Lights
      (Utilities|FlowControl|Sequence
        (:then_0
          (Rendering|SetVisibility _headlight_4 _headlights_on_off false)
          (Rendering|Components|Light|SetLightColor _headlight_4 _headlight_color)
          (Rendering|Material|SetVectorParameterValue _tr_material (Variables|Lights|GetLight%20Color) _headlight_color :!class /Script/Engine.MaterialInstanceDynamic)
          (if _headlights_on_off
            (Rendering|Material|SetScalarParameterValue _tr_material _bloom (Variables|Lights|GetBloom%20Intensity) :!class /Script/Engine.MaterialInstanceDynamic)
            (else
              (Rendering|Material|SetScalarParameterValue _tr_material _bloom 0.0 :!class /Script/Engine.MaterialInstanceDynamic))))
        (:then_1
          (Rendering|SetVisibility _taillight_1 (Variables|Lights|GetTaillights%20On/Off) false)
          (Rendering|Components|Light|SetLightColor _taillight_1 (Variables|Lights|GetTaillight%20Color)))
        (:then_2
          (Rendering|SetVisibility _underglow_light (Variables|Lights|GetChassis%20Light%20On/Off) false)
          (Rendering|Components|Light|SetLightColor _underglow_light (Variables|Lights|GetUnderglow%20Light%20Color)))))
    (:then_4
      ;[1 1 1] Composite Armor
      (Rendering|SetVisibility (Variables|Gameplay|GetComposite%20Armor) (Variables|Gameplay|GetComposite%20Armor%20On/Off) false))))