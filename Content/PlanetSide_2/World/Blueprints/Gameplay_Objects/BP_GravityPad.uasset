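; Gravity pad world object with Up and Down variants; this Blueprint handles its visuals and audio, with no movement logic in its graphs.
; The construction script sizes the sound trigger box from Height, then sets the mesh, material, light color and arrow billboard by GravityPadType.
; It also shows the matching particle component and destroys the opposite one.
; Overlapping LiftSoundArea activates the looping lift audio, and ending overlap deactivates it.
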(event OnComponentBeginOverlap(LiftSoundArea)
  (params (OtherActor :type Actor%20Object%20Reference) (OtherComp :type Primitive%20Component%20Object%20Reference) (OtherBodyIndex :type Integer) (bFromSweep :type Boolean) (SweepResult :type Hit%20Result%20Structure%20%28by%20ref%29))
  (Components|Activation|Activate (Variables|Sound|GetGravity%20Lift%20Audio%20Loop) false))

(event OnComponentEndOverlap(LiftSoundArea)
  (params (OtherActor :type Actor%20Object%20Reference) (OtherComp :type Primitive%20Component%20Object%20Reference) (OtherBodyIndex :type Integer))
  (Components|Activation|Deactivate (Variables|Sound|GetGravity%20Lift%20Audio%20Loop)))

(fn ConstructionScript
  (bind _returnvalue (Math|Transform|MakeTransform "0, 0,140.000000"))
  (bind _lift_sound_area (Variables|Default|GetLift%20Sound%20Area))
  (bind _height (Variables|GravityPad|GetHeight))
  (bind _gravity_pad (Variables|Meshes|GetGravity%20Pad))
  (bind _gravity_pad_particles_up (Variables|Particles|GetGravity%20Pad%20Particles%20Up))
  (bind _gravity_pad_particles_down (Variables|Particles|GetGravity%20Pad%20Particles%20Down))
  (bind _light (Variables|Default|GetLight))
  (Transformation|SetRelativeLocation _lift_sound_area (Math|Vector|MakeVector 0.0 0.0 (+ _height 13.0)) false false)
  (Components|Box|SetBoxExtent _lift_sound_area (Math|Vector|MakeVector 115.0 115.0 _height) true)
  (switch Utilities|FlowControl|Switch|SwitchonGravityPad (Variables|GravityPad|GetGravity%20Pad%20Type)
    (:NewEnumerator0
      (Components|StaticMesh|SetStaticMesh _gravity_pad "/Game/PlanetSide_2/World/Meshes/Gameplay/JumpPad3.JumpPad3")
      (Rendering|Material|SetMaterial _gravity_pad 0 "/Game/PlanetSide_2/World/Materials/Gameplay_Objects/MI_GravityPads_Up.MI_GravityPads_Up")
      (Rendering|SetVisibility _gravity_pad_particles_up true false)
      (Components|DestroyComponent _gravity_pad_particles_down)
      (Rendering|Components|Light|SetLightColor _light "(R=1.000000,G=0.800000,B=0.000000,A=1.000000)" true)
      (Components|DestroyComponent)
      (bind _returnvalue_2 (AddComponent|AddMaterialBillboardComponent false _returnvalue))
      (Variables|Default|SetArrow _returnvalue_2))
    (:NewEnumerator1
      (Components|StaticMesh|SetStaticMesh _gravity_pad "/Game/PlanetSide_2/World/Meshes/Gameplay/JumpPad2.JumpPad2")
      (Rendering|Material|SetMaterial _gravity_pad 0 "/Game/PlanetSide_2/World/Materials/Gameplay_Objects/MI_GravityPads_Down.MI_GravityPads_Down")
      (Components|DestroyComponent _gravity_pad_particles_up)
      (Rendering|SetVisibility _gravity_pad_particles_down true false)
      (Rendering|Components|Light|SetLightColor _light "(R=0.000000,G=0.491777,B=1.000000,A=1.000000)" true)
      (Components|DestroyComponent)
      (bind _returnvalue_3 (AddComponent|AddMaterialBillboardComponent false _returnvalue))
      (Variables|Default|SetArrow _returnvalue_3))))