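; Interactive Tempest Tower actor whose color the player changes through a UI widget while standing nearby.
; An overlap sphere creates the widget once, enables input and mouse-over events, and exit tears that down.
; Hovering toggles a custom-depth highlight, and clicking in range flip-flops the centered widget and cursor input mode.
; Construction and SetTempestTowerColor apply the color to a dynamic material, point light and resource-gather particles.
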(event OnComponentBeginOverlap(Sphere)
  (params (OtherActor :type Actor%20Object%20Reference) (OtherComp :type Primitive%20Component%20Object%20Reference) (OtherBodyIndex :type Integer) (bFromSweep :type Boolean) (SweepResult :type Hit%20Result%20Structure%20%28by%20ref%29))
  (bind _returnvalue (Game|GetPlayerController 0))
  (bind (_sizex _sizey) (HUD|GetViewportSize _returnvalue))
  (Utilities|FlowControl|Sequence
    (:then_0
      (Utilities|FlowControl|DoOnce false
        (:Completed
          (bind _returnvalue_2 (UserInterface|CreateWidget "/Game/PlanetSide_2/UI/TempestTower.TempestTower_C" _returnvalue self))
          (bind _output_get (Variables|Default|SetTempestTowerUI _returnvalue_2))
          (Class|UserWidget|SetPositioninViewport _output_get (Math|Vector2D|MakeVector2D (Math|Conversions|ToFloat(Integer) (- (/ _sizex 2) 150)) (Math|Conversions|ToFloat(Integer) (- (/ _sizey 2) 100))) true)
          (Class|Border|SetBrush (Variables|/Game/PlanetSide_2/UI/TempestTower.TempestTower_C|GetColorBox (Variables|Default|GetTempestTowerUI)) (Utilities|Struct|MakeSlateBrush "(X=32.000000,Y=32.000000)" "Image" "(Left=0.000000,Top=0.000000,Right=0.000000,Bottom=0.000000)" (Utilities|Struct|MakeSlateColor (Variables|Default|GetDefault%20Color)) "NoTile" "NoMirror" 0)))))
    (:then_1
      (Variables|Default|SetIsInRange true)
      (Input|EnableInput _returnvalue)
      (Variables|/Script/Engine.PlayerController|SetbEnableMouseOverEvents _returnvalue true))))

(event OnComponentEndOverlap(Sphere)
  (params (OtherActor :type Actor%20Object%20Reference) (OtherComp :type Primitive%20Component%20Object%20Reference) (OtherBodyIndex :type Integer))
  (bind _returnvalue (Game|GetPlayerController 0))
  (Variables|Default|SetIsInRange false)
  (Widget|RemovefromParent (Variables|Default|GetTempestTowerUI))
  (Input|DisableInput _returnvalue)
  (Variables|/Script/Engine.PlayerController|SetbShowMouseCursor _returnvalue false)
  (Variables|/Script/Engine.PlayerController|SetbEnableMouseOverEvents _returnvalue false)
  (Input|SetInputModeGameOnly _returnvalue)
  (Rendering|SetRenderCustomDepth (Variables|Default|GetTempestTower) false))

(event OnBeginCursorOver(TempestTower)
  (params (TouchedComponent :type Primitive%20Component%20Object%20Reference))
  (Rendering|SetRenderCustomDepth (Variables|Default|GetTempestTower) true))

(event OnEndCursorOver(TempestTower)
  (params (TouchedComponent :type Primitive%20Component%20Object%20Reference))
  (Rendering|SetRenderCustomDepth (Variables|Default|GetTempestTower) false))

(event OnClicked(TempestTower)
  (params (TouchedComponent :type Primitive%20Component%20Object%20Reference))
  (bind _returnvalue (Game|GetPlayerController 0))
  (bind _tempesttowerui (Variables|Default|GetTempestTowerUI))
  (Utilities|FlowControl|FlipFlop
    (:A
      (if (Variables|Default|GetIsInRange)
        (UserInterface|Viewport|AddtoViewport _tempesttowerui 0)
        (Variables|/Script/Engine.PlayerController|SetbShowMouseCursor _returnvalue true)
        (Input|SetInputModeGameandUI _returnvalue (Variables|Default|GetTempestTowerUI) true false)))
    (:B
      (Widget|RemovefromParent _tempesttowerui)
      (Variables|/Script/Engine.PlayerController|SetbShowMouseCursor _returnvalue false)
      (Input|SetInputModeGameOnly _returnvalue))))

(event Custom|Set%20Tempest%20Tower%20Color
  (bind _tempesttowerui (Variables|Default|GetTempestTowerUI))
  (bind _p_resourcegather (Variables|Default|GetP_ResourceGather))
  (bind _outgoingcolor (Variables|/Game/PlanetSide_2/UI/TempestTower.TempestTower_C|GetOutgoingColor _tempesttowerui))
  (Rendering|Material|SetVectorParameterValue (Variables|Default|GetTempestTowerMaterial) "Color" _outgoingcolor :!class /Script/Engine.MaterialInstanceDynamic)
  (Rendering|Components|Light|SetLightColor (Variables|Default|GetPointLight) _outgoingcolor true)
  (Effects|Components|ParticleSystem|SetColorParameter _p_resourcegather "ColorOverLife" _outgoingcolor)
  (Effects|Components|ParticleSystem|SetColorParameter _p_resourcegather "ColorOverLife2" _outgoingcolor))

(fn ConstructionScript
  (bind _tempesttower (Variables|Default|GetTempestTower))
  (bind _default_color (Variables|Default|GetDefault%20Color))
  (bind _p_resourcegather (Variables|Default|GetP_ResourceGather))
  (bind _returnvalue (Rendering|Material|CreateDynamicMaterialInstance _tempesttower 0 (Rendering|Material|GetMaterial _tempesttower 0) :!class /Script/Engine.PrimitiveComponent))
  (bind _output_get (Variables|Default|SetTempestTowerMaterial _returnvalue))
  (Rendering|Material|SetVectorParameterValue _output_get "Color" _default_color :!class /Script/Engine.MaterialInstanceDynamic)
  (Rendering|Components|Light|SetLightColor (Variables|Default|GetPointLight) _default_color true)
  (Effects|Components|ParticleSystem|SetColorParameter _p_resourcegather "ColorOverLife" _default_color)
  (Effects|Components|ParticleSystem|SetColorParameter _p_resourcegather "ColorOverLife2" _default_color))