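; Faction-themed jump pad with a landing target, where a faction switch event swaps the pad mesh and light color.
; The construction script places the landing pad and yaws the actor from the direction toward it.
; Functions compute a ballistic launch vector and instanced trajectory markers, but their calls are disconnected.
; Trigger overlap only plays a launch sound at world origin, with no launch applied here.
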(event OnComponentBeginOverlap(JumpTrigger)
  (params (OtherActor :type Actor%20Object%20Reference) (OtherComp :type Primitive%20Component%20Object%20Reference) (OtherBodyIndex :type Integer) (bFromSweep :type Boolean) (SweepResult :type Hit%20Result%20Structure%20%28by%20ref%29))
  (Audio|PlaySoundatLocation "/Game/PlanetSide_2/Audio/INT_THRUSTPAD_2D_LAUNCH_01.INT_THRUSTPAD_2D_LAUNCH_01" "0, 0, 0"))

(event Custom|Faction%20Switch
  (params (Faction%20Name :type Name :default "None"))
  (bind _light (Variables|Default|GetLight))
  (bind _jumppad (Variables|Default|GetJumpPad))
  (switch name Faction%20Name
    (:NS
      (Components|StaticMesh|SetStaticMesh _jumppad "/Game/PlanetSide_2/World/Meshes/Gameplay/JumpPad_NC.JumpPad_NC")
      (Rendering|Components|Light|SetLightColor _light "(R=1.000000,G=1.000000,B=1.000000,A=1.000000)"))
    (:NC
      (Components|StaticMesh|SetStaticMesh _jumppad "/Game/PlanetSide_2/World/Meshes/Gameplay/JumpPad_NC.JumpPad_NC")
      (Rendering|Components|Light|SetLightColor _light "(R=0.100000,G=0.100000,B=1.000000,A=1.000000)"))
    (:TR
      (Components|StaticMesh|SetStaticMesh _jumppad "/Game/PlanetSide_2/World/Meshes/Gameplay/JumpPad_TR.JumpPad_TR")
      (Rendering|Components|Light|SetLightColor _light "(R=1.000000,G=0.000000,B=0.000000,A=1.000000)"))
    (:VS
      (Components|StaticMesh|SetStaticMesh _jumppad "/Game/PlanetSide_2/World/Meshes/Gameplay/JumpPad_VS.JumpPad_VS")
      (Rendering|Components|Light|SetLightColor _light "(R=0.637439,G=0.000000,B=1.000000,A=1.000000)"))))

(fn ConstructionScript
  (Transformation|SetRelativeLocation (Variables|Default|GetLandingPad) (Variables|Default|GetLanding%20Position) false)
  (Transformation|SetWorldRotation (Class|KismetMathLibrary|MakeRot 0.0 (.Yaw (Class|KismetMathLibrary|BreakRot (Math|Rotator|CombineRotators (Math|Rotator|FindLookatRotation (Transformation|GetWorldLocation (Variables|Default|GetJumpPad)) (Transformation|GetWorldLocation (Variables|Default|GetLandingPad))) "0,90.000000, 0"))) 0.0) false))

(fn DrawTrajectory
  (bind _launch_vector (Variables|Default|GetLaunch%20Vector))
  (bind (_x _y _z) (Math|Vector|BreakVector _launch_vector))
  (if (Variables|Default|GetShow%20Trajectory)
    (for _index (range 1 (Variables|Default|GetMarker%20Amount))
      (bind _output_get (Variables|Default|SetLoop%20Time (* _index (Variables|Default|GetMarker%20Distance))))
      (bind _position (CallFunction|GetPositionatATime _launch_vector _output_get))
      (if (== (Math|Integer|%(Integer) (Math|Float|Floor _output_get) 2) 0)
        _
        (else
          _))
      (Components|InstancedStaticMesh|AddInstance (Math|Transform|MakeTransform (+ _position (Transformation|GetWorldLocation (Variables|Default|GetJumpPad))) (Math|Rotator|MakeRotfromX (Math|Vector|MakeVector _x _y (- _z (* (Variables|Default|GetLoop%20Time) (Variables|Default|GetGravity%20Z))))))))))

(fn GetPositionatATime
  (params (Launch%20Vector :type Vector :default "0, 0, 0") (Time :type Float%20%28single-precision%29 :default 0.0))
  (bind (_x _y _z) (Math|Vector|BreakVector Launch%20Vector))
  (bind _returnvalue (Math|Vector2D|MakeVector2D _x _y))
  (bind _returnvalue_2 (* _returnvalue Time))
  (bind (_x_2 _y_2) (Math|Vector2D|BreakVector2D _returnvalue_2))
  (return (Math|Vector|MakeVector _x_2 _y_2 (- (* _z Time) (* (Math|Float|Power Time 2.0) (/ (Variables|Default|GetGravity%20Z) 2.0))))))

(fn SetLaunchVector
  (bind _returnvalue (Transformation|GetWorldLocation))
  (bind _landing_position (Variables|Default|GetLanding%20Position))
  (bind _gravity_z (Variables|Default|GetGravity%20Z))
  (bind (_x _y _z) (Math|Vector|BreakVector _returnvalue))
  (bind (_x_2 _y_2 _z_2) (Math|Vector|BreakVector _landing_position))
  (bind _returnvalue_2 (Math|Vector2D|MakeVector2D _x _y))
  (bind _returnvalue_3 (Math|Vector2D|MakeVector2D _x_2 _y_2))
  (bind _returnvalue_4 (- _z_2 _z))
  (bind _returnvalue_5 (- _returnvalue_3 _returnvalue_2))
  (bind _returnvalue_6 (* _gravity_z _returnvalue_4 2.0))
  (bind _returnvalue_7 (Math|Float|Sqrt _returnvalue_6))
  (bind _returnvalue_8 (/ _gravity_z _returnvalue_7))
  (bind _returnvalue_9 (/ _returnvalue_5 _returnvalue_8))
  (bind (_x_3 _y_3) (Math|Vector2D|BreakVector2D _returnvalue_9))
  (Variables|Default|SetLaunch%20Vector (Math|Vector|MakeVector _x_3 _y_3 _returnvalue_7)))