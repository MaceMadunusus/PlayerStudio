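; Console Blueprint for a gameplay terminal, configured by ConsoleType (equipment, vehicle classes or warpgate) and skinned per faction.
; The construction script reveals the matching icon and applies the neutral NS screen material and default light color.
; The FactionSwitch event reskins the console and recolors its light for NS, NC, TR or VS.
; Both paths share ConsoleTypeSelect, which takes one material per type and sets the matching one on material slot 1.
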(event Custom|Faction%20Switch
  (params (Faction%20Name :type Name))
  (switch name Faction%20Name
    (:NS
      (Utilities|FlowControl|Sequence
        (:then_0
          (Utilities|ConsoleTypeSelect "/Game/PlanetSide_2/World/Materials/Gameplay_Objects/Console/Console_NS3.Console_NS3" "/Game/PlanetSide_2/World/Materials/Gameplay_Objects/Console/Console_NS6.Console_NS6" "/Game/PlanetSide_2/World/Materials/Gameplay_Objects/Console/Console_NS5.Console_NS5" "/Game/PlanetSide_2/World/Materials/Gameplay_Objects/Console/Console_NS4.Console_NS4" "/Game/PlanetSide_2/World/Materials/Gameplay_Objects/Console/Console_NS7.Console_NS7" "/Game/PlanetSide_2/World/Materials/Gameplay_Objects/Console/Console_NS1.Console_NS1" "/Game/PlanetSide_2/World/Materials/Gameplay_Objects/Console/Console_NS2.Console_NS2" "/Game/PlanetSide_2/World/Materials/Gameplay_Objects/Console/Console_NS8.Console_NS8"))
        (:then_1
          (Rendering|Components|Light|SetLightColor (Variables|Default|GetLight) (Variables|Default|GetLight%20Color)))))
    (:NC
      (Utilities|FlowControl|Sequence
        (:then_0
          (Utilities|ConsoleTypeSelect "/Game/PlanetSide_2/World/Materials/Gameplay_Objects/Console/Console_NC3.Console_NC3" "/Game/PlanetSide_2/World/Materials/Gameplay_Objects/Console/Console_NC6.Console_NC6" "/Game/PlanetSide_2/World/Materials/Gameplay_Objects/Console/Console_NC5.Console_NC5" "/Game/PlanetSide_2/World/Materials/Gameplay_Objects/Console/Console_NC4.Console_NC4" "/Game/PlanetSide_2/World/Materials/Gameplay_Objects/Console/Console_NC7.Console_NC7" "/Game/PlanetSide_2/World/Materials/Gameplay_Objects/Console/Console_NC1.Console_NC1" "/Game/PlanetSide_2/World/Materials/Gameplay_Objects/Console/Console_NC2.Console_NC2" "/Game/PlanetSide_2/World/Materials/Gameplay_Objects/Console/Console_NC8.Console_NC8"))
        (:then_1
          (Rendering|Components|Light|SetLightColor (Variables|Default|GetLight) (Variables|Default|GetLight%20Color%20NC)))))
    (:TR
      (Utilities|FlowControl|Sequence
        (:then_0
          (Utilities|ConsoleTypeSelect "/Game/PlanetSide_2/World/Materials/Gameplay_Objects/Console/Console_TR3.Console_TR3" "/Game/PlanetSide_2/World/Materials/Gameplay_Objects/Console/Console_TR6.Console_TR6" "/Game/PlanetSide_2/World/Materials/Gameplay_Objects/Console/Console_TR5.Console_TR5" "/Game/PlanetSide_2/World/Materials/Gameplay_Objects/Console/Console_TR4.Console_TR4" "/Game/PlanetSide_2/World/Materials/Gameplay_Objects/Console/Console_TR7.Console_TR7" "/Game/PlanetSide_2/World/Materials/Gameplay_Objects/Console/Console_TR1.Console_TR1" "/Game/PlanetSide_2/World/Materials/Gameplay_Objects/Console/Console_TR2.Console_TR2" "/Game/PlanetSide_2/World/Materials/Gameplay_Objects/Console/Console_TR8.Console_TR8"))
        (:then_1
          (Rendering|Components|Light|SetLightColor (Variables|Default|GetLight) (Variables|Default|GetLight%20Color%20TR)))))
    (:VS
      (Utilities|FlowControl|Sequence
        (:then_0
          (Utilities|ConsoleTypeSelect "/Game/PlanetSide_2/World/Materials/Gameplay_Objects/Console/Console_VS3.Console_VS3" "/Game/PlanetSide_2/World/Materials/Gameplay_Objects/Console/Console_VS6.Console_VS6" "/Game/PlanetSide_2/World/Materials/Gameplay_Objects/Console/Console_VS5.Console_VS5" "/Game/PlanetSide_2/World/Materials/Gameplay_Objects/Console/Console_VS4.Console_VS4" "/Game/PlanetSide_2/World/Materials/Gameplay_Objects/Console/Console_VS7.Console_VS7" "/Game/PlanetSide_2/World/Materials/Gameplay_Objects/Console/Console_VS1.Console_VS1" "/Game/PlanetSide_2/World/Materials/Gameplay_Objects/Console/Console_VS2.Console_VS2" "/Game/PlanetSide_2/World/Materials/Gameplay_Objects/Console/Console_VS8.Console_VS8"))
        (:then_1
          (Rendering|Components|Light|SetLightColor (Variables|Default|GetLight) (Variables|Default|GetLight%20Color%20VS)))))))

(fn ConstructionScript
  (Utilities|FlowControl|Sequence
    (:then_0
      (switch Utilities|FlowControl|Switch|SwitchonConsoleType (Variables|Default|GetConsole%20Type)
        (:NewEnumerator0
          (Rendering|SetVisibility (Variables|Icon|GetIcon%20Infantry) true false))
        (:NewEnumerator1
          (Rendering|SetVisibility (Variables|Icon|GetIcon%20Flash) true false))
        (:NewEnumerator2
          (Rendering|SetVisibility (Variables|Icon|GetIcon%20Lightning) true false))
        (:NewEnumerator3
          (Rendering|SetVisibility (Variables|Icon|GetIcon%20Vehicle) true false))
        (:NewEnumerator4
          (Rendering|SetVisibility (Variables|Icon|GetIcon%20Sunderer) true false))
        (:NewEnumerator5
          (Rendering|SetVisibility (Variables|Icon|GetIcon%20Aircraft) true false))
        (:NewEnumerator6
          (Rendering|SetVisibility (Variables|Icon|GetIcon%20Galaxy) true false))
        (:NewEnumerator8
          (Rendering|SetVisibility (Variables|Icon|GetIcon%20Warpgate) true false))))
    (:then_1
      (Utilities|ConsoleTypeSelect "/Game/PlanetSide_2/World/Materials/Gameplay_Objects/Console/Console_NS3.Console_NS3" "/Game/PlanetSide_2/World/Materials/Gameplay_Objects/Console/Console_NS6.Console_NS6" "/Game/PlanetSide_2/World/Materials/Gameplay_Objects/Console/Console_NS5.Console_NS5" "/Game/PlanetSide_2/World/Materials/Gameplay_Objects/Console/Console_NS4.Console_NS4" "/Game/PlanetSide_2/World/Materials/Gameplay_Objects/Console/Console_NS7.Console_NS7" "/Game/PlanetSide_2/World/Materials/Gameplay_Objects/Console/Console_NS1.Console_NS1" "/Game/PlanetSide_2/World/Materials/Gameplay_Objects/Console/Console_NS2.Console_NS2" "/Game/PlanetSide_2/World/Materials/Gameplay_Objects/Console/Console_NS8.Console_NS8"))
    (:then_2
      (Rendering|Components|Light|SetLightColor (Variables|Default|GetLight) (Variables|Default|GetLight%20Color)))))