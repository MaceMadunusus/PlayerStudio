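; Capturable generator objective that players overload, stabilize or repair by standing in separate trigger volumes, with delayed checks confirming presence.
; An overload escalates through three timed stages of materials, lights, sounds and particles to destruction unless stabilized; stabilizing or repairing restores the idle look.
; Destruction and repair toggle linked lights through calls, while the shield branch is empty.
; The construction script shows a shield icon per GeneratorType.
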(event OnComponentBeginOverlap(HackingAOE)
  (params (OtherActor :type Actor%20Object%20Reference) (OtherComp :type Primitive%20Component%20Object%20Reference) (OtherBodyIndex :type Integer))
  ;[1 1 1] Generator Triggers
  (Variables|Default|SetHacking true)
  (CallFunction|GeneratorEvent)
  (if (not (Variables|Default|GetHacked))
    (Development|PrintString "Overloading" true true "(R=0.000000,G=1.000000,B=0.000000,A=1.000000)")))

(event OnComponentEndOverlap(HackingAOE)
  (params (OtherActor :type Actor%20Object%20Reference) (OtherComp :type Primitive%20Component%20Object%20Reference) (OtherBodyIndex :type Integer))
  ;[1 1 1] Generator Triggers
  (Variables|Default|SetHacking false))

(event OnComponentBeginOverlap(RepairAOE)
  (params (OtherActor :type Actor%20Object%20Reference) (OtherComp :type Primitive%20Component%20Object%20Reference) (OtherBodyIndex :type Integer))
  ;[1 1 1] Generator Triggers
  (Variables|Default|SetRepairing true)
  (CallFunction|GeneratorEvent)
  (if (Variables|Default|GetIs%20Destroyed)
    (Development|PrintString "Repairing" true true "(R=0.000000,G=1.000000,B=0.000000,A=1.000000)")))

(event OnComponentEndOverlap(RepairAOE)
  (params (OtherActor :type Actor%20Object%20Reference) (OtherComp :type Primitive%20Component%20Object%20Reference) (OtherBodyIndex :type Integer))
  ;[1 1 1] Generator Triggers
  (Variables|Default|SetRepairing false))

(event OnComponentBeginOverlap(StabilizingAOE)
  (params (OtherActor :type Actor%20Object%20Reference) (OtherComp :type Primitive%20Component%20Object%20Reference) (OtherBodyIndex :type Integer))
  ;[1 1 1] Generator Triggers
  (Variables|Default|SetStabilizing true)
  (CallFunction|GeneratorEvent)
  (if (not (Variables|Default|GetIs%20Destroyed))
    (if (Variables|Default|GetHacked)
      (Development|PrintString "Stabilizing" true true "(R=0.000000,G=1.000000,B=0.000000,A=1.000000)"))))

(event OnComponentEndOverlap(StabilizingAOE)
  (params (OtherActor :type Actor%20Object%20Reference) (OtherComp :type Primitive%20Component%20Object%20Reference) (OtherBodyIndex :type Integer))
  ;[1 1 1] Generator Triggers
  (Variables|Default|SetStabilizing false))

(event Custom|Generator%20Event
  (bind _light (Variables|Default|GetLight))
  (bind _light_2 (Variables|Default|GetLight))
  (bind _light_3 (Variables|Default|GetLight))
  (bind _light_4 (Variables|Default|GetLight))
  (if (Variables|Default|GetIs%20Destroyed)
    ;[1 1 1] Repair
    (Utilities|FlowControl|Delay 8.0)
    (if (Variables|Default|GetRepairing)
      (Variables|Default|SetRepaired true)
      (Variables|Default|SetIs%20Destroyed false)
      (Variables|Default|SetHacked false)
      (Audio|PlaySoundatLocation "/Game/PlanetSide_2/Audio/Computer/GENERATOR_REPAIRED_Cue.GENERATOR_REPAIRED_Cue" "0, 0, 0")
      (Development|PrintString "Generator Repaired" true true "(R=0.000000,G=0.714328,B=1.000000,A=1.000000)")
      (CallFunction|GeneratorEnable)
      ;[1 1 1] Generator REset
      (Rendering|SetVisibility _light_4 true true :!label _label)
      (Rendering|SetVisibility (Variables|Default|GetDestroyed%20Generator) false true)
      (Rendering|Components|Light|SetLightFunctionMaterial _light_4 "/Game/PlanetSide_2/World/Materials/LightFunction/Generator_Light_Inst.Generator_Light_Inst")
      (Rendering|Components|Light|SetLightColor _light_4 "(R=0.690000,G=0.690000,B=1.000000,A=1.000000)")
      (Rendering|Material|SetMaterial (Variables|Default|GetGenerator) 0 "/Game/PlanetSide_2/World/Materials/Gameplay_Objects/Generator_Inst.Generator_Inst")
      (Audio|Components|Audio|Stop (Variables|Default|GetOverload%201%20Loop))
      (Audio|Components|Audio|Play (Variables|Default|GetIdle%20Loop) 0.0))
    (elif (Variables|Default|GetHacked)
      ;[1 1 1] Stabilize
      (Utilities|FlowControl|Delay 5.0)
      (if (Variables|Default|GetStabilizing)
        (Variables|Default|SetStabilized true)
        (Variables|Default|SetHacked false)
        (Audio|PlaySoundatLocation "/Game/PlanetSide_2/Audio/Computer/GENERATOR_STABILIZED_Cue.GENERATOR_STABILIZED_Cue" "0, 0, 0")
        (Development|PrintString "Generator Stabilized" true true "(R=0.000000,G=0.714000,B=1.000000,A=1.000000)")
        (goto _label))
      (else
        ;[1 0.6658 0.5002] Generator Overload Sequence
        (Utilities|FlowControl|Delay 5.0)
        (if (Variables|Default|GetHacking)
          (Variables|Default|SetHacked true)
          (Variables|Default|SetStabilized false)
          ;;[1 0.9484 0.03201] Stage 1
          (Utilities|FlowControl|Sequence
            (:then_0
              (Audio|PlaySoundatLocation "/Game/PlanetSide_2/Audio/Computer/GENERATOR_COMPROMISED_Cue.GENERATOR_COMPROMISED_Cue" "0, 0, 0")
              (Audio|Components|Audio|Play (Variables|Default|GetOverload%201%20Loop) 0.0)
              (Audio|Components|Audio|Stop (Variables|Default|GetIdle%20Loop)))
            (:then_1
              (Rendering|Components|Light|SetLightFunctionMaterial _light_3 "/Game/PlanetSide_2/World/Materials/LightFunction/Generator_Light_Inst_Critical1.Generator_Light_Inst_Critical1")
              (Rendering|Components|Light|SetLightColor _light_3 "(R=1.000000,G=0.773868,B=0.000000,A=1.000000)")
              (Rendering|Material|SetMaterial (Variables|Default|GetGenerator) 0 "/Game/PlanetSide_2/World/Materials/Gameplay_Objects/Generator_Inst_Critical1.Generator_Inst_Critical1")
              (Utilities|FlowControl|RetriggerableDelay 1e+01)
              (if (not (Variables|Default|GetStabilized))
                ;;[1 0.2877 0.006723] Stage 2
                (Utilities|FlowControl|Sequence
                  (:then_0
                    (Audio|Components|Audio|Play (Variables|Default|GetOverload%202%20Loop) 0.0)
                    (Audio|Components|Audio|Stop (Variables|Default|GetOverload%201%20Loop)))
                  (:then_1
                    (Rendering|Components|Light|SetLightFunctionMaterial _light "/Game/PlanetSide_2/World/Materials/LightFunction/Generator_Light_Inst_Critical2.Generator_Light_Inst_Critical2")
                    (Rendering|Components|Light|SetLightColor _light "(R=1.000000,G=0.277000,B=0.000000,A=1.000000)")
                    (Rendering|Material|SetMaterial (Variables|Default|GetGenerator) 0 "/Game/PlanetSide_2/World/Materials/Gameplay_Objects/Generator_Inst_Critical2.Generator_Inst_Critical2")
                    (Utilities|FlowControl|RetriggerableDelay 2e+01)
                    (if (not (Variables|Default|GetStabilized))
                      ;;[1 0.008924 0] Stage 3
                      (Utilities|FlowControl|Sequence
                        (:then_0
                          (Audio|PlaySoundatLocation "/Game/PlanetSide_2/Audio/Computer/GENERATOR_CRITICAL_Cue.GENERATOR_CRITICAL_Cue" "0, 0, 0")
                          (Audio|Components|Audio|Play (Variables|Default|GetOverload%203%20Loop) 0.0)
                          (Audio|Components|Audio|Stop (Variables|Default|GetOverload%202%20Loop)))
                        (:then_1
                          (Rendering|Components|Light|SetLightFunctionMaterial _light_2 "/Game/PlanetSide_2/World/Materials/LightFunction/Generator_Light_Inst_Critical3.Generator_Light_Inst_Critical3")
                          (Rendering|Components|Light|SetLightColor _light_2 "(R=1.000000,G=0.000000,B=0.000000,A=1.000000)")
                          (Rendering|Material|SetMaterial (Variables|Default|GetGenerator) 0 "/Game/PlanetSide_2/World/Materials/Gameplay_Objects/Generator_Inst_Critical3.Generator_Inst_Critical3")
                          (Utilities|FlowControl|RetriggerableDelay 1e+01)
                          (if (not (Variables|Default|GetStabilized))
                            ;;[1 1 1] Destroy Generator
                            (Utilities|FlowControl|Sequence
                              (:then_0
                                (Audio|PlaySoundatLocation "/Game/PlanetSide_2/Audio/Computer/GENERATOR_DESTROYED_Cue.GENERATOR_DESTROYED_Cue" "0, 0, 0")
                                (Audio|Components|Audio|Stop (Variables|Default|GetOverload%203%20Loop))
                                (Audio|Components|Audio|Play (Variables|Default|GetExplode) 0.0))
                              (:then_1
                                (Variables|Default|SetIs%20Destroyed true)
                                (Variables|Default|SetRepaired false)
                                (Rendering|SetVisibility (Variables|Default|GetLight) false true)
                                (Rendering|SetVisibility (Variables|Default|GetDestroyed%20Generator) true false)
                                (Components|Activation|Activate (Variables|Default|GetExplosion) false)
                                (Development|PrintString "Generator Destroyed" true true "(R=1.000000,G=0.000000,B=0.000000,A=1.000000)")
                                (CallFunction|GeneratorDisable)))))
                        (:then_2
                          (Rendering|SetVisibility (Variables|Default|GetFire%202) true true)
                          (Rendering|SetVisibility (Variables|Default|GetParticles%203) false true)
                          (Development|PrintString "Generator Overloading: Stage 3" true true "(R=1.000000,G=0.000000,B=0.000000,A=1.000000)")))))
                  (:then_2
                    (Rendering|SetVisibility (Variables|Default|GetFire%201) true true)
                    (Rendering|SetVisibility (Variables|Default|GetParticles%202) false true)
                    (Development|PrintString "Generator Overloading: Stage 2" true true "(R=1.000000,G=0.000000,B=0.000000,A=1.000000)")))))
            (:then_2
              (Rendering|SetVisibility (Variables|Default|GetSmoke) true true)
              (Rendering|SetVisibility (Variables|Default|GetParticles%201) false true)
              (Development|PrintString "Generator Overloading: Stage 1" true true "(R=1.000000,G=0.000000,B=0.000000,A=1.000000)"))))))))

(event Custom|Generator%20Enable
  (if (Variables|Generator|GetGenerator%20Disables%20Lights)
    (Default|CallGeneratorLightsEnabled)
    (elif (Variables|Generator|GetGenerator%20Disables%20Shield)
      _)))

(event Custom|Generator%20Disable
  (if (Variables|Generator|GetGenerator%20Disables%20Lights)
    (Default|CallGeneratorLightsDisabled)
    (elif (Variables|Generator|GetGenerator%20Disables%20Shield)
      _)))

(fn ConstructionScript
  (switch int (Variables|Generator|GetGenerator%20Type)
    (:1
      (Rendering|SetVisibility (Variables|Default|GetIcon%20Vehicle%20Shield) true false))
    (:2
      (Rendering|SetVisibility (Variables|Default|GetIcon%20Horizontal%20Shield) true false))
    (:3
      (Rendering|SetVisibility (Variables|Default|GetIcon%20Vertical%20Shield) true false))
    (:4
      (Rendering|SetVisibility (Variables|Default|GetIcon%20SCU%20Shield) true false))))