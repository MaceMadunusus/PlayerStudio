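; Faction banner prop with a light that re-skins itself for Nanite Systems, New Conglomerate, Terran Republic or Vanu Sovereignty.
; The construction script picks a wall or standing mesh, with old-style lit or unlit variants, and creates a dynamic base material.
; FactionSwitch acts only when FromBaseController matches UsesBaseController.
; It then swaps the second material slot and tints the light and dynamic material through SetFactionParameters.
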(event Custom|Faction%20Switch
  (params (Faction%20Name :type EFaction%20Enum) (FromBaseController :type Boolean))
  (bind _banner (Variables|Default|GetBanner))
  (bind _banner_base_material (Variables|Default|GetBanner%20Base%20Material))
  (bind _light (Variables|Default|GetLight))
  (if (not (Class|KismetMathLibrary|XORBoolean FromBaseController (Variables|Properties|GetUsesBaseController)))
    (switch Utilities|FlowControl|Switch|SwitchonEFaction Faction%20Name
      (:NewEnumerator3
        (CallFunction|SetFactionParameters _banner _light _banner_base_material "/Game/PlanetSide_2/World/Materials/Gameplay_Objects/Banners/MI_FactionBanner.MI_FactionBanner" (Variables|Default|GetLight%20Color)))
      (:NewEnumerator0
        (CallFunction|SetFactionParameters _banner _light _banner_base_material "/Game/PlanetSide_2/World/Materials/Gameplay_Objects/Banners/MI_FactionBanner_NC.MI_FactionBanner_NC" (Variables|Default|GetLight%20Color%20NC)))
      (:NewEnumerator1
        (CallFunction|SetFactionParameters _banner _light _banner_base_material "/Game/PlanetSide_2/World/Materials/Gameplay_Objects/Banners/MI_FactionBanner_TR.MI_FactionBanner_TR" (Variables|Default|GetLight%20Color%20TR)))
      (:NewEnumerator2
        (CallFunction|SetFactionParameters _banner _light _banner_base_material "/Game/PlanetSide_2/World/Materials/Gameplay_Objects/Banners/MI_FactionBanner_VS.MI_FactionBanner_VS" (Variables|Default|GetLight%20Color%20VS))))))

(fn ConstructionScript
  (bind _banner (Variables|Default|GetBanner))
  (bind _wall_mounted (Variables|Properties|GetWall%20Mounted))
  (bind _light (Variables|Default|GetLight))
  (bind _banner_2 (Variables|Default|GetBanner))
  (bind _banner_enabled (Variables|Properties|GetBanner%20Enabled))
  (if (Variables|Properties|GetOldStyle)
    (if _wall_mounted
      (Transformation|SetRelativeLocation _light "0, 0,-290.000000" false false)
      (if _banner_enabled
        (Components|StaticMesh|SetStaticMesh _banner_2 "/Game/PlanetSide_2/World/Meshes/Gameplay/Banner_Wall_Old.Banner_Wall_old")
        (bind _returnvalue (Rendering|Material|CreateDynamicMaterialInstance "/Game/PlanetSide_2/World/Materials/Gameplay_Objects/MI_FactionBanner.MI_FactionBanner" :!class /Script/Engine.KismetMaterialLibrary :!label _label))
        (bind _output_get (Variables|Default|SetBanner%20Base%20Material _returnvalue))
        (Rendering|Material|SetMaterial (Variables|Default|GetBanner) 0 _output_get)
        (else
          (Components|StaticMesh|SetStaticMesh _banner_2 "/Game/PlanetSide_2/World/Meshes/Gameplay/Banner_Wall_Off.Banner_Wall_Off")
          (bind _returnvalue_2 (Rendering|Material|CreateDynamicMaterialInstance "/Game/PlanetSide_2/World/Materials/Gameplay_Objects/MI_FactionBanner.MI_FactionBanner" :!class /Script/Engine.KismetMaterialLibrary :!label _label_2))
          (bind _output_get_2 (Variables|Default|SetBanner%20Base%20Material _returnvalue_2))
          (Rendering|Material|SetMaterial (Variables|Default|GetBanner) 0 _output_get_2)
          (Rendering|SetVisibility (Variables|Default|GetLight) false false)))
      (elif _banner_enabled
        (Components|StaticMesh|SetStaticMesh _banner_2 "/Game/PlanetSide_2/World/Meshes/Gameplay/Banner_Standing_Old.Banner_Standing_Old")
        (goto _label)
        (else
          (Components|StaticMesh|SetStaticMesh _banner_2 "/Game/PlanetSide_2/World/Meshes/Gameplay/Banner_Standing_Off.Banner_Standing_Off")
          (goto _label_2))))
    (else
      (if _wall_mounted
        (Transformation|SetRelativeLocation _light "0, 0,-290.000000" false false)
        (Components|StaticMesh|SetStaticMesh _banner "/Game/PlanetSide_2/World/Meshes/Gameplay/Banner_Wall.Banner_Wall")
        (else
          (Components|StaticMesh|SetStaticMesh _banner "/Game/PlanetSide_2/World/Meshes/Gameplay/Banner_Standing.Banner_Standing")))
      (bind _returnvalue_3 (Rendering|Material|CreateDynamicMaterialInstance "/Game/PlanetSide_2/World/Materials/Gameplay_Objects/MI_FactionBanner.MI_FactionBanner" :!class /Script/Engine.KismetMaterialLibrary))
      (bind _output_get_3 (Variables|Default|SetBanner%20Base%20Material _returnvalue_3))
      (Rendering|Material|SetMaterial (Variables|Default|GetBanner) 0 _output_get_3))))

(fn SetFactionParameters
  (params (Mesh :type Static%20Mesh%20Component%20Object%20Reference) (Light :type Light%20Component%20Object%20Reference) (Dynamic%20Material :type Material%20Instance%20Dynamic%20Object%20Reference) (Material :type Material%20Instance%20Object%20Reference) (Color :type Linear%20Color%20Structure))
  (Rendering|Material|SetMaterial Mesh 1 Material)
  (Rendering|Components|Light|SetLightColor Light Color true)
  (Rendering|Material|SetVectorParameterValue Dynamic%20Material "Color" Color :!class /Script/Engine.MaterialInstanceDynamic))