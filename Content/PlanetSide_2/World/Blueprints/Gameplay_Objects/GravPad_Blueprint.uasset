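; Gravity pad world object for a PlanetSide 2 map, with up and down variants and a looping lift sound.
; The construction script reads GravityPadType to set the pad mesh and material, show the matching up or down particles, and tint the light yellow or blue.
; At runtime, the LiftSoundArea overlap starts and stops the audio loop; no lift movement logic appears in these graphs.
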(event OnComponentBeginOverlap(LiftSoundArea)
  (params (OtherActor :type Actor%20Object%20Reference) (OtherComp :type Primitive%20Component%20Object%20Reference) (OtherBodyIndex :type Integer))
  (Components|Activation|Activate (Variables|Sound|GetGravity%20Lift%20Audio%20Loop) false))

(event OnComponentEndOverlap(LiftSoundArea)
  (params (OtherActor :type Actor%20Object%20Reference) (OtherComp :type Primitive%20Component%20Object%20Reference) (OtherBodyIndex :type Integer))
  (Components|Activation|Deactivate (Variables|Sound|GetGravity%20Lift%20Audio%20Loop)))

(fn ConstructionScript
  (bind _gravity_pad (Variables|Meshes|GetGravity%20Pad))
  (bind _gravity_pad_particles_up (Variables|Particles|GetGravity%20Pad%20Particles%20Up))
  (bind _gravity_pad_particles_down (Variables|Particles|GetGravity%20Pad%20Particles%20Down))
  (bind _light (Variables|Default|GetLight))
  (switch int (Variables|GravityPad|GetGravity%20Pad%20Type)
    (:1
      (Components|StaticMesh|SetStaticMesh _gravity_pad "/Game/PlanetSide_2/World/Meshes/Gameplay/JumpPad3.JumpPad3")
      (Rendering|Material|SetMaterial _gravity_pad 0 "/Game/PlanetSide_2/World/Materials/Gameplay_Objects/GravityPads_Up.GravityPads_Up")
      (Rendering|SetVisibility _gravity_pad_particles_up true false)
      (Rendering|SetVisibility _gravity_pad_particles_down false false)
      (Rendering|Components|Light|SetLightColor _light "(R=1.000000,G=0.800000,B=0.000000,A=1.000000)"))
    (:2
      (Components|StaticMesh|SetStaticMesh _gravity_pad "/Game/PlanetSide_2/World/Meshes/Gameplay/JumpPad2.JumpPad2")
      (Rendering|Material|SetMaterial _gravity_pad 0 "/Game/PlanetSide_2/World/Materials/Gameplay_Objects/GravityPads_Down.GravityPads_Down")
      (Rendering|SetVisibility _gravity_pad_particles_up false false)
      (Rendering|SetVisibility _gravity_pad_particles_down true false)
      (Rendering|Components|Light|SetLightColor _light "(R=0.000000,G=0.491777,B=1.000000,A=1.000000)"))))