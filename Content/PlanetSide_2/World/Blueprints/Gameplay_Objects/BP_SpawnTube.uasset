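; BP_SpawnTube is a spawn tube gameplay object that switches between an enabled and a disabled look and sound.
; The construction script sets Shield and Light visibility from SpawnEnabled, adding a child actor and TubeAudio when enabled, or applying the off material otherwise.
; The SpawnTubeEnable/Disable event toggles the tube material, Shield and Light visibility, and audio playback at runtime.
; TubeAudio is created only for tubes enabled at construction.
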(event Custom|SpawnTube%20Enable/Disable
  (params (Spawn%20Enabled :type Boolean))
  (bind _spawntube (Variables|Meshes|GetSpawnTube))
  (bind _tube_audio (Variables|Default|GetTube%20Audio))
  (if Spawn%20Enabled
    (Rendering|Material|SetMaterial _spawntube 0 "/Game/PlanetSide_2/World/Materials/Gameplay_Objects/MI_SpawnTube.MI_SpawnTube")
    (Rendering|SetVisibility (Variables|Default|GetLight) true false)
    (Audio|Components|Audio|Play _tube_audio 0.0)
    (else
      (Rendering|Material|SetMaterial _spawntube 0 "/Game/PlanetSide_2/World/Materials/Gameplay_Objects/MI_SpawnTube_Off.MI_SpawnTube_Off")
      (Rendering|SetVisibility (Variables|Meshes|GetShield) false false)
      (Audio|Components|Audio|Stop _tube_audio))))

(fn ConstructionScript
  (Rendering|SetVisibility (Variables|Meshes|GetShield) (Variables|Properties|GetSpawn%20Enabled) false)
  (if (Variables|Properties|GetSpawn%20Enabled)
    (AddComponent|AddChildActorComponent false)
    (bind _returnvalue (AddComponent|AddAudioComponent false))
    (Variables|Default|SetTube%20Audio _returnvalue)
    (else
      (Rendering|Material|SetMaterial (Variables|Meshes|GetSpawnTube) 0 "/Game/PlanetSide_2/World/Materials/Gameplay_Objects/MI_SpawnTube_Off.MI_SpawnTube_Off"))))