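; BP_Shield is a one-way shield gameplay object that shows its owning faction's spawn shield color.
; The construction script assigns the configured mesh and swaps its outer and inner material slots for dynamic instances.
; FactionSwitch recolors both instances from class-default faction colors, only when the caller's base-controller flag matches the shield's own setting.
; A separate enable/disable event only toggles mesh visibility.
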(event Custom|Faction%20Switch
  (params (Faction%20Name :type EFaction%20Enum :default "NewEnumerator3") (FromBaseController :type Boolean))
  (bind (_ns_spawn_shield_color _nc_spawn_shield_color _tr_spawn_shield_color _vs_spawn_shield_color) (Utilities|GetClassDefaults "/Game/PlanetSide_2/UI/FactionSwitch.FactionSwitch_C"))
  (bind _shieldoutermaterial (Variables|Default|GetShieldOuterMaterial))
  (if (not (Class|KismetMathLibrary|XORBoolean FromBaseController (Variables|Properties|GetUsesBaseController)))
    (switch Utilities|FlowControl|Switch|SwitchonEFaction Faction%20Name
      (:NewEnumerator3
        (Rendering|Material|SetVectorParameterValue _shieldoutermaterial "Color" _ns_spawn_shield_color :!class /Script/Engine.MaterialInstanceDynamic))
      (:NewEnumerator0
        (Rendering|Material|SetVectorParameterValue _shieldoutermaterial "Color" _nc_spawn_shield_color :!class /Script/Engine.MaterialInstanceDynamic))
      (:NewEnumerator1
        (Rendering|Material|SetVectorParameterValue _shieldoutermaterial "Color" _tr_spawn_shield_color :!class /Script/Engine.MaterialInstanceDynamic))
      (:NewEnumerator2
        (Rendering|Material|SetVectorParameterValue _shieldoutermaterial "Color" _vs_spawn_shield_color :!class /Script/Engine.MaterialInstanceDynamic)))))

(event Custom|Shield%20Enable/Disable
  (params (Enabled :type Boolean))
  (bind _onewayshield (Variables|Default|GetOneWayShield))
  (if Enabled
    (Rendering|SetVisibility _onewayshield true false)
    (else
      (Rendering|SetVisibility _onewayshield false false))))

(event EventBeginPlay)

(event EventActorBeginOverlap
  (params (OtherActor :type Actor%20Object%20Reference)))

(event EventTick
  (params (DeltaSeconds :type Float%20%28single-precision%29)))

(fn ConstructionScript
  (bind _onewayshield (Variables|Default|GetOneWayShield))
  (bind _returnvalue (Rendering|Material|GetMaterials _onewayshield))
  (Components|StaticMesh|SetStaticMesh _onewayshield (Variables|Properties|GetShield%20Mesh))
  (bind _returnvalue_2 (Rendering|Material|CreateDynamicMaterialInstance "/Game/PlanetSide_2/World/Materials/Gameplay_Objects/Shields/Shield_Outer_Manual.Shield_Outer_Manual" "None" :!class /Script/Engine.KismetMaterialLibrary))
  (bind _output_get (Variables|Default|SetShieldOuterMaterial _returnvalue_2))
  (Rendering|Material|SetMaterial (Variables|Default|GetOneWayShield) (Utilities|Array|FindItem _returnvalue "/Game/PlanetSide_2/World/Materials/Gameplay_Objects/Shields/Shield_Outer.Shield_Outer") _output_get)
  (bind _returnvalue_3 (Rendering|Material|CreateDynamicMaterialInstance "/Game/PlanetSide_2/World/Materials/Gameplay_Objects/Shields/Shield_Inner_Manual.Shield_Inner_Manual" "None" :!class /Script/Engine.KismetMaterialLibrary))
  (bind _output_get_2 (Variables|Default|SetShieldInnerMaterial _returnvalue_3))
  (Rendering|Material|SetMaterial (Variables|Default|GetOneWayShield) (Utilities|Array|FindItem _returnvalue "/Game/PlanetSide_2/World/Materials/Gameplay_Objects/Shields/Shield_Inner.Shield_Inner") _output_get_2))