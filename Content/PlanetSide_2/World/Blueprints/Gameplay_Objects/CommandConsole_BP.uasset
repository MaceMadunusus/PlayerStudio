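; Capture console for PlanetSide 2 facilities that shows the owning faction through its material and light color.
; Overlapping the capture radius starts a short timer, which leaving cancels unless the point is already captured.
; Point capture plays a notification and, gated by a DoOnce, starts a longer timer that calls FacilityCaptured on the target facility matching its base type, then resets.
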(event OnComponentBeginOverlap(CaptureRadius)
  (params (OtherActor :type Actor%20Object%20Reference) (OtherComp :type Primitive%20Component%20Object%20Reference) (OtherBodyIndex :type Integer) (bFromSweep :type Boolean) (SweepResult :type Hit%20Result%20Structure%20%28by%20ref%29))
  (bind _returnvalue (Utilities|Time|SetTimerbyFunctionName 0 "Capture Point" 5.0))
  (Variables|Default|SetCaptureBaseTimer _returnvalue))

(event OnComponentEndOverlap(CaptureRadius)
  (params (OtherActor :type Actor%20Object%20Reference) (OtherComp :type Primitive%20Component%20Object%20Reference) (OtherBodyIndex :type Integer))
  (if (not (Variables|Default|GetCaptured))
    (Class|KismetSystemLibrary|ClearTimerHandle (Variables|Default|GetCaptureBaseTimer))))

(event Custom|Capture%20Point
  (Variables|Default|SetCaptured true)
  (Audio|PlaySoundatLocation "/Game/PlanetSide_2/Audio/UI/UI_WHISPER_NOTIFICATION.UI_WHISPER_NOTIFICATION" "0, 0, 0")
  (Utilities|FlowControl|DoOnce false
    (:Completed
      (Utilities|Time|SetTimerbyFunctionName 0 "Capture Base" 6e+01))))

(event Custom|Capture%20Base
  (bind _captured_by (Variables|Default|GetCaptured%20By))
  (Variables|Default|SetCaptured false)
  (Class|KismetSystemLibrary|ClearTimerHandle (Variables|Default|GetCaptureBaseTimer))
  (Utilities|FlowControl|Sequence
    (:then_0
      (switch Utilities|FlowControl|Switch|SwitchonCapturePoint_BaseTarget (Variables|Default|GetCapture%20Base%20Type%20Target)
        (:NewEnumerator1
          (Default|FacilityCaptured (Variables|Default|GetAmp%20Station%20Target) _captured_by))
        (:NewEnumerator2
          (Default|FacilityCaptured (Variables|Default|GetBiolab%20Target) _captured_by))
        (:NewEnumerator3
          (Default|FacilityCaptured (Variables|Default|GetTech%20Plant%20Target) _captured_by))
        (:NewEnumerator4
          (Default|FacilityCaptured (Variables|Default|GetInterlink%20Target) _captured_by))
        (:NewEnumerator5
          (Default|FacilityCaptured (Variables|Default|GetWarpgate%20Target) _captured_by))))
    (:then_1
      (Utilities|FlowControl|DoOnce false) ; enters at Reset
    )))

(event Custom|Faction%20Switch
  (params (Faction :type Name :default "None"))
  (bind _light (Variables|Default|GetLight))
  (bind _console (Variables|Default|GetConsole))
  (switch name Faction
    (:NS
      (Rendering|Material|SetMaterial _console 1 "/Game/PlanetSide_2/World/Materials/Gameplay_Objects/Console/Commandconsole_NS.CommandConsole_NS")
      (Rendering|Components|Light|SetLightColor _light (Variables|Default|GetLight%20Color%20NS) true))
    (:NC
      (Rendering|Material|SetMaterial _console 1 "/Game/PlanetSide_2/World/Materials/Gameplay_Objects/Console/Commandconsole_NC.CommandConsole_NC")
      (Rendering|Components|Light|SetLightColor _light (Variables|Default|GetLight%20Color%20NC) true))
    (:TR
      (Rendering|Material|SetMaterial _console 1 "/Game/PlanetSide_2/World/Materials/Gameplay_Objects/Console/Commandconsole_TR.CommandConsole_TR")
      (Rendering|Components|Light|SetLightColor _light (Variables|Default|GetLight%20Color%20TR) true))
    (:VS
      (Rendering|Material|SetMaterial _console 1 "/Game/PlanetSide_2/World/Materials/Gameplay_Objects/Console/Commandconsole_VS.CommandConsole_VS")
      (Rendering|Components|Light|SetLightColor _light (Variables|Default|GetLight%20Color%20VS) true))))

(fn ConstructionScript
  (switch Utilities|FlowControl|Switch|SwitchonCapturePoint (Variables|Default|GetLetter)))