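; Facility turret placeable whose weapon mesh follows its TurretType: anti-infantry, anti-vehicle, anti-air or missile.
; The construction script sets that mesh and chooses a standard base or a rotated wall platform.
; Overlapping the Sphere enables mouse interaction and creates a TurretTowers widget once, which clicking toggles; leaving removes it.
; Hover highlights the turret through custom depth, and SetTurretType swaps the mesh at runtime.
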(event OnComponentBeginOverlap(Sphere)
  (params (OtherActor :type Actor%20Object%20Reference) (OtherComp :type Primitive%20Component%20Object%20Reference) (OtherBodyIndex :type Integer) (bFromSweep :type Boolean) (SweepResult :type Hit%20Result%20Structure%20%28by%20ref%29))
  (bind _returnvalue (Game|GetPlayerController 0))
  (bind (_sizex _sizey) (HUD|GetViewportSize _returnvalue))
  (Utilities|FlowControl|Sequence
    (:then_0
      (Utilities|FlowControl|DoOnce false
        (:Completed
          (bind _returnvalue_2 (UserInterface|CreateWidget "/Game/PlanetSide_2/UI/TurretTowers.TurretTowers_C" _returnvalue self))
          (bind _output_get (Variables|Default|SetTurretUI _returnvalue_2))
          (Class|UserWidget|SetPositioninViewport _output_get (Math|Vector2D|MakeVector2D (Math|Conversions|ToFloat(Integer) (- (/ _sizex 2) 200)) (Math|Conversions|ToFloat(Integer) (- (/ _sizey 2) 75))) true))))
    (:then_1
      (Variables|Default|SetIsInRange true)
      (Input|EnableInput _returnvalue)
      (Variables|/Script/Engine.PlayerController|SetbEnableMouseOverEvents _returnvalue true))))

(event OnComponentEndOverlap(Sphere)
  (params (OtherActor :type Actor%20Object%20Reference) (OtherComp :type Primitive%20Component%20Object%20Reference) (OtherBodyIndex :type Integer))
  (bind _returnvalue (Game|GetPlayerController 0))
  (Variables|Default|SetIsInRange false)
  (Widget|RemovefromParent (Variables|Default|GetTurretUI))
  (Input|DisableInput _returnvalue)
  (Variables|/Script/Engine.PlayerController|SetbShowMouseCursor _returnvalue false)
  (Variables|/Script/Engine.PlayerController|SetbEnableMouseOverEvents _returnvalue false)
  (Input|SetInputModeGameOnly _returnvalue)
  (Rendering|SetRenderCustomDepth (Variables|Default|GetFacilityTurret) false))

(event OnClicked(FacilityTurret)
  (params (TouchedComponent :type Primitive%20Component%20Object%20Reference))
  (bind _returnvalue (Game|GetPlayerController 0))
  (bind _turretui (Variables|Default|GetTurretUI))
  (Utilities|FlowControl|FlipFlop
    (:A
      (if (Variables|Default|GetIsInRange)
        (UserInterface|Viewport|AddtoViewport _turretui 0)
        (Variables|/Script/Engine.PlayerController|SetbShowMouseCursor _returnvalue true)
        (Input|SetInputModeGameandUI _returnvalue (Variables|Default|GetTurretUI) true false)))
    (:B
      (Widget|RemovefromParent _turretui)
      (Variables|/Script/Engine.PlayerController|SetbShowMouseCursor _returnvalue false)
      (Input|SetInputModeGameOnly _returnvalue))))

(event OnBeginCursorOver(FacilityTurret)
  (params (TouchedComponent :type Primitive%20Component%20Object%20Reference))
  (Rendering|SetRenderCustomDepth (Variables|Default|GetFacilityTurret) true))

(event OnEndCursorOver(FacilityTurret)
  (params (TouchedComponent :type Primitive%20Component%20Object%20Reference))
  (Rendering|SetRenderCustomDepth (Variables|Default|GetFacilityTurret) false))

(event Custom|Set%20Turret%20Type
  (params (Turret%20Type :type TurretType%20Enum))
  (bind _facilityturret (Variables|Default|GetFacilityTurret))
  (switch Utilities|FlowControl|Switch|SwitchonTurretType Turret%20Type
    (:NewEnumerator0
      (Components|StaticMesh|SetStaticMesh _facilityturret "/Game/PlanetSide_2/World/Meshes/Gameplay/FacilityTurret_Chaingun.FacilityTurret_Chaingun"))
    (:NewEnumerator1
      (Components|StaticMesh|SetStaticMesh _facilityturret "/Game/PlanetSide_2/World/Meshes/Gameplay/FacilityTurret_TankCannon.FacilityTurret_TankCannon"))
    (:NewEnumerator2
      (Components|StaticMesh|SetStaticMesh _facilityturret "/Game/PlanetSide_2/World/Meshes/Gameplay/FacilityTurret_FlakCannon.FacilityTurret_FlakCannon"))
    (:NewEnumerator3
      (Components|StaticMesh|SetStaticMesh _facilityturret "/Game/PlanetSide_2/World/Meshes/Gameplay/FacilityTurret_MissileLauncher.FacilityTurret_MissileLauncher"))))

(fn ConstructionScript
  (bind _facilityturret (Variables|Default|GetFacilityTurret))
  (bind _facilityturret_base (Variables|Default|GetFacilityTurret_Base))
  (Utilities|FlowControl|Sequence
    (:then_0
      (switch Utilities|FlowControl|Switch|SwitchonTurretType (Variables|Turret|GetTurret%20Type)
        (:NewEnumerator0
          (Components|StaticMesh|SetStaticMesh _facilityturret "/Game/PlanetSide_2/World/Meshes/Gameplay/FacilityTurret_Chaingun.FacilityTurret_Chaingun"))
        (:NewEnumerator1
          (Components|StaticMesh|SetStaticMesh _facilityturret "/Game/PlanetSide_2/World/Meshes/Gameplay/FacilityTurret_TankCannon.FacilityTurret_TankCannon"))
        (:NewEnumerator2
          (Components|StaticMesh|SetStaticMesh _facilityturret "/Game/PlanetSide_2/World/Meshes/Gameplay/FacilityTurret_FlakCannon.FacilityTurret_FlakCannon"))
        (:NewEnumerator3
          (Components|StaticMesh|SetStaticMesh _facilityturret "/Game/PlanetSide_2/World/Meshes/Gameplay/FacilityTurret_MissileLauncher.FacilityTurret_MissileLauncher"))))
    (:then_1
      (if (Variables|Turret|GetWall%20Turret)
        (Components|StaticMesh|SetStaticMesh _facilityturret_base "/Game/PlanetSide_2/World/Meshes/Gameplay/FacilityTurret_Platform.FacilityTurret_Platform")
        (Transformation|SetRelativeRotation _facilityturret_base "0,90.000000, 0" false false)
        (Transformation|SetRelativeLocation (Variables|Default|GetFacilityTurret) "0,610.000000,20.000000" false false)
        (else
          (Components|StaticMesh|SetStaticMesh _facilityturret_base "/Game/PlanetSide_2/World/Meshes/Gameplay/FacilityTurret_Base.FacilityTurret_Base"))))))