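; BP_AmmoTower is a world ammo tower with faction access, a vehicle resupply icon and an ammo restore range sphere.
; With UsesBaseController enabled, construction creates the dynamic icon material and sizes the sphere.
; FactionSwitch sets access and recolors the icon from shared class-default faction colors, only when the call's source matches that flag.
; Tick continuously spins the top; no ammo-restoring logic is present.
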(event Custom|Faction%20Switch
  (params (Faction%20Name :type EFaction%20Enum) (FromBaseController :type Boolean))
  (bind (_ns_ui_color _nc_ui_color _tr_ui_color _vs_ui_color) (Utilities|GetClassDefaults "/Game/PlanetSide_2/UI/FactionSwitch.FactionSwitch_C"))
  (bind _icon_material (Variables|Default|GetIcon%20Material))
  (if (not (Class|KismetMathLibrary|XORBoolean FromBaseController (Variables|Default|GetUsesBaseController)))
    (switch Utilities|FlowControl|Switch|SwitchonEFaction Faction%20Name
      (:NewEnumerator3
        (Variables|Default|SetFactionAccess "NewEnumerator3")
        (Rendering|Material|SetVectorParameterValue _icon_material "Color" _ns_ui_color :!class /Script/Engine.MaterialInstanceDynamic))
      (:NewEnumerator0
        (Variables|Default|SetFactionAccess "NewEnumerator0")
        (Rendering|Material|SetVectorParameterValue _icon_material "Color" _nc_ui_color :!class /Script/Engine.MaterialInstanceDynamic))
      (:NewEnumerator1
        (Variables|Default|SetFactionAccess "NewEnumerator1")
        (Rendering|Material|SetVectorParameterValue _icon_material "Color" _tr_ui_color :!class /Script/Engine.MaterialInstanceDynamic))
      (:NewEnumerator2
        (Variables|Default|SetFactionAccess "NewEnumerator2")
        (Rendering|Material|SetVectorParameterValue _icon_material "Color" _vs_ui_color :!class /Script/Engine.MaterialInstanceDynamic)))))

(event EventTick
  (params (DeltaSeconds :type Float%20%28single-precision%29))
  (Transformation|AddLocalRotation (Variables|Default|GetTop) (Math|Rotator|MakeRotator 0.0 0.0 (Variables|Default|GetRotationRate)) false false))

(fn ConstructionScript
  (if (Variables|Default|GetUsesBaseController)
    (bind _returnvalue (Rendering|Material|CreateDynamicMaterialInstance "/Game/PlanetSide_2/UI/Icons/Materials/MI_Icon_Base_Manual.MI_Icon_Base_Manual" :!class /Script/Engine.KismetMaterialLibrary))
    (bind _output_get (Variables|Default|SetIcon%20Material _returnvalue))
    (Rendering|Material|SetMaterial (Variables|Default|GetIcons) 0 _output_get)
    (Rendering|Material|SetTextureParameterValue (Variables|Default|GetIcon%20Material) "Texture" "/Game/PlanetSide_2/UI/Icons/Textures/Icon_Vehicle_Resupply.Icon_Vehicle_Resupply")
    (Components|Sphere|SetSphereRadius (Variables|Default|GetAmmoRestoreRange) (Variables|Default|GetAmmo%20Restore%20Radius) true)))