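; Spawn Control Unit base objective that players inside its hacking area can overload, stabilize or repair with the Ability input.
; An overload escalates through timed critical stages to destruction using retriggerable delays, swapping light, materials, effects and audio unless stabilized.
; Each state change is reported to BaseController.
; A billboard icon reflects faction color and destruction, and debug lines can show links to its spawn tube targets.
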(event OnComponentBeginOverlap(HackingAOE)
  (params (OtherActor :type Actor%20Object%20Reference) (OtherComp :type Primitive%20Component%20Object%20Reference) (OtherBodyIndex :type Integer) (bFromSweep :type Boolean) (SweepResult :type Hit%20Result%20Structure%20%28by%20ref%29))
  (Input|EnableInput (Game|GetPlayerController 0)))

(event OnComponentEndOverlap(HackingAOE)
  (params (OtherActor :type Actor%20Object%20Reference) (OtherComp :type Primitive%20Component%20Object%20Reference) (OtherBodyIndex :type Integer))
  (Input|DisableInput (Game|GetPlayerController 0)))

(event Custom|Enable/Disable%20Icons
  (params (Visibility :type Boolean))
  (Rendering|SetVisibility (Variables|Default|GetIcon%20SCU) Visibility false))

(event Custom|Display%20Connection%20Lines
  ;[1 1 1] Draw Connections
  (for _array_element (Variables|Properties|GetSpawn%20Tube%20Targets)
    (Rendering|Debug|DrawDebugLine (+ (Transformation|GetWorldLocation (Variables|Default|GetSCU)) "0, 0,244.000000") (+ (Transformation|GetActorLocation _array_element) "0, 0,122.000000") "(R=1.000000,G=1.000000,B=0.000000,A=1.000000)" 6e+01 5.0)))

(event Custom|Faction%20Switch
  (params (Faction%20Name :type EFaction%20Enum) (FromBaseController :type Boolean))
  (bind (_ns_ui_color _nc_ui_color _tr_ui_color _vs_ui_color) (Utilities|GetClassDefaults "/Game/PlanetSide_2/UI/FactionSwitch.FactionSwitch_C"))
  (bind _icon_material (Variables|Default|GetIcon%20Material))
  ;[1 1 1] Faction Switching
  (if (not (Class|KismetMathLibrary|XORBoolean FromBaseController (Variables|Properties|GetUsesBaseController)))
    (switch Utilities|FlowControl|Switch|SwitchonEFaction Faction%20Name
      (:NewEnumerator3
        (Variables|Default|SetFactionAccess "NewEnumerator3")
        (Rendering|Material|SetVectorParameterValue _icon_material "Color" _ns_ui_color :!class /Script/Engine.MaterialInstanceDynamic))
      (:NewEnumerator0
        (Variables|Default|SetFactionAccess "NewEnumerator0")
        (Rendering|Material|SetVectorParameterValue _icon_material "Color" _nc_ui_color :!class /Script/Engine.MaterialInstanceDynamic))
      (:NewEnumerator1
        (Variables|Default|SetFactionAccess "NewEnumerator1")
        (Rendering|Material|SetVectorParameterValue _icon_material "Color" _tr_ui_color :!class /Script/Engine.MaterialInstanceDynamic))
      (:NewEnumerator2
        (Variables|Default|SetFactionAccess "NewEnumerator2")
        (Rendering|Material|SetVectorParameterValue _icon_material "Color" _vs_ui_color :!class /Script/Engine.MaterialInstanceDynamic)))))

(event Input|ActionEvents|InputActionAbility
  (params (Key :type Key%20Structure :default "AnyKey"))
  (bind _light (Variables|Default|GetLight))
  (bind _light_2 (Variables|Default|GetLight))
  (bind _light_3 (Variables|Default|GetLight))
  (bind _light_4 (Variables|Default|GetLight))
  (bind _scu_audio (Variables|Default|GetSCU%20Audio))
  (:Pressed
    (if (Variables|Default|GetIs%20Destroyed)
      ;[1 1 1] Repair
      (Variables|Default|SetHacked false)
      (Variables|Default|SetIs%20Destroyed false)
      (Default|SCURepaired (Variables|Properties|GetBase%20Controller))
      (Utilities|FlowControl|Sequence
        (:then_1
          ;[1 1 1] Generator Reset
          (Rendering|SetVisibility _light_4 true true :!label _label)
          (Rendering|SetVisibility (Variables|Default|GetDestroyed%20SCU) false true)
          (Rendering|Components|Light|SetLightFunctionMaterial _light_4 "/Game/PlanetSide_2/Effects/LightFunction/MI_Generator_Light.MI_Generator_Light")
          (Rendering|Components|Light|SetLightColor _light_4 "(R=0.690000,G=0.690000,B=1.000000,A=1.000000)" true)
          (Rendering|Material|SetMaterial (Variables|Default|GetSCU) 0 "/Game/PlanetSide_2/World/Materials/Gameplay_Objects/MI_SpawnControlUnit.MI_SpawnControlUnit")
          (Effects|Components|ParticleSystem|SetIntParameter _scu_audio "SCU Damage Level" 0)
          (Audio|Components|Audio|Play _scu_audio 0.0)
          (Rendering|Material|SetTextureParameterValue (Variables|Default|GetIcon%20Material) "Texture" "/Game/PlanetSide_2/UI/Icons/Textures/Icon_SCU.Icon_SCU")))
      (else
        ;[1 1 1] Stabilize
        (if (Variables|Default|GetHacked)
          (Variables|Default|SetHacked false)
          (Variables|Default|SetStabilized true)
          (Default|SCUStabilized (Variables|Properties|GetBase%20Controller))
          (goto _label)
          (else
            ;[1 0.6658 0.5002] Generator Overload Sequence
            (Variables|Default|SetStabilized false)
            (Variables|Default|SetHacked true)
            ;;[1 0.9484 0.03201] Stage 1
            (Utilities|FlowControl|Sequence
              (:then_0
                (Default|SCUChangeStatus (Variables|Properties|GetBase%20Controller) 1)
                (Effects|Components|ParticleSystem|SetIntParameter (Variables|Default|GetSCU%20Audio) "SCU Damage Level" 1))
              (:then_1
                (Rendering|Components|Light|SetLightFunctionMaterial _light_3 "/Game/PlanetSide_2/Effects/LightFunction/MI_Generator_Light_Critical1.MI_Generator_Light_Critical1")
                (Rendering|Components|Light|SetLightColor _light_3 "(R=1.000000,G=0.773868,B=0.000000,A=1.000000)" true)
                (Rendering|Material|SetMaterial (Variables|Default|GetSCU) 0 "/Game/PlanetSide_2/World/Materials/Gameplay_Objects/MI_SCU_Critical1.MI_SCU_Critical1")
                (Utilities|FlowControl|RetriggerableDelay 1e+01)
                (if (not (Variables|Default|GetStabilized))
                  ;;[1 0.2877 0.006723] Stage 2
                  (Utilities|FlowControl|Sequence
                    (:then_0
                      (Effects|Components|ParticleSystem|SetIntParameter (Variables|Default|GetSCU%20Audio) "SCU Damage Level" 2)
                      (Default|SCUChangeStatus (Variables|Properties|GetBase%20Controller) 2))
                    (:then_1
                      (Rendering|Components|Light|SetLightFunctionMaterial _light "/Game/PlanetSide_2/Effects/LightFunction/MI_Generator_Light_Critical2.MI_Generator_Light_Critical2")
                      (Rendering|Components|Light|SetLightColor _light "(R=1.000000,G=0.277000,B=0.000000,A=1.000000)" true)
                      (Rendering|Material|SetMaterial (Variables|Default|GetSCU) 0 "/Game/PlanetSide_2/World/Materials/Gameplay_Objects/MI_SCU_Critical2.MI_SCU_Critical2")
                      (Utilities|FlowControl|RetriggerableDelay 2e+01)
                      (if (not (Variables|Default|GetStabilized))
                        ;;[1 0.008924 0] Stage 3
                        (Utilities|FlowControl|Sequence
                          (:then_0
                            (Default|SCUChangeStatus (Variables|Properties|GetBase%20Controller) 3)
                            (Effects|Components|ParticleSystem|SetIntParameter (Variables|Default|GetSCU%20Audio) "SCU Damage Level" 3))
                          (:then_1
                            (Rendering|Components|Light|SetLightFunctionMaterial _light_2 "/Game/PlanetSide_2/Effects/LightFunction/MI_Generator_Light_Critical3.MI_Generator_Light_Critical3")
                            (Rendering|Components|Light|SetLightColor _light_2 "(R=1.000000,G=0.000000,B=0.000000,A=1.000000)" true)
                            (Rendering|Material|SetMaterial (Variables|Default|GetSCU) 0 "/Game/PlanetSide_2/World/Materials/Gameplay_Objects/MI_SCU_Critical3.MI_SCU_Critical3")
                            (Utilities|FlowControl|RetriggerableDelay 1e+01)
                            (if (not (Variables|Default|GetStabilized))
                              ;;[1 1 1] Destroy Generator
                              (Utilities|FlowControl|Sequence
                                (:then_0
                                  (Default|SCUDestroyed (Variables|Properties|GetBase%20Controller))
                                  (Audio|Components|Audio|Stop (Variables|Default|GetSCU%20Audio))
                                  (Audio|Components|Audio|Play (Variables|Default|GetExplode) 0.0))
                                (:then_1
                                  (Variables|Default|SetIs%20Destroyed true)
                                  (Rendering|SetVisibility (Variables|Default|GetLight) false true)
                                  (Rendering|SetVisibility (Variables|Default|GetDestroyed%20SCU) true false)
                                  (Components|Activation|Activate (Variables|Default|GetExplosion) false)
                                  (Rendering|Material|SetTextureParameterValue (Variables|Default|GetIcon%20Material) "Texture" "/Game/PlanetSide_2/UI/Icons/Textures/Icon_SCU_Destroyed.Icon_SCU_Destroyed")))))
                          (:then_2
                            (Rendering|SetVisibility (Variables|Default|GetFire%202) true true)
                            (Rendering|SetVisibility (Variables|Default|GetParticles%203) false true)))))
                    (:then_2
                      (Rendering|SetVisibility (Variables|Default|GetFire%201) true true)
                      (Rendering|SetVisibility (Variables|Default|GetParticles%202) false true)))))
              (:then_2
                (Rendering|SetVisibility (Variables|Default|GetSmoke) true true)
                (Rendering|SetVisibility (Variables|Default|GetParticles%201) false true)))))))))

(fn ConstructionScript
  (bind _returnvalue (AddComponent|AddMaterialBillboardComponent false))
  (Variables|Default|SetIcon%20SCU _returnvalue)
  (if (Variables|Properties|GetUsesBaseController)
    (bind _returnvalue_2 (Rendering|Material|CreateDynamicMaterialInstance "/Game/PlanetSide_2/UI/Icons/Materials/MI_Icon_Base_Manual.MI_Icon_Base_Manual" :!class /Script/Engine.KismetMaterialLibrary))
    (bind _output_get (Variables|Default|SetIcon%20Material _returnvalue_2))
    (Rendering|Material|SetMaterial (Variables|Default|GetIcon%20SCU) 0 _output_get)
    (Rendering|Material|SetTextureParameterValue (Variables|Default|GetIcon%20Material) "Texture" "/Game/PlanetSide_2/UI/Icons/Textures/Icon_SCU.Icon_SCU"))
  (Rendering|Debug|FlushPersistentDebugLines)
  (if (Variables|Properties|GetConnection%20Line%20Enabled)
    (for _array_element (Variables|Properties|GetSpawn%20Tube%20Targets)
      (Rendering|Debug|DrawDebugLine (+ (Transformation|GetWorldLocation (Variables|Default|GetSCU)) "0, 0,244.000000") (+ (Transformation|GetActorLocation _array_element) "0, 0,122.000000") "(R=0.056284,G=0.594981,B=1.000000,A=1.000000)" 6e+01 5.0))))