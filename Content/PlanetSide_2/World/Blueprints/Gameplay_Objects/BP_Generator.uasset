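; Hackable base shield generator that drops its ShieldTargets' shields when destroyed and restores them when repaired.
; Within HackingAOE, F starts an overload, stabilizes it or repairs the wreck.
; Overload escalates through three RetriggerableDelay stages of lighting, materials, effects and audio before exploding, reporting changes to BaseController.
; The construction script picks the icon by GeneratorType, and FactionSwitch tints it by faction, filtered by UsesBaseController.
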(event OnComponentBeginOverlap(HackingAOE)
  (params (OverlappedComponent :type Primitive%20Component%20Object%20Reference) (OtherActor :type Actor%20Object%20Reference) (OtherComp :type Primitive%20Component%20Object%20Reference) (OtherBodyIndex :type Integer) (bFromSweep :type Boolean) (SweepResult :type Hit%20Result%20Structure%20%28by%20ref%29))
  (Input|EnableInput (Game|GetPlayerController 0)))

(event OnComponentEndOverlap(HackingAOE)
  (params (OverlappedComponent :type Primitive%20Component%20Object%20Reference) (OtherActor :type Actor%20Object%20Reference) (OtherComp :type Primitive%20Component%20Object%20Reference) (OtherBodyIndex :type Integer))
  (Input|DisableInput (Game|GetPlayerController 0)))

(event Custom|Enable/Disable%20Icons
  (params (Visibility :type Boolean))
  (Rendering|SetVisibility (Variables|Default|GetIcon) Visibility false))

(event Custom|Faction%20Switch
  (params (Faction%20Name :type EFaction%20Enum :default "NewEnumerator3") (FromBaseController :type Boolean))
  (bind (_ns_ui_color _nc_ui_color _tr_ui_color _vs_ui_color) (Utilities|GetClassDefaults "/Game/PlanetSide_2/UI/FactionSwitch.FactionSwitch_C"))
  (bind _icon_material (Variables|Default|GetIcon%20Material))
  (if (not (Class|KismetMathLibrary|XORBoolean FromBaseController (Variables|Generator|GetUsesBaseController)))
    (switch Utilities|FlowControl|Switch|SwitchonEFaction Faction%20Name
      (:NewEnumerator3
        (Rendering|Material|SetVectorParameterValue _icon_material "Color" _ns_ui_color :!class /Script/Engine.MaterialInstanceDynamic))
      (:NewEnumerator0
        (Rendering|Material|SetVectorParameterValue _icon_material "Color" _nc_ui_color :!class /Script/Engine.MaterialInstanceDynamic))
      (:NewEnumerator1
        (Rendering|Material|SetVectorParameterValue _icon_material "Color" _tr_ui_color :!class /Script/Engine.MaterialInstanceDynamic))
      (:NewEnumerator2
        (Rendering|Material|SetVectorParameterValue _icon_material "Color" _vs_ui_color :!class /Script/Engine.MaterialInstanceDynamic)))))

(event Input|KeyboardEvents|F
  (params (Key :type Key%20Structure))
  (bind _light (Variables|Default|GetLight))
  (bind _light_2 (Variables|Default|GetLight))
  (bind _light_3 (Variables|Default|GetLight))
  (bind _light_4 (Variables|Default|GetLight))
  (bind _generatoraudio (Variables|Default|GetGeneratorAudio))
  (:Pressed
    (if (Variables|Default|GetIs%20Destroyed)
      ;[1 1 1] Repair
      (Variables|Default|SetHacked false)
      (Variables|Default|SetIs%20Destroyed false)
      (Default|GeneratorRepaired (Variables|Generator|GetBase%20Controller))
      (Utilities|FlowControl|Sequence
        (:then_0
          (Variables|Default|SetEnable/Disable%20Shields%20Status true)
          (for _array_element (Variables|Generator|GetShield%20Targets)
            (Default|ShieldEnable/Disable _array_element (Variables|Default|GetEnable/Disable%20Shields%20Status))))
        (:then_1
          ;[1 1 1] Generator REset
          (Rendering|SetVisibility _light_4 true true :!label _label)
          (Rendering|SetVisibility (Variables|Default|GetDestroyed%20Generator) false true)
          (Rendering|Components|Light|SetLightFunctionMaterial _light_4 "/Game/PlanetSide_2/Effects/LightFunction/MI_Generator_Light.MI_Generator_Light")
          (Rendering|Components|Light|SetLightColor _light_4 "(R=0.690000,G=0.690000,B=1.000000,A=1.000000)" true)
          (Rendering|Material|SetMaterial (Variables|Default|GetGenerator) 0 "/Game/PlanetSide_2/World/Materials/Gameplay_Objects/MI_Generator.MI_Generator")
          (Effects|Components|ParticleSystem|SetIntParameter _generatoraudio "Generator Damage Level" 0)
          (Audio|Components|Audio|Play _generatoraudio 0.0)))
      (else
        ;[1 1 1] Stabilize
        (if (Variables|Default|GetHacked)
          (Variables|Default|SetHacked false)
          (Variables|Default|SetStabilized true)
          (Default|GeneratorStabilized (Variables|Generator|GetBase%20Controller))
          (goto _label)
          (else
            ;[1 0.6658 0.5002] Generator Overload Sequence
            (Variables|Default|SetStabilized false)
            (Variables|Default|SetHacked true)
            ;;[1 0.9484 0.03201] Stage 1
            (Utilities|FlowControl|Sequence
              (:then_0
                (Default|GeneratorChangeStatus (Variables|Generator|GetBase%20Controller) 1)
                (Effects|Components|ParticleSystem|SetIntParameter (Variables|Default|GetGeneratorAudio) "Generator Damage Level" 1))
              (:then_1
                (Rendering|Components|Light|SetLightFunctionMaterial _light_3 "/Game/PlanetSide_2/Effects/LightFunction/MI_Generator_Light_Critical1.MI_Generator_Light_Critical1")
                (Rendering|Components|Light|SetLightColor _light_3 "(R=1.000000,G=0.773868,B=0.000000,A=1.000000)" true)
                (Rendering|Material|SetMaterial (Variables|Default|GetGenerator) 0 "/Game/PlanetSide_2/World/Materials/Gameplay_Objects/MI_Generator_Critical1.MI_Generator_Critical1")
                (Utilities|FlowControl|RetriggerableDelay 1e+01)
                (if (not (Variables|Default|GetStabilized))
                  ;;[1 0.2877 0.006723] Stage 2
                  (Utilities|FlowControl|Sequence
                    (:then_0
                      (Effects|Components|ParticleSystem|SetIntParameter (Variables|Default|GetGeneratorAudio) "Generator Damage Level" 2)
                      (Default|GeneratorChangeStatus (Variables|Generator|GetBase%20Controller) 2))
                    (:then_1
                      (Rendering|Components|Light|SetLightFunctionMaterial _light "/Game/PlanetSide_2/Effects/LightFunction/MI_Generator_Light_Critical2.MI_Generator_Light_Critical2")
                      (Rendering|Components|Light|SetLightColor _light "(R=1.000000,G=0.277000,B=0.000000,A=1.000000)" true)
                      (Rendering|Material|SetMaterial (Variables|Default|GetGenerator) 0 "/Game/PlanetSide_2/World/Materials/Gameplay_Objects/MI_Generator_Critical2.MI_Generator_Critical2")
                      (Utilities|FlowControl|RetriggerableDelay 2e+01)
                      (if (not (Variables|Default|GetStabilized))
                        ;;[1 0.008924 0] Stage 3
                        (Utilities|FlowControl|Sequence
                          (:then_0
                            (Default|GeneratorChangeStatus (Variables|Generator|GetBase%20Controller) 3)
                            (Effects|Components|ParticleSystem|SetIntParameter (Variables|Default|GetGeneratorAudio) "Generator Damage Level" 3))
                          (:then_1
                            (Rendering|Components|Light|SetLightFunctionMaterial _light_2 "/Game/PlanetSide_2/Effects/LightFunction/MI_Generator_Light_Critical3.MI_Generator_Light_Critical3")
                            (Rendering|Components|Light|SetLightColor _light_2 "(R=1.000000,G=0.000000,B=0.000000,A=1.000000)" true)
                            (Rendering|Material|SetMaterial (Variables|Default|GetGenerator) 0 "/Game/PlanetSide_2/World/Materials/Gameplay_Objects/MI_Generator_Critical3.MI_Generator_Critical3")
                            (Utilities|FlowControl|RetriggerableDelay 1e+01)
                            (if (not (Variables|Default|GetStabilized))
                              ;;[1 1 1] Destroy Generator
                              (Utilities|FlowControl|Sequence
                                (:then_0
                                  (Default|GeneratorDestroyed (Variables|Generator|GetBase%20Controller))
                                  (Audio|Components|Audio|Stop (Variables|Default|GetGeneratorAudio))
                                  (Audio|Components|Audio|Play (Variables|Default|GetExplode) 0.0)
                                  (Variables|Default|SetEnable/Disable%20Shields%20Status false)
                                  (for _array_element_2 (Variables|Generator|GetShield%20Targets)
                                    (Default|ShieldEnable/Disable _array_element_2 (Variables|Default|GetEnable/Disable%20Shields%20Status))))
                                (:then_1
                                  (Variables|Default|SetIs%20Destroyed true)
                                  (Rendering|SetVisibility (Variables|Default|GetLight) false true)
                                  (Rendering|SetVisibility (Variables|Default|GetDestroyed%20Generator) true false)
                                  (Components|Activation|Activate (Variables|Default|GetExplosion) false)
                                  (Development|PrintString "Generator Destroyed" true true "(R=1.000000,G=0.000000,B=0.000000,A=1.000000)")))))
                          (:then_2
                            (Rendering|SetVisibility (Variables|Default|GetFire%202) true true)
                            (Rendering|SetVisibility (Variables|Default|GetParticles%203) false true)))))
                    (:then_2
                      (Rendering|SetVisibility (Variables|Default|GetFire%201) true true)
                      (Rendering|SetVisibility (Variables|Default|GetParticles%202) false true)))))
              (:then_2
                (Rendering|SetVisibility (Variables|Default|GetSmoke) true true)
                (Rendering|SetVisibility (Variables|Default|GetParticles%201) false true)))))))))

(fn ConstructionScript
  (bind _icon (Variables|Default|GetIcon))
  (if (Variables|Generator|GetUsesBaseController)
    (bind _returnvalue (Rendering|Material|CreateDynamicMaterialInstance "/Game/PlanetSide_2/UI/Icons/Materials/MI_Icon_Base_Manual.MI_Icon_Base_Manual" "None" :!class /Script/Engine.KismetMaterialLibrary))
    (bind _output_get (Variables|Default|SetIcon%20Material _returnvalue))
    (Rendering|Material|SetMaterial (Variables|Default|GetIcon) 0 _output_get)
    (switch int (Variables|Generator|GetGenerator%20Type)
      (:1
        (Rendering|Material|SetTextureParameterValue (Variables|Default|GetIcon%20Material) "Texture" "/Game/PlanetSide_2/UI/Icons/Textures/Icon_Vehicle_Shield.Icon_Vehicle_Shield"))
      (:2
        (Rendering|Material|SetTextureParameterValue (Variables|Default|GetIcon%20Material) "Texture" "/Game/PlanetSide_2/UI/Icons/Textures/Icon_Horizontal_Shield.Icon_Horizontal_Shield"))
      (:3
        (Rendering|Material|SetTextureParameterValue (Variables|Default|GetIcon%20Material) "Texture" "/Game/PlanetSide_2/UI/Icons/Textures/Icon_Vertical_Shield.Icon_Vertical_Shield"))
      (:4
        (Rendering|Material|SetTextureParameterValue (Variables|Default|GetIcon%20Material) "Texture" "/Game/PlanetSide_2/UI/Icons/Textures/Icon_SCU_Shield.Icon_SCU_Shield")))
    (else
      (switch int (Variables|Generator|GetGenerator%20Type)
        (:1
          (Rendering|Material|SetMaterial _icon 0 "/Game/PlanetSide_2/UI/Icons/Materials/Icon_Shield_Vehicle.Icon_Shield_Vehicle"))
        (:2
          (Rendering|Material|SetMaterial _icon 0 "/Game/PlanetSide_2/UI/Icons/Materials/Icon_Shield_Horizontal.Icon_Shield_Horizontal"))
        (:3
          (Rendering|Material|SetMaterial _icon 0 "/Game/PlanetSide_2/UI/Icons/Materials/Icon_Shield_Vertical.Icon_Shield_Vertical"))
        (:4
          (Rendering|Material|SetMaterial _icon 0 "/Game/PlanetSide_2/UI/Icons/Materials/Icon_Shield_SCU.Icon_Shield_SCU"))))))

(fn CastingtoShieldTargets
  (params (Shield%20Enabled :type Boolean) (Target%20Types :type Array%20of%20Integers) (Actors :type Array%20of%20Actor%20Object%20References))
  (for _array_element Actors
    (for _array_element_2 Target%20Types
      (switch int _array_element_2
        (:1
          (bind _asbp_warpgate (Utilities|Casting|CastToBP_Warpgate _array_element))
          (Default|ShieldEnable/Disable _asbp_warpgate Shield%20Enabled))
        (:2
          (bind _asbp_biolab (Utilities|Casting|CastToBP_Biolab _array_element :!label _label))
          (Default|ShieldEnable/Disable _asbp_biolab Shield%20Enabled))
        (:3
          (bind _asbp_biolab_2 (Utilities|Casting|CastToBP_Biolab _array_element :!label _label_2))
          (Default|SCUShieldDisable _asbp_biolab_2 Shield%20Enabled)
          (bind _asbp_amp_station (Utilities|Casting|CastToBP_AmpStation _array_element))
          (Default|SCUShieldDisable _asbp_amp_station Shield%20Enabled))
        (:4
          (bind _asbp_biolab_3 (Utilities|Casting|CastToBP_Biolab _array_element :!label _label_3))
          (Default|VehicleShieldDsiable _asbp_biolab_3 Shield%20Enabled)
          (bind _asbp_tech_plant (Utilities|Casting|CastToBP_TechPlant _array_element))
          (Default|VehicleShieldDsiable _asbp_tech_plant Shield%20Enabled)
          (bind _asbp_amp_station_2 (Utilities|Casting|CastToBP_AmpStation _array_element))
          (Default|VehicleShieldDsiable _asbp_amp_station_2 Shield%20Enabled))
        (:5
          (Utilities|FlowControl|Sequence
            (:then_0
              (goto _label))
            (:then_1
              (goto _label_2))
            (:then_2
              (goto _label_3))))
        (:6
          (Utilities|FlowControl|Sequence
            (:then_0
              (goto _label_2))
            (:then_1
              (goto _label_3))))))))