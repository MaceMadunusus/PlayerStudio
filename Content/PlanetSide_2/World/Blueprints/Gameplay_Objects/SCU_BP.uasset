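; Spawn Control Unit that players can overload, stabilize or repair, controlling whether its linked spawn tubes work.
; Overlapping HackingAOE enables player 0's input, and F picks the action from the Hacked and IsDestroyed flags.
; Overload escalates through three stages of lights, materials, loops and effects via RetriggerableDelays, each checking Stabilized before continuing.
; Destruction swaps in the wreck and disables SpawnTubeTargets; repair re-enables them and shares the visual reset with stabilizing.
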(event OnComponentBeginOverlap(HackingAOE)
  (params (OtherActor :type Actor%20Object%20Reference) (OtherComp :type Primitive%20Component%20Object%20Reference) (OtherBodyIndex :type Integer) (bFromSweep :type Boolean) (SweepResult :type Hit%20Result%20Structure%20%28by%20ref%29))
  (Input|EnableInput (Game|GetPlayerController 0)))

(event OnComponentEndOverlap(HackingAOE)
  (params (OtherActor :type Actor%20Object%20Reference) (OtherComp :type Primitive%20Component%20Object%20Reference) (OtherBodyIndex :type Integer))
  (Input|DisableInput (Game|GetPlayerController 0)))

(event Input|KeyboardEvents|F
  (bind _light (Variables|Default|GetLight))
  (bind _light_2 (Variables|Default|GetLight))
  (bind _light_3 (Variables|Default|GetLight))
  (bind _light_4 (Variables|Default|GetLight))
  (:Pressed
    (if (Variables|Default|GetIs%20Destroyed)
      ;[1 1 1] Repair
      (Variables|Default|SetHacked false)
      (Variables|Default|SetIs%20Destroyed false)
      (Audio|PlaySoundatLocation "/Game/PlanetSide_2/Audio/Computer/DX_COMPUTER_SCU_REPAIRED_Cue.DX_COMPUTER_SCU_REPAIRED_Cue" "0, 0, 0")
      (Development|PrintString "SCU Repaired" true true "(R=0.000000,G=0.714328,B=1.000000,A=1.000000)")
      (Utilities|FlowControl|Sequence
        (:then_0
          (for _array_element (Variables|Properties|GetSpawn%20Tube%20Targets)
            (bind _asspawn_tube_blueprint (Utilities|Casting|CastToSpawnTube_Blueprint _array_element))
            (Default|SpawnTubeEnable/Disable _asspawn_tube_blueprint true)))
        (:then_1
          ;[1 1 1] Generator REset
          (Rendering|SetVisibility _light_4 true true :!label _label)
          (Rendering|SetVisibility (Variables|Default|GetDestroyed%20SCU) false true)
          (Rendering|Components|Light|SetLightFunctionMaterial _light_4 "/Game/PlanetSide_2/World/Materials/LightFunction/Generator_Light_Inst.Generator_Light_Inst")
          (Rendering|Components|Light|SetLightColor _light_4 "(R=0.690000,G=0.690000,B=1.000000,A=1.000000)")
          (Rendering|Material|SetMaterial (Variables|Default|GetSCU) 0 "/Game/PlanetSide_2/World/Materials/Gameplay_Objects/SpawnControlUnit_Inst.SpawnControlUnit_Inst")
          (Audio|Components|Audio|Stop (Variables|Default|GetOverload%201%20Loop))
          (Audio|Components|Audio|Play (Variables|Default|GetIdle%20Loop) 0.0)))
      (else
        ;[1 1 1] Stabilize
        (if (Variables|Default|GetHacked)
          (Variables|Default|SetHacked false)
          (Variables|Default|SetStabilized true)
          (Audio|PlaySoundatLocation "/Game/PlanetSide_2/Audio/Computer/DX_COMPUTER_SCU_STABILIZED_Cue.DX_COMPUTER_SCU_STABILIZED_Cue" "0, 0, 0")
          (Development|PrintString "SCU Stabilized" true true "(R=0.000000,G=0.714000,B=1.000000,A=1.000000)")
          (goto _label)
          (else
            ;[1 0.6658 0.5002] Generator Overload Sequence
            (Variables|Default|SetStabilized false)
            (Variables|Default|SetHacked true)
            ;;[1 0.9484 0.03201] Stage 1
            (Utilities|FlowControl|Sequence
              (:then_0
                (Audio|PlaySoundatLocation "/Game/PlanetSide_2/Audio/Computer/DX_COMPUTER_SCU_COMPROMISED_Cue.DX_COMPUTER_SCU_COMPROMISED_Cue" "0, 0, 0")
                (Audio|Components|Audio|Play (Variables|Default|GetOverload%201%20Loop) 0.0)
                (Audio|Components|Audio|Stop (Variables|Default|GetIdle%20Loop)))
              (:then_1
                (Rendering|Components|Light|SetLightFunctionMaterial _light_3 "/Game/PlanetSide_2/World/Materials/LightFunction/Generator_Light_Inst_Critical1.Generator_Light_Inst_Critical1")
                (Rendering|Components|Light|SetLightColor _light_3 "(R=1.000000,G=0.773868,B=0.000000,A=1.000000)")
                (Rendering|Material|SetMaterial (Variables|Default|GetSCU) 0 "/Game/PlanetSide_2/World/Materials/Gameplay_Objects/SCU_Critical1.SCU_Critical1")
                (Utilities|FlowControl|RetriggerableDelay 1e+01)
                (if (not (Variables|Default|GetStabilized))
                  ;;[1 0.2877 0.006723] Stage 2
                  (Utilities|FlowControl|Sequence
                    (:then_0
                      (Audio|Components|Audio|Play (Variables|Default|GetOverload%202%20Loop) 0.0)
                      (Audio|Components|Audio|Stop (Variables|Default|GetOverload%201%20Loop)))
                    (:then_1
                      (Rendering|Components|Light|SetLightFunctionMaterial _light "/Game/PlanetSide_2/World/Materials/LightFunction/Generator_Light_Inst_Critical2.Generator_Light_Inst_Critical2")
                      (Rendering|Components|Light|SetLightColor _light "(R=1.000000,G=0.277000,B=0.000000,A=1.000000)")
                      (Rendering|Material|SetMaterial (Variables|Default|GetSCU) 0 "/Game/PlanetSide_2/World/Materials/Gameplay_Objects/SCU_Critical2.SCU_Critical2")
                      (Utilities|FlowControl|RetriggerableDelay 2e+01)
                      (if (not (Variables|Default|GetStabilized))
                        ;;[1 0.008924 0] Stage 3
                        (Utilities|FlowControl|Sequence
                          (:then_0
                            (Audio|PlaySoundatLocation "/Game/PlanetSide_2/Audio/Computer/DX_COMPUTER_SCU_CRITICAL_Cue.DX_COMPUTER_SCU_CRITICAL_Cue" "0, 0, 0")
                            (Audio|Components|Audio|Play (Variables|Default|GetOverload%203%20Loop) 0.0)
                            (Audio|Components|Audio|Stop (Variables|Default|GetOverload%202%20Loop)))
                          (:then_1
                            (Rendering|Components|Light|SetLightFunctionMaterial _light_2 "/Game/PlanetSide_2/World/Materials/LightFunction/Generator_Light_Inst_Critical3.Generator_Light_Inst_Critical3")
                            (Rendering|Components|Light|SetLightColor _light_2 "(R=1.000000,G=0.000000,B=0.000000,A=1.000000)")
                            (Rendering|Material|SetMaterial (Variables|Default|GetSCU) 0 "/Game/PlanetSide_2/World/Materials/Gameplay_Objects/SCU_Critical3.SCU_Critical3")
                            (Utilities|FlowControl|RetriggerableDelay 1e+01)
                            (if (not (Variables|Default|GetStabilized))
                              ;;[1 1 1] Destroy Generator
                              (Utilities|FlowControl|Sequence
                                (:then_0
                                  (Audio|PlaySoundatLocation "/Game/PlanetSide_2/Audio/Computer/DX_COMPUTER_SCU_DESTROYED_Cue.DX_COMPUTER_SCU_DESTROYED_Cue" "0, 0, 0")
                                  (Audio|Components|Audio|Stop (Variables|Default|GetOverload%203%20Loop))
                                  (Audio|Components|Audio|Play (Variables|Default|GetExplode) 0.0)
                                  (for _array_element_2 (Variables|Properties|GetSpawn%20Tube%20Targets)
                                    (bind _asspawn_tube_blueprint_2 (Utilities|Casting|CastToSpawnTube_Blueprint _array_element_2))
                                    (Default|SpawnTubeEnable/Disable _asspawn_tube_blueprint_2 false)))
                                (:then_1
                                  (Variables|Default|SetIs%20Destroyed true)
                                  (Rendering|SetVisibility (Variables|Default|GetLight) false true)
                                  (Rendering|SetVisibility (Variables|Default|GetDestroyed%20SCU) true false)
                                  (Components|Activation|Activate (Variables|Default|GetExplosion) false)
                                  (Development|PrintString "SCU Destroyed" true true "(R=1.000000,G=0.000000,B=0.000000,A=1.000000)")))))
                          (:then_2
                            (Rendering|SetVisibility (Variables|Default|GetFire%202) true true)
                            (Rendering|SetVisibility (Variables|Default|GetParticles%203) false true)
                            (Development|PrintString "SCU Overloading: Stage 3" true true "(R=1.000000,G=0.000000,B=0.000000,A=1.000000)")))))
                    (:then_2
                      (Rendering|SetVisibility (Variables|Default|GetFire%201) true true)
                      (Rendering|SetVisibility (Variables|Default|GetParticles%202) false true)
                      (Development|PrintString "SCU Overloading: Stage 2" true true "(R=1.000000,G=0.000000,B=0.000000,A=1.000000)")))))
              (:then_2
                (Rendering|SetVisibility (Variables|Default|GetSmoke) true true)
                (Rendering|SetVisibility (Variables|Default|GetParticles%201) false true)
                (Development|PrintString "SCU Overloading: Stage 1" true true "(R=1.000000,G=0.000000,B=0.000000,A=1.000000)")))))))))

(fn ConstructionScript)