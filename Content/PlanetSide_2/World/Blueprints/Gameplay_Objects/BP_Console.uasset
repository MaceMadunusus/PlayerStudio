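; BP_Console is a faction-switchable terminal for equipment, vehicle, aircraft and warpgate types, with a screen material, icon and light.
; The construction script picks the icon by ConsoleType, using a dynamic material for base-controlled consoles, and defaults to Nanite Systems visuals.
; FactionSwitch, filtered by matching base-controller flag, updates FactionAccess and recolors it through the shared ConsoleTypeSelect macro.
; Other events toggle icon visibility and draw a debug line to VehiclePadTarget.
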(event Custom|Enable/Disable%20Icons
  (params (Visibility :type Boolean))
  (Rendering|SetVisibility (Variables|Default|GetIcon) Visibility false))

(event Custom|Faction%20Switch
  (params (Faction%20Name :type EFaction%20Enum) (FromBaseController :type Boolean))
  (if (not (Class|KismetMathLibrary|XORBoolean FromBaseController (Variables|Properties|GetUsesBaseController)))
    (switch Utilities|FlowControl|Switch|SwitchonEFaction Faction%20Name
      (:NewEnumerator3
        (Utilities|ConsoleTypeSelect "/Game/PlanetSide_2/World/Materials/Gameplay_Objects/Console/Console_NS3.Console_NS3" "/Game/PlanetSide_2/World/Materials/Gameplay_Objects/Console/Console_NS6.Console_NS6" "/Game/PlanetSide_2/World/Materials/Gameplay_Objects/Console/Console_NS5.Console_NS5" "/Game/PlanetSide_2/World/Materials/Gameplay_Objects/Console/Console_NS4.Console_NS4" "/Game/PlanetSide_2/World/Materials/Gameplay_Objects/Console/Console_NS7.Console_NS7" "/Game/PlanetSide_2/World/Materials/Gameplay_Objects/Console/Console_NS1.Console_NS1" "/Game/PlanetSide_2/World/Materials/Gameplay_Objects/Console/Console_NS2.Console_NS2" "/Game/PlanetSide_2/World/Materials/Gameplay_Objects/Console/Console_NS8.Console_NS8" (Variables|Default|GetLight%20Color)
          (:Result
            (Variables|Default|SetFaction%20Access "NewEnumerator3")
            (Rendering|Material|SetVectorParameterValue (Variables|Default|GetIcon%20Material) "Color" (Utilities|GetClassDefaults "/Game/PlanetSide_2/UI/FactionSwitch.FactionSwitch_C") :!class /Script/Engine.MaterialInstanceDynamic))))
      (:NewEnumerator0
        (Utilities|ConsoleTypeSelect "/Game/PlanetSide_2/World/Materials/Gameplay_Objects/Console/Console_NC3.Console_NC3" "/Game/PlanetSide_2/World/Materials/Gameplay_Objects/Console/Console_NC6.Console_NC6" "/Game/PlanetSide_2/World/Materials/Gameplay_Objects/Console/Console_NC5.Console_NC5" "/Game/PlanetSide_2/World/Materials/Gameplay_Objects/Console/Console_NC4.Console_NC4" "/Game/PlanetSide_2/World/Materials/Gameplay_Objects/Console/Console_NC7.Console_NC7" "/Game/PlanetSide_2/World/Materials/Gameplay_Objects/Console/Console_NC1.Console_NC1" "/Game/PlanetSide_2/World/Materials/Gameplay_Objects/Console/Console_NC2.Console_NC2" "/Game/PlanetSide_2/World/Materials/Gameplay_Objects/Console/Console_NC8.Console_NC8" (Variables|Default|GetLight%20Color%20NC)
          (:Result
            (Variables|Default|SetFaction%20Access "NewEnumerator0")
            (Rendering|Material|SetVectorParameterValue (Variables|Default|GetIcon%20Material) "Color" (Utilities|GetClassDefaults "/Game/PlanetSide_2/UI/FactionSwitch.FactionSwitch_C") :!class /Script/Engine.MaterialInstanceDynamic))))
      (:NewEnumerator1
        (Utilities|ConsoleTypeSelect "/Game/PlanetSide_2/World/Materials/Gameplay_Objects/Console/Console_TR3.Console_TR3" "/Game/PlanetSide_2/World/Materials/Gameplay_Objects/Console/Console_TR6.Console_TR6" "/Game/PlanetSide_2/World/Materials/Gameplay_Objects/Console/Console_TR5.Console_TR5" "/Game/PlanetSide_2/World/Materials/Gameplay_Objects/Console/Console_TR4.Console_TR4" "/Game/PlanetSide_2/World/Materials/Gameplay_Objects/Console/Console_TR7.Console_TR7" "/Game/PlanetSide_2/World/Materials/Gameplay_Objects/Console/Console_TR1.Console_TR1" "/Game/PlanetSide_2/World/Materials/Gameplay_Objects/Console/Console_TR2.Console_TR2" "/Game/PlanetSide_2/World/Materials/Gameplay_Objects/Console/Console_TR8.Console_TR8" (Variables|Default|GetLight%20Color%20TR)
          (:Result
            (Variables|Default|SetFaction%20Access "NewEnumerator1")
            (Rendering|Material|SetVectorParameterValue (Variables|Default|GetIcon%20Material) "Color" (Utilities|GetClassDefaults "/Game/PlanetSide_2/UI/FactionSwitch.FactionSwitch_C") :!class /Script/Engine.MaterialInstanceDynamic))))
      (:NewEnumerator2
        (Utilities|ConsoleTypeSelect "/Game/PlanetSide_2/World/Materials/Gameplay_Objects/Console/Console_VS3.Console_VS3" "/Game/PlanetSide_2/World/Materials/Gameplay_Objects/Console/Console_VS6.Console_VS6" "/Game/PlanetSide_2/World/Materials/Gameplay_Objects/Console/Console_VS5.Console_VS5" "/Game/PlanetSide_2/World/Materials/Gameplay_Objects/Console/Console_VS4.Console_VS4" "/Game/PlanetSide_2/World/Materials/Gameplay_Objects/Console/Console_VS7.Console_VS7" "/Game/PlanetSide_2/World/Materials/Gameplay_Objects/Console/Console_VS1.Console_VS1" "/Game/PlanetSide_2/World/Materials/Gameplay_Objects/Console/Console_VS2.Console_VS2" "/Game/PlanetSide_2/World/Materials/Gameplay_Objects/Console/Console_VS8.Console_VS8" (Variables|Default|GetLight%20Color%20VS)
          (:Result
            (Variables|Default|SetFaction%20Access "NewEnumerator2")
            (Rendering|Material|SetVectorParameterValue (Variables|Default|GetIcon%20Material) "Color" (Utilities|GetClassDefaults "/Game/PlanetSide_2/UI/FactionSwitch.FactionSwitch_C") :!class /Script/Engine.MaterialInstanceDynamic)))))))

(event Custom|Display%20Connection%20Lines
  (bind _vehiclepadtarget (Variables|Properties|GetVehiclePadTarget))
  (Utilities|IsValid _vehiclepadtarget
    (:Is%20Valid
      (Rendering|Debug|DrawDebugLine (+ (Transformation|GetWorldLocation (Variables|Default|GetConsole)) "0, 0,200.000000") (+ (Transformation|GetActorLocation _vehiclepadtarget) "0, 0,200.000000") "(R=1.000000,G=1.000000,B=0.000000,A=1.000000)" 6e+01 5.0))))

(fn ConstructionScript
  (bind _icon (Variables|Default|GetIcon))
  (if (Variables|Properties|GetUsesBaseController)
    (bind _returnvalue (Rendering|Material|CreateDynamicMaterialInstance "/Game/PlanetSide_2/UI/Icons/Materials/MI_Icon_Base_Manual.MI_Icon_Base_Manual" :!class /Script/Engine.KismetMaterialLibrary))
    (bind _output_get (Variables|Default|SetIcon%20Material _returnvalue))
    (Rendering|Material|SetMaterial (Variables|Default|GetIcon) 0 _output_get)
    (Utilities|FlowControl|Sequence
      (:then_0
        (switch Utilities|FlowControl|Switch|SwitchonConsoleType (Variables|Properties|GetConsole%20Type)
          (:NewEnumerator0
            (Rendering|Material|SetTextureParameterValue (Variables|Default|GetIcon%20Material) "Texture" "/Game/PlanetSide_2/UI/Icons/Textures/Icon_Infantry_Terminal.Icon_Infantry_Terminal"))
          (:NewEnumerator1
            (Rendering|Material|SetTextureParameterValue (Variables|Default|GetIcon%20Material) "Texture" "/Game/PlanetSide_2/UI/Icons/Textures/Icon_Flash_Terminal.Icon_Flash_Terminal"))
          (:NewEnumerator2
            (Rendering|Material|SetTextureParameterValue (Variables|Default|GetIcon%20Material) "Texture" "/Game/PlanetSide_2/UI/Icons/Textures/Icon_Lightning_Terminal.Icon_Lightning_Terminal"))
          (:NewEnumerator3
            (Rendering|Material|SetTextureParameterValue (Variables|Default|GetIcon%20Material) "Texture" "/Game/PlanetSide_2/UI/Icons/Textures/Icon_Vehicle_Terminal.Icon_Vehicle_Terminal"))
          (:NewEnumerator4
            (Rendering|Material|SetTextureParameterValue (Variables|Default|GetIcon%20Material) "Texture" "/Game/PlanetSide_2/UI/Icons/Textures/Icon_Sunderer_Terminal.Icon_Sunderer_Terminal"))
          (:NewEnumerator5
            (Rendering|Material|SetTextureParameterValue (Variables|Default|GetIcon%20Material) "Texture" "/Game/PlanetSide_2/UI/Icons/Textures/Icon_Aircraft_Terminal.Icon_Aircraft_Terminal"))
          (:NewEnumerator6
            (Rendering|Material|SetTextureParameterValue (Variables|Default|GetIcon%20Material) "Texture" "/Game/PlanetSide_2/UI/Icons/Textures/Icon_Galaxy_Terminal.Icon_Galaxy_Terminal"))
          (:NewEnumerator8
            (Rendering|Material|SetTextureParameterValue (Variables|Default|GetIcon%20Material) "Texture" "/Game/PlanetSide_2/UI/Icons/Textures/Icon_Warpgate_Terminal.Icon_Warpgate_Terminal"))))
      (:then_1
        (Utilities|ConsoleTypeSelect "/Game/PlanetSide_2/World/Materials/Gameplay_Objects/Console/Console_NS3.Console_NS3" "/Game/PlanetSide_2/World/Materials/Gameplay_Objects/Console/Console_NS6.Console_NS6" "/Game/PlanetSide_2/World/Materials/Gameplay_Objects/Console/Console_NS5.Console_NS5" "/Game/PlanetSide_2/World/Materials/Gameplay_Objects/Console/Console_NS4.Console_NS4" "/Game/PlanetSide_2/World/Materials/Gameplay_Objects/Console/Console_NS7.Console_NS7" "/Game/PlanetSide_2/World/Materials/Gameplay_Objects/Console/Console_NS1.Console_NS1" "/Game/PlanetSide_2/World/Materials/Gameplay_Objects/Console/Console_NS2.Console_NS2" "/Game/PlanetSide_2/World/Materials/Gameplay_Objects/Console/Console_NS8.Console_NS8" :!label _label))
      (:then_2
        (Rendering|Components|Light|SetLightColor (Variables|Default|GetLight) (Variables|Default|GetLight%20Color) true :!label _label_2)))
    (else
      (Utilities|FlowControl|Sequence
        (:then_0
          (switch Utilities|FlowControl|Switch|SwitchonConsoleType (Variables|Properties|GetConsole%20Type)
            (:NewEnumerator0
              (Rendering|Material|SetMaterial _icon 0 "/Game/PlanetSide_2/UI/Icons/Materials/Icon_Infantry.Icon_Infantry"))
            (:NewEnumerator1
              (Rendering|Material|SetMaterial _icon 0 "/Game/PlanetSide_2/UI/Icons/Materials/Icon_Flash.Icon_Flash"))
            (:NewEnumerator2
              (Rendering|Material|SetMaterial _icon 0 "/Game/PlanetSide_2/UI/Icons/Materials/Icon_Lightning.Icon_Lightning"))
            (:NewEnumerator3
              (Rendering|Material|SetMaterial _icon 0 "/Game/PlanetSide_2/UI/Icons/Materials/Icon_Vehicle.Icon_Vehicle"))
            (:NewEnumerator4
              (Rendering|Material|SetMaterial _icon 0 "/Game/PlanetSide_2/UI/Icons/Materials/Icon_Infantry.Icon_Infantry"))
            (:NewEnumerator5
              (Rendering|Material|SetMaterial _icon 0 "/Game/PlanetSide_2/UI/Icons/Materials/Icon_Infantry.Icon_Infantry"))
            (:NewEnumerator6
              (Rendering|Material|SetMaterial _icon 0 "/Game/PlanetSide_2/UI/Icons/Materials/Icon_Infantry.Icon_Infantry"))
            (:NewEnumerator8
              (Rendering|Material|SetMaterial _icon 0 "/Game/PlanetSide_2/UI/Icons/Materials/Icon_Infantry.Icon_Infantry"))))
        (:then_1
          (goto _label))
        (:then_2
          (goto _label_2))))))