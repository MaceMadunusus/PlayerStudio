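; BP_CommandConsole is a capture point console that recolors its screen material, light and icon for each of four factions.
; FactionSwitch applies only when its FromBaseController flag matches UsesBaseController.
; Overlapping the radius starts a five-second timer, cancelled on leaving, that marks the point captured and plays a sound.
; A DoOnce then starts a sixty-second Capture Base timer, which resets the captured state without changing faction.
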(event OnComponentBeginOverlap(CaptureRadius)
  (params (OtherActor :type Actor%20Object%20Reference) (OtherComp :type Primitive%20Component%20Object%20Reference) (OtherBodyIndex :type Integer) (bFromSweep :type Boolean) (SweepResult :type Hit%20Result%20Structure%20%28by%20ref%29))
  (bind _returnvalue (Utilities|Time|SetTimerbyFunctionName 0 "Capture Point" 5.0))
  (Variables|Default|SetCaptureBaseTimer _returnvalue))

(event OnComponentEndOverlap(CaptureRadius)
  (params (OtherActor :type Actor%20Object%20Reference) (OtherComp :type Primitive%20Component%20Object%20Reference) (OtherBodyIndex :type Integer))
  (if (not (Variables|Default|GetCaptured))
    (Class|KismetSystemLibrary|ClearTimerHandle (Variables|Default|GetCaptureBaseTimer))))

(event Custom|Enable/Disable%20Icons
  (params (Visibility :type Boolean))
  (Rendering|SetVisibility (Variables|Default|GetIcon) Visibility false))

(event Custom|Capture%20Point
  (Variables|Default|SetCaptured true)
  (Audio|PlaySoundatLocation "/Game/PlanetSide_2/Audio/UI/UI_WHISPER_NOTIFICATION.UI_WHISPER_NOTIFICATION" "0, 0, 0")
  (Utilities|FlowControl|DoOnce false
    (:Completed
      (Utilities|Time|SetTimerbyFunctionName 0 "Capture Base" 6e+01))))

(event Custom|Capture%20Base
  (Variables|Default|SetCaptured false)
  (Class|KismetSystemLibrary|ClearTimerHandle (Variables|Default|GetCaptureBaseTimer))
  (Utilities|FlowControl|Sequence
    (:then_1
      (Utilities|FlowControl|DoOnce false) ; enters at Reset
    )))

(event Custom|Faction%20Switch
  (params (Faction :type EFaction%20Enum) (FromBaseController :type Boolean))
  (bind (_ns_ui_color _nc_ui_color _tr_ui_color _vs_ui_color) (Utilities|GetClassDefaults "/Game/PlanetSide_2/UI/FactionSwitch.FactionSwitch_C"))
  (bind _light (Variables|Default|GetLight))
  (bind _console (Variables|Default|GetConsole))
  (bind _icon_material (Variables|Default|GetIcon%20Material))
  (if (not (Class|KismetMathLibrary|XORBoolean FromBaseController (Variables|Properties|GetUsesBaseController)))
    (switch Utilities|FlowControl|Switch|SwitchonEFaction Faction
      (:NewEnumerator3
        (Rendering|Material|SetMaterial _console 1 "/Game/PlanetSide_2/World/Materials/Gameplay_Objects/Console/Commandconsole_NS.CommandConsole_NS")
        (Rendering|Components|Light|SetLightColor _light (Variables|Default|GetLight%20Color%20NS) true)
        (Rendering|Material|SetVectorParameterValue _icon_material "Color" _ns_ui_color :!class /Script/Engine.MaterialInstanceDynamic))
      (:NewEnumerator0
        (Rendering|Material|SetMaterial _console 1 "/Game/PlanetSide_2/World/Materials/Gameplay_Objects/Console/Commandconsole_NC.CommandConsole_NC")
        (Rendering|Components|Light|SetLightColor _light (Variables|Default|GetLight%20Color%20NC) true)
        (Rendering|Material|SetVectorParameterValue _icon_material "Color" _nc_ui_color :!class /Script/Engine.MaterialInstanceDynamic))
      (:NewEnumerator1
        (Rendering|Material|SetMaterial _console 1 "/Game/PlanetSide_2/World/Materials/Gameplay_Objects/Console/Commandconsole_TR.CommandConsole_TR")
        (Rendering|Components|Light|SetLightColor _light (Variables|Default|GetLight%20Color%20TR) true)
        (Rendering|Material|SetVectorParameterValue _icon_material "Color" _tr_ui_color :!class /Script/Engine.MaterialInstanceDynamic))
      (:NewEnumerator2
        (Rendering|Material|SetMaterial _console 1 "/Game/PlanetSide_2/World/Materials/Gameplay_Objects/Console/Commandconsole_VS.CommandConsole_VS")
        (Rendering|Components|Light|SetLightColor _light (Variables|Default|GetLight%20Color%20VS) true)
        (Rendering|Material|SetVectorParameterValue _icon_material "Color" _vs_ui_color :!class /Script/Engine.MaterialInstanceDynamic)))))

(fn ConstructionScript
  (bind _returnvalue (Rendering|Material|CreateDynamicMaterialInstance (Variables|Default|GetIcon) 0 "/Game/PlanetSide_2/UI/Icons/Materials/MI_Icon_Base_Manual.MI_Icon_Base_Manual" :!class /Script/Engine.PrimitiveComponent))
  (Variables|Default|SetIcon%20Material _returnvalue)
  (switch Utilities|FlowControl|Switch|SwitchonCapturePoint (Variables|Properties|GetLetter)
    (:NewEnumerator0
      _)
    (:NewEnumerator1
      _)
    (:NewEnumerator2
      _)
    (:NewEnumerator3
      _)
    (:NewEnumerator4
      _)
    (:NewEnumerator5
      _))
  (Rendering|Material|SetTextureParameterValue (Variables|Default|GetIcon%20Material) "Texture" "/Game/PlanetSide_2/UI/Icons/Textures/Icon_CapturePoint.Icon_CapturePoint"))