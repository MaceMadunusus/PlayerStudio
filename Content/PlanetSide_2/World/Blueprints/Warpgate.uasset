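; Warpgate world actor whose shield, stands, core and arms take the colours of its owning faction (NS, NC, TR or VS).
; The construction script applies the material set for the FAction variable, so placed instances show their faction.
; The FactionSwitch event stores a new faction and reapplies materials through a duplicated copy of that switch.
; A separate event toggles shield visibility, including its child components.
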(event Custom|Shield%20Enable/Disable
  (params (Shield%20Enabled :type Boolean))
  (Rendering|SetVisibility (Variables|Default|GetShield) Shield%20Enabled true))

(event Custom|Faction%20Switch
  (params (Faction%20Name :type Name))
  (bind _shield (Variables|Default|GetShield))
  (bind _stand1 (Variables|Default|GetStand1))
  (bind _core (Variables|Default|GetCore))
  (bind _arm1 (Variables|Default|GetArm1))
  (bind _stand1_2 (Variables|Default|GetStand1))
  (bind _core_2 (Variables|Default|GetCore))
  (bind _arm1_2 (Variables|Default|GetArm1))
  (bind _stand1_3 (Variables|Default|GetStand1))
  (bind _core_3 (Variables|Default|GetCore))
  (bind _arm1_3 (Variables|Default|GetArm1))
  (bind _stand1_4 (Variables|Default|GetStand1))
  (bind _core_4 (Variables|Default|GetCore))
  (bind _arm1_4 (Variables|Default|GetArm1))
  (Variables|Default|SetFAction Faction%20Name)
  (switch name (Variables|Default|GetFAction)
    (:NS
      (Rendering|Material|SetMaterial _shield 0 "/Game/PlanetSide_2/World/Materials/Warpgate/Shield_Inst.Shield_Inst")
      (Rendering|Material|SetMaterial _stand1_2 0 "/Game/PlanetSide_2/World/Materials/Warpgate/Warpgate_Reduced_Mat.Warpgate_Reduced_Mat")
      (Rendering|Material|SetMaterial _stand1_2 1 "/Game/PlanetSide_2/World/Materials/Warpgate/Hex_Tile_Pulse.Hex_Tile_Pulse")
      (Rendering|Material|SetMaterial _stand1_2 2 "/Game/PlanetSide_2/World/Materials/Warpgate/Warpgate_Pulse_C_Mat.Warpgate_Pulse_C_Mat")
      (Rendering|Material|SetMaterial _stand1_2 3 "/Game/PlanetSide_2/World/Materials/Warpgate/Warpgate_Electronics_Inst.Warpgate_Electronics_Inst")
      (Rendering|Material|SetMaterial _core_2 1 "/Game/PlanetSide_2/World/Materials/Warpgate/Warpgate_Electronics_Inst.Warpgate_Electronics_Inst")
      (Rendering|Material|SetMaterial _core_2 2 "/Game/PlanetSide_2/World/Materials/Warpgate/Warpgate_Pulse_C_Mat.Warpgate_Pulse_C_Mat")
      (Rendering|Material|SetMaterial _arm1_2 1 "/Game/PlanetSide_2/World/Materials/Warpgate/Warpgate_Pulse_C_Mat.Warpgate_Pulse_C_Mat")
      (Rendering|Material|SetMaterial _arm1_2 2 "/Game/PlanetSide_2/World/Materials/Warpgate/Warpgate_Electronics_Inst.Warpgate_Electronics_Inst"))
    (:NC
      (Rendering|Material|SetMaterial _shield 0 "/Game/PlanetSide_2/World/Materials/Warpgate/Shield_Inst_NC.Shield_Inst_NC")
      (Rendering|Material|SetMaterial _stand1_3 0 "/Game/PlanetSide_2/World/Materials/Warpgate/Warpgate_Reduced_Inst_NC.Warpgate_Reduced_Inst_NC")
      (Rendering|Material|SetMaterial _stand1_3 1 "/Game/PlanetSide_2/World/Materials/Warpgate/Hex_Tile_Pulse_Inst_NC.Hex_Tile_Pulse_Inst_NC")
      (Rendering|Material|SetMaterial _stand1_3 2 "/Game/PlanetSide_2/World/Materials/Warpgate/Warpgate_Pulse_C_Inst_NC.Warpgate_Pulse_C_Inst_NC")
      (Rendering|Material|SetMaterial _stand1_3 3 "/Game/PlanetSide_2/World/Materials/Warpgate/Warpgate_Electronics_Inst_NC.Warpgate_Electronics_Inst_NC")
      (Rendering|Material|SetMaterial _core_3 1 "/Game/PlanetSide_2/World/Materials/Warpgate/Warpgate_Electronics_Inst_NC.Warpgate_Electronics_Inst_NC")
      (Rendering|Material|SetMaterial _core_3 2 "/Game/PlanetSide_2/World/Materials/Warpgate/Warpgate_Pulse_C_Inst_NC.Warpgate_Pulse_C_Inst_NC")
      (Rendering|Material|SetMaterial _arm1_3 1 "/Game/PlanetSide_2/World/Materials/Warpgate/Warpgate_Pulse_C_Inst_NC.Warpgate_Pulse_C_Inst_NC")
      (Rendering|Material|SetMaterial _arm1_3 2 "/Game/PlanetSide_2/World/Materials/Warpgate/Warpgate_Electronics_Inst_NC.Warpgate_Electronics_Inst_NC"))
    (:TR
      (Rendering|Material|SetMaterial _shield 0 "/Game/PlanetSide_2/World/Materials/Warpgate/Shield_Inst_TR.Shield_Inst_TR")
      (Rendering|Material|SetMaterial _stand1_4 0 "/Game/PlanetSide_2/World/Materials/Warpgate/Warpgate_Reduced_Inst_TR.Warpgate_Reduced_Inst_TR")
      (Rendering|Material|SetMaterial _stand1_4 1 "/Game/PlanetSide_2/World/Materials/Warpgate/Hex_Tile_Pulse_Inst_TR.Hex_Tile_Pulse_Inst_TR")
      (Rendering|Material|SetMaterial _stand1_4 2 "/Game/PlanetSide_2/World/Materials/Warpgate/Warpgate_Pulse_C_Inst_TR.Warpgate_Pulse_C_Inst_TR")
      (Rendering|Material|SetMaterial _stand1_4 3 "/Game/PlanetSide_2/World/Materials/Warpgate/Warpgate_Electronics_Inst_TR.Warpgate_Electronics_Inst_TR")
      (Rendering|Material|SetMaterial _core_4 1 "/Game/PlanetSide_2/World/Materials/Warpgate/Warpgate_Electronics_Inst_TR.Warpgate_Electronics_Inst_TR")
      (Rendering|Material|SetMaterial _core_4 2 "/Game/PlanetSide_2/World/Materials/Warpgate/Warpgate_Pulse_C_Inst_TR.Warpgate_Pulse_C_Inst_TR")
      (Rendering|Material|SetMaterial _arm1_4 1 "/Game/PlanetSide_2/World/Materials/Warpgate/Warpgate_Pulse_C_Inst_TR.Warpgate_Pulse_C_Inst_TR")
      (Rendering|Material|SetMaterial _arm1_4 2 "/Game/PlanetSide_2/World/Materials/Warpgate/Warpgate_Electronics_Inst_TR.Warpgate_Electronics_Inst_TR"))
    (:VS
      (Rendering|Material|SetMaterial _shield 0 "/Game/PlanetSide_2/World/Materials/Warpgate/Shield_Inst_VS.Shield_Inst_VS")
      (Rendering|Material|SetMaterial _stand1 0 "/Game/PlanetSide_2/World/Materials/Warpgate/Warpgate_Reduced_Inst_VS.Warpgate_Reduced_Inst_VS")
      (Rendering|Material|SetMaterial _stand1 1 "/Game/PlanetSide_2/World/Materials/Warpgate/Hex_Tile_Pulse_Inst_VS.Hex_Tile_Pulse_Inst_VS")
      (Rendering|Material|SetMaterial _stand1 2 "/Game/PlanetSide_2/World/Materials/Warpgate/Warpgate_Pulse_C_Inst_VS.Warpgate_Pulse_C_Inst_VS")
      (Rendering|Material|SetMaterial _stand1 3 "/Game/PlanetSide_2/World/Materials/Warpgate/Warpgate_Electronics_Inst_VS.Warpgate_Electronics_Inst_VS")
      (Rendering|Material|SetMaterial _core 1 "/Game/PlanetSide_2/World/Materials/Warpgate/Warpgate_Electronics_Inst_VS.Warpgate_Electronics_Inst_VS")
      (Rendering|Material|SetMaterial _core 2 "/Game/PlanetSide_2/World/Materials/Warpgate/Warpgate_Pulse_C_Inst_VS.Warpgate_Pulse_C_Inst_VS")
      (Rendering|Material|SetMaterial _arm1 1 "/Game/PlanetSide_2/World/Materials/Warpgate/Warpgate_Pulse_C_Inst_VS.Warpgate_Pulse_C_Inst_VS")
      (Rendering|Material|SetMaterial _arm1 2 "/Game/PlanetSide_2/World/Materials/Warpgate/Warpgate_Electronics_Inst_VS.Warpgate_Electronics_Inst_VS"))))

(fn ConstructionScript
  (bind _shield (Variables|Default|GetShield))
  (bind _stand1 (Variables|Default|GetStand1))
  (bind _core (Variables|Default|GetCore))
  (bind _arm1 (Variables|Default|GetArm1))
  (bind _stand1_2 (Variables|Default|GetStand1))
  (bind _core_2 (Variables|Default|GetCore))
  (bind _arm1_2 (Variables|Default|GetArm1))
  (bind _stand1_3 (Variables|Default|GetStand1))
  (bind _core_3 (Variables|Default|GetCore))
  (bind _arm1_3 (Variables|Default|GetArm1))
  (bind _stand1_4 (Variables|Default|GetStand1))
  (bind _core_4 (Variables|Default|GetCore))
  (bind _arm1_4 (Variables|Default|GetArm1))
  (switch name (Variables|Default|GetFAction)
    (:NS
      (Rendering|Material|SetMaterial _shield 0 "/Game/PlanetSide_2/World/Materials/Warpgate/Shield_Inst.Shield_Inst")
      (Rendering|Material|SetMaterial _stand1_2 0 "/Game/PlanetSide_2/World/Materials/Warpgate/Warpgate_Reduced_Mat.Warpgate_Reduced_Mat")
      (Rendering|Material|SetMaterial _stand1_2 1 "/Game/PlanetSide_2/World/Materials/Warpgate/Hex_Tile_Pulse.Hex_Tile_Pulse")
      (Rendering|Material|SetMaterial _stand1_2 2 "/Game/PlanetSide_2/World/Materials/Warpgate/Warpgate_Pulse_C_Mat.Warpgate_Pulse_C_Mat")
      (Rendering|Material|SetMaterial _stand1_2 3 "/Game/PlanetSide_2/World/Materials/Warpgate/Warpgate_Electronics_Inst.Warpgate_Electronics_Inst")
      (Rendering|Material|SetMaterial _core_2 1 "/Game/PlanetSide_2/World/Materials/Warpgate/Warpgate_Electronics_Inst.Warpgate_Electronics_Inst")
      (Rendering|Material|SetMaterial _core_2 2 "/Game/PlanetSide_2/World/Materials/Warpgate/Warpgate_Pulse_C_Mat.Warpgate_Pulse_C_Mat")
      (Rendering|Material|SetMaterial _arm1_2 1 "/Game/PlanetSide_2/World/Materials/Warpgate/Warpgate_Pulse_C_Mat.Warpgate_Pulse_C_Mat")
      (Rendering|Material|SetMaterial _arm1_2 2 "/Game/PlanetSide_2/World/Materials/Warpgate/Warpgate_Electronics_Inst.Warpgate_Electronics_Inst"))
    (:NC
      (Rendering|Material|SetMaterial _shield 0 "/Game/PlanetSide_2/World/Materials/Warpgate/Shield_Inst_NC.Shield_Inst_NC")
      (Rendering|Material|SetMaterial _stand1_3 0 "/Game/PlanetSide_2/World/Materials/Warpgate/Warpgate_Reduced_Inst_NC.Warpgate_Reduced_Inst_NC")
      (Rendering|Material|SetMaterial _stand1_3 1 "/Game/PlanetSide_2/World/Materials/Warpgate/Hex_Tile_Pulse_Inst_NC.Hex_Tile_Pulse_Inst_NC")
      (Rendering|Material|SetMaterial _stand1_3 2 "/Game/PlanetSide_2/World/Materials/Warpgate/Warpgate_Pulse_C_Inst_NC.Warpgate_Pulse_C_Inst_NC")
      (Rendering|Material|SetMaterial _stand1_3 3 "/Game/PlanetSide_2/World/Materials/Warpgate/Warpgate_Electronics_Inst_NC.Warpgate_Electronics_Inst_NC")
      (Rendering|Material|SetMaterial _core_3 1 "/Game/PlanetSide_2/World/Materials/Warpgate/Warpgate_Electronics_Inst_NC.Warpgate_Electronics_Inst_NC")
      (Rendering|Material|SetMaterial _core_3 2 "/Game/PlanetSide_2/World/Materials/Warpgate/Warpgate_Pulse_C_Inst_NC.Warpgate_Pulse_C_Inst_NC")
      (Rendering|Material|SetMaterial _arm1_3 1 "/Game/PlanetSide_2/World/Materials/Warpgate/Warpgate_Pulse_C_Inst_NC.Warpgate_Pulse_C_Inst_NC")
      (Rendering|Material|SetMaterial _arm1_3 2 "/Game/PlanetSide_2/World/Materials/Warpgate/Warpgate_Electronics_Inst_NC.Warpgate_Electronics_Inst_NC"))
    (:TR
      (Rendering|Material|SetMaterial _shield 0 "/Game/PlanetSide_2/World/Materials/Warpgate/Shield_Inst_TR.Shield_Inst_TR")
      (Rendering|Material|SetMaterial _stand1_4 0 "/Game/PlanetSide_2/World/Materials/Warpgate/Warpgate_Reduced_Inst_TR.Warpgate_Reduced_Inst_TR")
      (Rendering|Material|SetMaterial _stand1_4 1 "/Game/PlanetSide_2/World/Materials/Warpgate/Hex_Tile_Pulse_Inst_TR.Hex_Tile_Pulse_Inst_TR")
      (Rendering|Material|SetMaterial _stand1_4 2 "/Game/PlanetSide_2/World/Materials/Warpgate/Warpgate_Pulse_C_Inst_TR.Warpgate_Pulse_C_Inst_TR")
      (Rendering|Material|SetMaterial _stand1_4 3 "/Game/PlanetSide_2/World/Materials/Warpgate/Warpgate_Electronics_Inst_TR.Warpgate_Electronics_Inst_TR")
      (Rendering|Material|SetMaterial _core_4 1 "/Game/PlanetSide_2/World/Materials/Warpgate/Warpgate_Electronics_Inst_TR.Warpgate_Electronics_Inst_TR")
      (Rendering|Material|SetMaterial _core_4 2 "/Game/PlanetSide_2/World/Materials/Warpgate/Warpgate_Pulse_C_Inst_TR.Warpgate_Pulse_C_Inst_TR")
      (Rendering|Material|SetMaterial _arm1_4 1 "/Game/PlanetSide_2/World/Materials/Warpgate/Warpgate_Pulse_C_Inst_TR.Warpgate_Pulse_C_Inst_TR")
      (Rendering|Material|SetMaterial _arm1_4 2 "/Game/PlanetSide_2/World/Materials/Warpgate/Warpgate_Electronics_Inst_TR.Warpgate_Electronics_Inst_TR"))
    (:VS
      (Rendering|Material|SetMaterial _shield 0 "/Game/PlanetSide_2/World/Materials/Warpgate/Shield_Inst_VS.Shield_Inst_VS")
      (Rendering|Material|SetMaterial _stand1 0 "/Game/PlanetSide_2/World/Materials/Warpgate/Warpgate_Reduced_Inst_VS.Warpgate_Reduced_Inst_VS")
      (Rendering|Material|SetMaterial _stand1 1 "/Game/PlanetSide_2/World/Materials/Warpgate/Hex_Tile_Pulse_Inst_VS.Hex_Tile_Pulse_Inst_VS")
      (Rendering|Material|SetMaterial _stand1 2 "/Game/PlanetSide_2/World/Materials/Warpgate/Warpgate_Pulse_C_Inst_VS.Warpgate_Pulse_C_Inst_VS")
      (Rendering|Material|SetMaterial _stand1 3 "/Game/PlanetSide_2/World/Materials/Warpgate/Warpgate_Electronics_Inst_VS.Warpgate_Electronics_Inst_VS")
      (Rendering|Material|SetMaterial _core 1 "/Game/PlanetSide_2/World/Materials/Warpgate/Warpgate_Electronics_Inst_VS.Warpgate_Electronics_Inst_VS")
      (Rendering|Material|SetMaterial _core 2 "/Game/PlanetSide_2/World/Materials/Warpgate/Warpgate_Pulse_C_Inst_VS.Warpgate_Pulse_C_Inst_VS")
      (Rendering|Material|SetMaterial _arm1 1 "/Game/PlanetSide_2/World/Materials/Warpgate/Warpgate_Pulse_C_Inst_VS.Warpgate_Pulse_C_Inst_VS")
      (Rendering|Material|SetMaterial _arm1 2 "/Game/PlanetSide_2/World/Materials/Warpgate/Warpgate_Electronics_Inst_VS.Warpgate_Electronics_Inst_VS"))))