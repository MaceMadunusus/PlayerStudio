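; Modular bridge for the PlanetSide_2 world that builds itself in the construction script from a tile count and tile length.
; Center sections are instances on BridgeCenter, spaced along local X.
; The Covered option swaps in the covered mesh and attaches two angled spot lights per tile.
; An added static mesh closes the far end, either mirrored with negative X scale or unmirrored and one tile further back when UnfinishedEnd is set.
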(fn ConstructionScript
  (bind _tile_length (Variables|Properties|GetTile%20Length))
  (if (Variables|Properties|GetCovered)
    (Components|StaticMesh|SetStaticMesh (Variables|Default|GetBridge%20Center) "/Game/PlanetSide_2/World/Meshes/Bridges/BridgeCovered.BridgeCovered")
    (Utilities|FlowControl|Sequence
      (:then_0
        (for _index (range 1 (Variables|Properties|GetTiling%20Count))
          (bind _returnvalue (AddComponent|AddSpotLightComponent false (Math|Transform|MakeTransform (Math|Vector|MakeVector (- (* _index (Variables|Properties|GetTile%20Length)) 1.87e+03) 0.0 2.11e+03) "-120.000000,0.000000, 0" "1,1,0.000000")))
          (bind _returnvalue_2 (AddComponent|AddSpotLightComponent false (Math|Transform|MakeTransform (Math|Vector|MakeVector (- (* _index (Variables|Properties|GetTile%20Length)) 1.13e+03) 0.0 2.11e+03) "-60.000000, 0, 0")))
          (Class|SceneComponent|Attachto _returnvalue_2 (Variables|Default|GetBridge%20Center) "None" "KeepRelativeOffset" true)))
      (:then_1
        (for _index_2 (range 1 (Variables|Properties|GetTiling%20Count)) :!label _label
          (Components|InstancedStaticMesh|AddInstance (Variables|Default|GetBridge%20Center) (Math|Transform|MakeTransform (Math|Vector|MakeVector (* _index_2 _tile_length) 0.0 0.0))))
        (if (Variables|Properties|GetUnfinished%20End)
          (AddComponent|AddStaticMeshComponent false (Math|Transform|MakeTransform (Math|Vector|MakeVector (- (- (* _index_2 _tile_length) _tile_length) _tile_length) 0.0 0.0) "0, 0, 0" "1.000000,1,1"))
          (else
            (AddComponent|AddStaticMeshComponent false (Math|Transform|MakeTransform (Math|Vector|MakeVector (- (* _index_2 _tile_length) _tile_length) 0.0 0.0) "0, 0, 0" "-1.000000,1,1"))))))
    (else
      (goto _label))))