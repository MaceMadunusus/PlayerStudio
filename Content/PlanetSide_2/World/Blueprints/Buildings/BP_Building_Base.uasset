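; Base building actor for PlanetSide_2 world buildings, built from separate Interior and Exterior mesh components.
; The construction script applies the configured interior and exterior materials to each component's first slot.
; When FacadeOnly is set, it destroys the interior component and swaps the exterior to a facade mesh.
; An UpdateMaterials event replaces both materials on demand; BeginPlay, overlap and Tick are unused.
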(event Custom|UpdateMaterials
  (params (Interior :type Material%20Instance%20Dynamic%20Object%20Reference) (Exterior :type Material%20Instance%20Dynamic%20Object%20Reference))
  (Rendering|Material|SetMaterial (Variables|Default|GetInterior) 0 Interior)
  (Rendering|Material|SetMaterial (Variables|Default|GetExterior) 0 Exterior))

(event EventBeginPlay)

(event EventActorBeginOverlap
  (params (OtherActor :type Actor%20Object%20Reference)))

(event EventTick
  (params (DeltaSeconds :type Float%20%28single-precision%29)))

(fn ConstructionScript
  (if (Variables|Properties|GetFacade%20Only)
    (Components|DestroyComponent (Variables|Default|GetInterior))
    (Components|StaticMesh|SetStaticMesh (Variables|Default|GetExterior) (Variables|Properties|GetFacade%20Mesh))
    (else
      (Rendering|Material|SetMaterial (Variables|Default|GetInterior) 0 (Variables|Materials|GetInterior%20Material))))
  (Rendering|Material|SetMaterial (Variables|Default|GetExterior) 0 (Variables|Materials|GetExterior%20Material)))