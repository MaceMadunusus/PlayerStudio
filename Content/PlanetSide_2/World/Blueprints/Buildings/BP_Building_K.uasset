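; BP_Building_K is a world building whose construction script assembles one of two visual styles after running its parent's script.
; Style selects the exterior mesh, and the second style also swaps the interior mesh.
; When attachments are enabled, flagged covers are added as instanced static meshes at preset transforms: door covers for both styles, plus window covers for the second.
; The second style reuses the first's door-cover branch after placing its windows.
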(fn ConstructionScript
  (bind _exterior (Variables|Default|GetExterior))
  (bind _has_attachments (Variables|Attachments|GetHas%20Attachments))
  (|CallParentFunction)
  (switch int (Variables|Building|GetStyle)
    (:1
      (Components|StaticMesh|SetStaticMesh _exterior "/Game/PlanetSide_2/World/Meshes/Buildings/Building_K_Exterior.Building_K_Exterior")
      (if _has_attachments
        (bind _returnvalue (AddComponent|AddInstancedStaticMeshComponent false :!label _label))
        (Utilities|FlowControl|Sequence
          (:then_0
            (if (Variables|Attachments|GetDoor%201%20Cover)
              (Components|InstancedStaticMesh|AddInstance _returnvalue (Variables|Attachments|GetDoor%201%20Cover%20Location))))
          (:then_1
            (if (Variables|Attachments|GetDoor%202%20Cover)
              (Components|InstancedStaticMesh|AddInstance _returnvalue (Variables|Attachments|GetDoor%202%20Cover%20Location)))))))
    (:2
      (Components|StaticMesh|SetStaticMesh _exterior "/Game/PlanetSide_2/World/Meshes/Buildings/Building_K_Exterior2.Building_K_Exterior2")
      (Components|StaticMesh|SetStaticMesh (Variables|Default|GetInterior) "/Game/PlanetSide_2/World/Meshes/Buildings/Building_K_Interior2.Building_K_Interior2")
      (if _has_attachments
        (bind _returnvalue_2 (AddComponent|AddInstancedStaticMeshComponent false))
        (Utilities|FlowControl|Sequence
          (:then_0
            (if (Variables|Attachments|GetWindow%201%20Cover)
              (Components|InstancedStaticMesh|AddInstance _returnvalue_2 (Variables|Attachments|GetWindow%201%20Cover%20Location))))
          (:then_1
            (if (Variables|Attachments|GetWindow%202%20Cover)
              (Components|InstancedStaticMesh|AddInstance _returnvalue_2 (Variables|Attachments|GetWindow%202%20Cover%20Location))))
          (:then_2
            (if (Variables|Attachments|GetWindow%203%20Cover)
              (Components|InstancedStaticMesh|AddInstance _returnvalue_2 (Variables|Attachments|GetWindow%203%20Cover%20Location))))
          (:then_3
            (if (Variables|Attachments|GetWindow%204%20Cover)
              (Components|InstancedStaticMesh|AddInstance _returnvalue_2 (Variables|Attachments|GetWindow%204%20Cover%20Location))))
          (:then_4
            (if (Variables|Attachments|GetWindow%205%20Cover)
              (Components|InstancedStaticMesh|AddInstance _returnvalue_2 (Variables|Attachments|GetWindow%205%20Cover%20Location))))
          (:then_5
            (if (Variables|Attachments|GetWindow%206%20Cover)
              (Components|InstancedStaticMesh|AddInstance _returnvalue_2 (Variables|Attachments|GetWindow%206%20Cover%20Location))))
          (:then_6
            (goto _label)))))))