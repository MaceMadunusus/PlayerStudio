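; Construction script for the Building H world prop, which has separate Interior and Exterior components and a FacadeOnly switch.
; When FacadeOnly is off, it shows the interior, sets the exterior mesh and creates a dynamic instance of the master building material.
; When it is on, it only creates a dynamic instance of the facility buildings material.
; Material assignment, hiding and Bloom parameter nodes are disconnected and never run.
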(fn ConstructionScript
  (if (Variables|Default|GetFacade%20Only)
    (Rendering|Material|CreateDynamicMaterialInstance "/Game/PlanetSide_2/World/Materials/FacilityBuildings_Inst.FacilityBuildings_Inst" :!class /Script/Engine.KismetMaterialLibrary)
    (else
      (Rendering|SetVisibility (Variables|Default|GetInterior) true true)
      (Components|StaticMesh|SetStaticMesh (Variables|Default|GetExterior) "/Game/PlanetSide_2/World/Meshes/Buildings/Building_H_Exterior.Building_H_Exterior")
      (Rendering|Material|CreateDynamicMaterialInstance "/Game/PlanetSide_2/World/Materials/Building_Master.Building_Master" :!class /Script/Engine.KismetMaterialLibrary))))