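; Construction-time Blueprint for Building K, a world building with selectable style variants and a facade-only option.
; When FacadeOnly is off, the construction script shows the interior and swaps meshes by Style, with the second style replacing both exterior and interior.
; That same branch then creates a dynamic material instance from Building_Master, with no parameters set on it.
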(fn ConstructionScript
  (bind _exterior (Variables|Default|GetExterior))
  (if (not (Variables|Default|GetFacade%20Only))
    (Rendering|SetVisibility (Variables|Default|GetInterior) true true)
    (switch int (Variables|Default|GetStyle)
      (:1
        (Components|StaticMesh|SetStaticMesh _exterior "/Game/PlanetSide_2/World/Meshes/Buildings/Building_K_Exterior.Building_K_Exterior"))
      (:2
        (Components|StaticMesh|SetStaticMesh _exterior "/Game/PlanetSide_2/World/Meshes/Buildings/Building_K_Exterior2.Building_K_Exterior2")
        (Components|StaticMesh|SetStaticMesh (Variables|Default|GetInterior) "/Game/PlanetSide_2/World/Meshes/Buildings/Building_K_Interior2.Building_K_Interior2")))
    (Rendering|Material|CreateDynamicMaterialInstance "/Game/PlanetSide_2/World/Materials/Building_Master.Building_Master" :!class /Script/Engine.KismetMaterialLibrary)))