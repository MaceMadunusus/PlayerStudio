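; Medical wing building Blueprint that optionally places cover attachments at up to eight doorways.
; Its construction script runs the parent's setup, then, if HasAttachments is set, adds one instanced static mesh component.
; Each enabled DoorNCover flag adds an instance at its matching DoorNCoverLocation, so all covers share that single component.
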(fn ConstructionScript
  (|CallParentFunction)
  (if (Variables|Attachments|GetHas%20Attachments)
    (bind _returnvalue (AddComponent|AddInstancedStaticMeshComponent false))
    (Utilities|FlowControl|Sequence
      (:then_0
        (if (Variables|Attachments|GetDoor%201%20Cover)
          (Components|InstancedStaticMesh|AddInstance _returnvalue (Variables|Attachments|GetDoor%201%20Cover%20Location))))
      (:then_1
        (if (Variables|Attachments|GetDoor%202%20Cover)
          (Components|InstancedStaticMesh|AddInstance _returnvalue (Variables|Attachments|GetDoor%202%20Cover%20Location))))
      (:then_2
        (if (Variables|Attachments|GetDoor%203%20Cover)
          (Components|InstancedStaticMesh|AddInstance _returnvalue (Variables|Attachments|GetDoor%203%20Cover%20Location))))
      (:then_3
        (if (Variables|Attachments|GetDoor%204%20Cover)
          (Components|InstancedStaticMesh|AddInstance _returnvalue (Variables|Attachments|GetDoor%204%20Cover%20Location))))
      (:then_4
        (if (Variables|Attachments|GetDoor%205%20Cover)
          (Components|InstancedStaticMesh|AddInstance _returnvalue (Variables|Attachments|GetDoor%205%20Cover%20Location))))
      (:then_5
        (if (Variables|Attachments|GetDoor%206%20Cover)
          (Components|InstancedStaticMesh|AddInstance _returnvalue (Variables|Attachments|GetDoor%206%20Cover%20Location))))
      (:then_6
        (if (Variables|Attachments|GetDoor%207%20Cover)
          (Components|InstancedStaticMesh|AddInstance _returnvalue (Variables|Attachments|GetDoor%207%20Cover%20Location))))
      (:then_7
        (if (Variables|Attachments|GetDoor%208%20Cover)
          (Components|InstancedStaticMesh|AddInstance _returnvalue (Variables|Attachments|GetDoor%208%20Cover%20Location)))))))