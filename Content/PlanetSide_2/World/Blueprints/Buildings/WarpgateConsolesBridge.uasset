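; Warpgate consoles bridge building piece with switchable lighting.
; The construction script creates a dynamic instance of the bridge material, applies it to the covered bridge mesh and sets the initial light state from LightsEnabled.
; A LightsOn/Off event updates that state at runtime, toggling the underside lights' visibility and driving the material's Bloom parameter to make the bridge glow or go dark.
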(event Custom|Lights%20On/Off
  (params (Lights%20Enabled :type Boolean))
  (bind _bloom (Variables|Default|GetBloom))
  (bind _bridge_dynamic_material (Variables|Default|GetBridge%20Dynamic%20MAterial))
  (Variables|Lights|SetLights%20Enabled Lights%20Enabled)
  (Rendering|Material|SetMaterial (Variables|Default|GetBridgeCovered) 0 (Variables|Default|GetBridge%20Dynamic%20MAterial))
  (Rendering|SetVisibility (Variables|Default|GetUnderside%20Lights) (Variables|Lights|GetLights%20Enabled) true)
  (if (Variables|Lights|GetLights%20Enabled)
    (Rendering|Material|SetScalarParameterValue _bridge_dynamic_material _bloom 1e+02 :!class /Script/Engine.MaterialInstanceDynamic)
    (else
      (Rendering|Material|SetScalarParameterValue _bridge_dynamic_material _bloom 0.0 :!class /Script/Engine.MaterialInstanceDynamic))))

(fn ConstructionScript
  (bind _lights_enabled (Variables|Lights|GetLights%20Enabled))
  (bind _bloom (Variables|Default|GetBloom))
  (bind _returnvalue (Rendering|Material|CreateDynamicMaterialInstance "/Game/PlanetSide_2/World/Materials/Bridges_Inst.Bridges_Inst" :!class /Script/Engine.KismetMaterialLibrary))
  (Variables|Default|SetBridge%20Dynamic%20MAterial _returnvalue)
  (Rendering|Material|SetMaterial (Variables|Default|GetBridgeCovered) 0 (Variables|Default|GetBridge%20Dynamic%20MAterial))
  (Rendering|SetVisibility (Variables|Default|GetUnderside%20Lights) _lights_enabled true)
  (if _lights_enabled
    (Rendering|Material|SetScalarParameterValue (Variables|Default|GetBridge%20Dynamic%20MAterial) _bloom 1e+02 :!class /Script/Engine.MaterialInstanceDynamic)
    (else
      (Rendering|Material|SetScalarParameterValue (Variables|Default|GetBridge%20Dynamic%20MAterial) _bloom 0.0 :!class /Script/Engine.MaterialInstanceDynamic))))