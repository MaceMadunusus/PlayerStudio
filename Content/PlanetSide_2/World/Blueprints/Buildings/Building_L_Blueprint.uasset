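; Building_L_Blueprint is a configurable L building for the PlanetSide_2 world, set up entirely in its construction script.
; Unless FacadeOnly is set, it shows the interior, assigns the exterior mesh and gives the interior a dynamic material instance.
; The exterior always gets its own dynamic instance, whose Bloom parameter follows the ExteriorLightsEnabled flag that also toggles exterior light visibility.
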(fn ConstructionScript
  (bind _exterior_lights_enabled (Variables|Default|GetExterior%20Lights%20Enabled))
  (if (Variables|Default|GetFacade%20Only)
    _
    (else
      (Rendering|SetVisibility (Variables|Default|GetInterior) true true)
      (Components|StaticMesh|SetStaticMesh (Variables|Default|GetExterior) "/Game/PlanetSide_2/World/Meshes/Buildings/Building_L_Exterior.Building_L_Exterior")
      (bind _returnvalue (Rendering|Material|CreateDynamicMaterialInstance "/Game/PlanetSide_2/World/Materials/FacilityBuildings_Interior_Inst.FacilityBuildings_Interior_Inst" :!class /Script/Engine.KismetMaterialLibrary))
      (Variables|Default|SetInterior%20Dynamic%20Mat _returnvalue)
      (Rendering|Material|SetMaterial (Variables|Default|GetInterior) 0 (Variables|Default|GetInterior%20Dynamic%20Mat))))
  (bind _returnvalue_2 (Rendering|Material|CreateDynamicMaterialInstance "/Game/PlanetSide_2/World/Materials/FacilityBuildings_Inst.FacilityBuildings_Inst" :!class /Script/Engine.KismetMaterialLibrary))
  (Variables|Default|SetExterior%20Dynamic%20Mat _returnvalue_2)
  (Rendering|Material|SetMaterial (Variables|Default|GetExterior) 0 (Variables|Default|GetExterior%20Dynamic%20Mat))
  (Rendering|SetVisibility (Variables|Default|GetExterior%20Lights) _exterior_lights_enabled true)
  (if _exterior_lights_enabled
    (Rendering|Material|SetScalarParameterValue (Variables|Default|GetExterior%20Dynamic%20Mat) "Bloom" 1e+02 :!class /Script/Engine.MaterialInstanceDynamic)
    (else
      (Rendering|Material|SetScalarParameterValue (Variables|Default|GetExterior%20Dynamic%20Mat) "Bloom" 0.0 :!class /Script/Engine.MaterialInstanceDynamic))))