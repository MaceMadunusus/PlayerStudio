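; Small spawn room building Blueprint in a PlanetSide 2 world, with shield lighting that reflects the owning faction.
; FactionSwitch recolors five shield lights to white for NS, blue for NC, red for TR or dark purple for VS.
; A separate ShieldEnable/Disable event toggles visibility from a boolean, propagating it to child components.
; The construction script is empty.
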(event Custom|Faction%20Switch
  (params (Faction :type Name :default "None"))
  (bind _shield_light_3 (Variables|Default|GetShield%20Light%203))
  (switch name Faction
    (:NS
      (Rendering|Components|Light|SetLightColor (Variables|Default|GetShield%20Light%207) "(R=1.000000,G=1.000000,B=1.000000,A=1.000000)"))
    (:NC
      (Rendering|Components|Light|SetLightColor _shield_light_3 "(R=0.000000,G=0.000000,B=1.000000,A=1.000000)"))
    (:TR
      (Rendering|Components|Light|SetLightColor _shield_light_3 "(R=1.000000,G=0.000000,B=0.000000,A=1.000000)"))
    (:VS
      (Rendering|Components|Light|SetLightColor _shield_light_3 "(R=0.073828,G=0.000000,B=0.073828,A=1.000000)"))))

(event Custom|Shield%20Enable/Disable
  (params (Shield :type Boolean))
  (Rendering|SetVisibility Shield true))

(fn ConstructionScript)