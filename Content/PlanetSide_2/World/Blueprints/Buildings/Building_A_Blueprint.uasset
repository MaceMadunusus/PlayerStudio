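; Placeable Building A for a PlanetSide 2 world, with faction colors, switchable exterior lights and a facade-only option.
; The construction script creates dynamic materials and, unless FacadeOnly, shows the interior, swaps in the full exterior mesh and hides facade-only lights.
; It then applies light visibility, material bloom and the NS, NC, TR or VS primary color.
; Two events repeat that lighting and color logic for later changes.
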(event Custom|Faction%20Switch
  (params (Faction%20Name :type Name))
  (bind _interior_dynamic_material (Variables|Default|GetInterior%20Dynamic%20Material))
  (Variables|Default|SetFAction Faction%20Name)
  (switch name (Variables|Default|GetFAction)
    (:NS
      (Rendering|Material|SetVectorParameterValue _interior_dynamic_material "Faction Primary Color" "(R=0.383775,G=0.325037,B=0.157281,A=1.000000)" :!class /Script/Engine.MaterialInstanceDynamic))
    (:NC
      (Rendering|Material|SetVectorParameterValue _interior_dynamic_material "Faction Primary Color" "(R=0.025000,G=0.025000,B=0.250000,A=1.000000)" :!class /Script/Engine.MaterialInstanceDynamic))
    (:TR
      (Rendering|Material|SetVectorParameterValue _interior_dynamic_material "Faction Primary Color" "(R=0.250000,G=0.025000,B=0.025000,A=1.000000)" :!class /Script/Engine.MaterialInstanceDynamic))
    (:VS
      (Rendering|Material|SetVectorParameterValue _interior_dynamic_material "Faction Primary Color" "(R=0.250000,G=0.025000,B=0.250000,A=1.000000)" :!class /Script/Engine.MaterialInstanceDynamic))))

(event Custom|Exterior%20Lights%20On/Off
  (params (Lights%20Enabled :type Boolean))
  (bind _exterior_dymamic_material (Variables|Default|GetExterior%20Dymamic%20Material))
  (Variables|Default|SetExterior%20Lights%20Enabled Lights%20Enabled)
  (Rendering|SetVisibility (Variables|Default|GetExterior%20Lights) (Variables|Default|GetExterior%20Lights%20Enabled) true)
  (if (Variables|Default|GetExterior%20Lights%20Enabled)
    (Rendering|Material|SetScalarParameterValue _exterior_dymamic_material "Bloom" 1e+02 :!class /Script/Engine.MaterialInstanceDynamic)
    (else
      (Rendering|Material|SetScalarParameterValue _exterior_dymamic_material "Bloom" 0.0 :!class /Script/Engine.MaterialInstanceDynamic))))

(fn ConstructionScript
  (bind _exterior_lights_enabled (Variables|Default|GetExterior%20Lights%20Enabled))
  (if (Variables|Default|GetFacade%20Only)
    _
    (else
      (Rendering|SetVisibility (Variables|Default|GetInterior) true true)
      (Components|StaticMesh|SetStaticMesh (Variables|Default|GetExterior) "/Game/PlanetSide_2/World/Meshes/Building_A_Exterior.Building_A_Exterior")
      (Rendering|SetVisibility (Variables|Default|GetExterior%20Lights%20Facade%20Only) false true)
      (bind _returnvalue (Rendering|Material|CreateDynamicMaterialInstance "/Game/PlanetSide_2/World/Materials/FacilityBuildings_Interior_Inst.FacilityBuildings_Interior_Inst" :!class /Script/Engine.KismetMaterialLibrary))
      (Variables|Default|SetInterior%20Dynamic%20Material _returnvalue)
      (Rendering|Material|SetMaterial (Variables|Default|GetInterior) 0 (Variables|Default|GetInterior%20Dynamic%20Material))))
  (bind _returnvalue_2 (Rendering|Material|CreateDynamicMaterialInstance "/Game/PlanetSide_2/World/Materials/FacilityBuildings_Inst.FacilityBuildings_Inst" :!class /Script/Engine.KismetMaterialLibrary))
  (Variables|Default|SetExterior%20Dymamic%20Material _returnvalue_2)
  (Rendering|Material|SetMaterial (Variables|Default|GetExterior) 0 (Variables|Default|GetExterior%20Dymamic%20Material))
  (Rendering|SetVisibility (Variables|Default|GetExterior%20Lights) _exterior_lights_enabled true)
  (if _exterior_lights_enabled
    (Rendering|Material|SetScalarParameterValue (Variables|Default|GetExterior%20Dymamic%20Material) "Bloom" 1e+02 :!class /Script/Engine.MaterialInstanceDynamic)
    (else
      (Rendering|Material|SetScalarParameterValue (Variables|Default|GetExterior%20Dymamic%20Material) "Bloom" 0.0 :!class /Script/Engine.MaterialInstanceDynamic)))
  (switch name (Variables|Default|GetFAction)
    (:NS
      (Rendering|Material|SetVectorParameterValue (Variables|Default|GetExterior%20Dymamic%20Material) "Faction Primary Color" "(R=0.383775,G=0.325037,B=0.157281,A=1.000000)" :!class /Script/Engine.MaterialInstanceDynamic))
    (:NC
      (Rendering|Material|SetVectorParameterValue (Variables|Default|GetExterior%20Dymamic%20Material) "Faction Primary Color" "(R=0.025000,G=0.025000,B=0.250000,A=1.000000)" :!class /Script/Engine.MaterialInstanceDynamic))
    (:TR
      (Rendering|Material|SetVectorParameterValue (Variables|Default|GetExterior%20Dymamic%20Material) "Faction Primary Color" "(R=0.250000,G=0.025000,B=0.025000,A=1.000000)" :!class /Script/Engine.MaterialInstanceDynamic))
    (:VS
      (Rendering|Material|SetVectorParameterValue (Variables|Default|GetExterior%20Dymamic%20Material) "Faction Primary Color" "(R=0.250000,G=0.025000,B=0.250000,A=1.000000)" :!class /Script/Engine.MaterialInstanceDynamic))))