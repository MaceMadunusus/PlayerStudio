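; BP_Building_B is a placeable world building with optional covers for four doors and two interior doors.
; Its construction script runs the parent script, then, if HasAttachments is set, adds one instanced static mesh component.
; Each enabled cover flag adds an instance to that component at its matching location variable, so all covers share one component.
; The event graph has no active logic.
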(event EventBeginPlay)

(event EventActorBeginOverlap
  (params (OtherActor :type Actor%20Object%20Reference)))

(event EventTick
  (params (DeltaSeconds :type Float%20%28single-precision%29)))

(fn ConstructionScript
  (|CallParentFunction)
  (if (Variables|Attachments|GetHas%20Attachments)
    (bind _returnvalue (AddComponent|AddInstancedStaticMeshComponent false))
    (Utilities|FlowControl|Sequence
      (:then_0
        (if (Variables|Attachments|GetDoor%201%20Cover)
          (Components|InstancedStaticMesh|AddInstance _returnvalue (Variables|Attachments|GetDoor%201%20Cover%20Location))))
      (:then_1
        (if (Variables|Attachments|GetDoor%202%20Cover)
          (Components|InstancedStaticMesh|AddInstance _returnvalue (Variables|Attachments|GetDoor%202%20Cover%20Location))))
      (:then_2
        (if (Variables|Attachments|GetDoor%203%20Cover)
          (Components|InstancedStaticMesh|AddInstance _returnvalue (Variables|Attachments|GetDoor%203%20Cover%20Location))))
      (:then_3
        (if (Variables|Attachments|GetDoor%204%20Cover)
          (Components|InstancedStaticMesh|AddInstance _returnvalue (Variables|Attachments|GetDoor%204%20Cover%20Location))))
      (:then_4
        (if (Variables|Attachments|GetInterior%20Door%201%20Cover)
          (Components|InstancedStaticMesh|AddInstance _returnvalue (Variables|Attachments|GetInterior%20Door%201%20Cover%20Location))))
      (:then_5
        (if (Variables|Attachments|GetInterior%20Door%202%20Cover)
          (Components|InstancedStaticMesh|AddInstance _returnvalue (Variables|Attachments|GetInterior%20Door%202%20Cover%20Location)))))))