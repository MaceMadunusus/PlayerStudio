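; BP_Building_I is a building Blueprint that can add optional covers at two door positions.
; Its construction script runs the parent's, then, if attachments are enabled, creates an instanced static mesh component.
; Each enabled door cover flag adds an instance at that door's stored location, so both covers share one component.
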(fn ConstructionScript
  (|CallParentFunction)
  (if (Variables|Attachments|GetHas%20Attachments)
    (bind _returnvalue (AddComponent|AddInstancedStaticMeshComponent false))
    (Utilities|FlowControl|Sequence
      (:then_0
        (if (Variables|Attachments|GetDoor%201%20Cover)
          (Components|InstancedStaticMesh|AddInstance _returnvalue (Variables|Attachments|GetDoor%201%20Cover%20Location))))
      (:then_1
        (if (Variables|Attachments|GetDoor%202%20Cover)
          (Components|InstancedStaticMesh|AddInstance _returnvalue (Variables|Attachments|GetDoor%202%20Cover%20Location)))))))