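; TeleporteR_BP is a world teleporter Blueprint that tints its Light to match the owning faction: NS, NC, TR or VS.
; The construction script applies the color for the current FAction value, and the FactionSwitch event stores a new faction and repeats the same color switch at runtime.
; It contains no teleport logic, only this faction-based lighting.
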(event Custom|Faction%20Switch
  (params (Faction%20Name :type Name))
  (bind _light (Variables|Default|GetLight))
  (Variables|Default|SetFAction Faction%20Name)
  (switch name (Variables|Default|GetFAction)
    (:NS
      (Rendering|Components|Light|SetLightColor _light (Variables|Default|GetLight%20Color)))
    (:NC
      (Rendering|Components|Light|SetLightColor _light (Variables|Default|GetLight%20Color%20NC)))
    (:TR
      (Rendering|Components|Light|SetLightColor _light (Variables|Default|GetLight%20Color%20TR)))
    (:VS
      (Rendering|Components|Light|SetLightColor _light (Variables|Default|GetLight%20Color%20VS)))))

(fn ConstructionScript
  (bind _light (Variables|Default|GetLight))
  (switch name (Variables|Default|GetFAction)
    (:NS
      (Rendering|Components|Light|SetLightColor _light (Variables|Default|GetLight%20Color)))
    (:NC
      (Rendering|Components|Light|SetLightColor _light (Variables|Default|GetLight%20Color%20NC)))
    (:TR
      (Rendering|Components|Light|SetLightColor _light (Variables|Default|GetLight%20Color%20TR)))
    (:VS
      (Rendering|Components|Light|SetLightColor _light (Variables|Default|GetLight%20Color%20VS)))))