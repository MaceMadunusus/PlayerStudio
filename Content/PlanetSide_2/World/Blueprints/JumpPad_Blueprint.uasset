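; Jump pad actor Blueprint that themes its appearance by faction (NS, NC, TR or VS), with no launch logic in its graphs.
; The construction script and FactionSwitch event repeat one switch that sets the pad mesh and spotlight color, with NS reusing the NC mesh.
; Particle color goes through a shared Material Parameter Collection, so the last pad to write it sets that color for every material using it.
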(event Custom|Faction%20Switch
  (params (Faction%20Name :type Name))
  (bind _spotlight1 (Variables|Default|GetSpotLight1))
  (bind _jumppad (Variables|Default|GetJumpPad))
  (Variables|JumpPad|SetFAction Faction%20Name)
  (switch name (Variables|JumpPad|GetFAction)
    (:NS
      (Components|StaticMesh|SetStaticMesh _jumppad "/Game/PlanetSide_2/World/Meshes/Gameplay/JumpPad_NC.JumpPad_NC")
      (Rendering|Components|Light|SetLightColor _spotlight1 "(R=1.000000,G=1.000000,B=1.000000,A=1.000000)")
      (Rendering|Material|SetVectorParameterValue "/Game/PlanetSide_2/World/Particles/Materials/Particle_Mat_Collection.Particle_Mat_Collection" "Faction Color" (Variables|Default|GetParticle%20Color%20NS) :!class /Script/Engine.KismetMaterialLibrary))
    (:NC
      (Components|StaticMesh|SetStaticMesh _jumppad "/Game/PlanetSide_2/World/Meshes/Gameplay/JumpPad_NC.JumpPad_NC")
      (Rendering|Components|Light|SetLightColor _spotlight1 "(R=0.100000,G=0.100000,B=1.000000,A=1.000000)")
      (Rendering|Material|SetVectorParameterValue "/Game/PlanetSide_2/World/Particles/Materials/Particle_Mat_Collection.Particle_Mat_Collection" "Faction Color" (Variables|Default|GetParticle%20Color%20NC) :!class /Script/Engine.KismetMaterialLibrary))
    (:TR
      (Components|StaticMesh|SetStaticMesh _jumppad "/Game/PlanetSide_2/World/Meshes/Gameplay/JumpPad_TR.JumpPad_TR")
      (Rendering|Components|Light|SetLightColor _spotlight1 "(R=1.000000,G=0.000000,B=0.000000,A=1.000000)")
      (Rendering|Material|SetVectorParameterValue "/Game/PlanetSide_2/World/Particles/Materials/Particle_Mat_Collection.Particle_Mat_Collection" "Faction Color" (Variables|Default|GetParticle%20Color%20TR) :!class /Script/Engine.KismetMaterialLibrary))
    (:VS
      (Components|StaticMesh|SetStaticMesh _jumppad "/Game/PlanetSide_2/World/Meshes/Gameplay/JumpPad_VS.JumpPad_VS")
      (Rendering|Components|Light|SetLightColor _spotlight1 "(R=0.637439,G=0.000000,B=1.000000,A=1.000000)")
      (Rendering|Material|SetVectorParameterValue "/Game/PlanetSide_2/World/Particles/Materials/Particle_Mat_Collection.Particle_Mat_Collection" "Faction Color" (Variables|Default|GetParticle%20Color%20VS) :!class /Script/Engine.KismetMaterialLibrary))))

(fn ConstructionScript
  (bind _jumppad (Variables|Default|GetJumpPad))
  (bind _spotlight1 (Variables|Default|GetSpotLight1))
  (switch name (Variables|JumpPad|GetFAction)
    (:NS
      (Components|StaticMesh|SetStaticMesh _jumppad "/Game/PlanetSide_2/World/Meshes/Gameplay/JumpPad_NC.JumpPad_NC")
      (Rendering|Components|Light|SetLightColor _spotlight1 "(R=1.000000,G=1.000000,B=1.000000,A=1.000000)")
      (Rendering|Material|SetVectorParameterValue "/Game/PlanetSide_2/World/Particles/Materials/Particle_Mat_Collection.Particle_Mat_Collection" "Faction Color" (Variables|Default|GetParticle%20Color%20NS) :!class /Script/Engine.KismetMaterialLibrary))
    (:NC
      (Components|StaticMesh|SetStaticMesh _jumppad "/Game/PlanetSide_2/World/Meshes/Gameplay/JumpPad_NC.JumpPad_NC")
      (Rendering|Components|Light|SetLightColor _spotlight1 "(R=0.100000,G=0.100000,B=1.000000,A=1.000000)")
      (Rendering|Material|SetVectorParameterValue "/Game/PlanetSide_2/World/Particles/Materials/Particle_Mat_Collection.Particle_Mat_Collection" "Faction Color" (Variables|Default|GetParticle%20Color%20NC) :!class /Script/Engine.KismetMaterialLibrary))
    (:TR
      (Components|StaticMesh|SetStaticMesh _jumppad "/Game/PlanetSide_2/World/Meshes/Gameplay/JumpPad_TR.JumpPad_TR")
      (Rendering|Components|Light|SetLightColor _spotlight1 "(R=1.000000,G=0.000000,B=0.000000,A=1.000000)")
      (Rendering|Material|SetVectorParameterValue "/Game/PlanetSide_2/World/Particles/Materials/Particle_Mat_Collection.Particle_Mat_Collection" "Faction Color" (Variables|Default|GetParticle%20Color%20TR) :!class /Script/Engine.KismetMaterialLibrary))
    (:VS
      (Components|StaticMesh|SetStaticMesh _jumppad "/Game/PlanetSide_2/World/Meshes/Gameplay/JumpPad_VS.JumpPad_VS")
      (Rendering|Components|Light|SetLightColor _spotlight1 "(R=0.637439,G=0.000000,B=1.000000,A=1.000000)")
      (Rendering|Material|SetVectorParameterValue "/Game/PlanetSide_2/World/Particles/Materials/Particle_Mat_Collection.Particle_Mat_Collection" "Faction Color" (Variables|Default|GetParticle%20Color%20VS) :!class /Script/Engine.KismetMaterialLibrary))))