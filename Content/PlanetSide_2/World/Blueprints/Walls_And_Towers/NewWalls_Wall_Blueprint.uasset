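; Modular wall Blueprint for world building that tiles wall segments along local Y in its Construction Script, driven by a tile count and length.
; Wall segments are added as instances to an instanced mesh, with or without a canopy.
; When the canopy is enabled, it is made visible and one of two styles adds a mesh component and angled spotlight per tile, with style 2 also swapping the base canopy mesh.
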(fn ConstructionScript
  (if (Variables|Default|GetCanopy%20Enabled)
    (Utilities|FlowControl|Sequence
      (:then_0
        (Rendering|SetVisibility (Variables|Meshes|GetCanopy) true true)
        (switch int (Variables|Default|GetCanopy%20Style)
          (:1
            ;[1 1 1] Canopy Style 1 Tiling
            (for _index (range 1 (Variables|Default|GetTiling%20Count))
              (bind _returnvalue (AddComponent|AddStaticMeshComponent false))
              (Class|SceneComponent|Attachto _returnvalue 0 "None" "KeepWorldPosition" true)
              (Transformation|SetRelativeLocation _returnvalue (Math|Vector|MakeVector 0.0 (+ (* _index (Variables|Default|GetTile%20Length)) 1242.0) 0.0) false)
              (bind _returnvalue_2 (AddComponent|AddSpotLightComponent false (Math|Transform|MakeTransform (Math|Vector|MakeVector -178.0 (+ (* _index (Variables|Default|GetTile%20Length)) 1242.0) 1416.0) "-40.000000, 0, 0")))
              (Class|SceneComponent|Attachto _returnvalue_2 0 "None" "KeepWorldPosition" true)))
          (:2
            ;[1 1 1] Canopy Style 2 Tiling
            (Components|StaticMesh|SetStaticMesh (Variables|Meshes|GetCanopy) "/Game/PlanetSide_2/World/Meshes/Walls/NewWalls_Canopy2.NewWalls_Canopy2")
            (for _index_2 (range 1 (Variables|Default|GetTiling%20Count))
              (bind _returnvalue_3 (AddComponent|AddStaticMeshComponent false))
              (Class|SceneComponent|Attachto _returnvalue_3 0 "None" "KeepWorldPosition" true)
              (Transformation|SetRelativeLocation _returnvalue_3 (Math|Vector|MakeVector 0.0 (+ (* _index_2 (Variables|Default|GetTile%20Length)) 1242.0) 0.0) false)
              (bind _returnvalue_4 (AddComponent|AddSpotLightComponent false (Math|Transform|MakeTransform (Math|Vector|MakeVector -178.0 (+ (* _index_2 (Variables|Default|GetTile%20Length)) 1242.0) 1416.0) "-40.000000, 0, 0")))
              (Class|SceneComponent|Attachto _returnvalue_4 0 "None" "KeepWorldPosition" true)))))
      (:then_1
        ;[1 1 1] Wall Tiling
        (for _index_3 (range 1 (Variables|Default|GetTiling%20Count)) :!label _label
          (Components|InstancedStaticMesh|AddInstance (Variables|Default|GetNewWalls_Wall) (Math|Transform|MakeTransform (Math|Vector|MakeVector 0.0 (* _index_3 (Variables|Default|GetTile%20Length)) 0.0))))))
    (else
      (goto _label))))