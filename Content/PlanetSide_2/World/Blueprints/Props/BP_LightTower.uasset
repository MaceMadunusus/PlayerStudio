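; Light tower prop with two spotlights and an emissive mesh material that can be switched on or off.
; With ManualColoring, the construction script creates a dynamic material and applies LightColor to lit towers; otherwise, disabled towers get a static off material.
; Towers disabled at construction destroy their spotlights.
; The LightsOn/Off event toggles spotlight visibility and the dynamic material's Bloom, which exists only with ManualColoring.
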(event Custom|Lights%20On/Off
  (params (Lights%20Enabled :type Boolean))
  (bind _bloom (Variables|Default|GetBloom))
  (bind _light_tower_dynamic_material (Variables|Default|GetLight%20Tower%20Dynamic%20Material))
  (bind _output_get (Variables|Default|SetLights%20Enabled Lights%20Enabled))
  (Rendering|SetVisibility (Variables|Default|GetSpotLight13) _output_get false)
  (if (Variables|Default|GetLights%20Enabled)
    (Rendering|Material|SetScalarParameterValue _light_tower_dynamic_material _bloom 1e+02 :!class /Script/Engine.MaterialInstanceDynamic)
    (else
      (Rendering|Material|SetScalarParameterValue _light_tower_dynamic_material _bloom 0.0 :!class /Script/Engine.MaterialInstanceDynamic))))

(fn ConstructionScript
  (bind _bloom (Variables|Default|GetBloom))
  (bind _light_color (Variables|Default|GetLight%20Color))
  (if (Variables|Default|GetManual%20Coloring)
    (bind _returnvalue (Rendering|Material|CreateDynamicMaterialInstance "/Game/PlanetSide_2/World/Materials/Props/LightTower_Modifiable_Inst.LightTower_Modifiable_Inst" :!class /Script/Engine.KismetMaterialLibrary))
    (bind _output_get (Variables|Default|SetLight%20Tower%20Dynamic%20Material _returnvalue))
    (Rendering|Material|SetMaterial (Variables|Default|GetLightTower) 0 _output_get)
    (if (Variables|Default|GetLights%20Enabled)
      (Rendering|Material|SetScalarParameterValue (Variables|Default|GetLight%20Tower%20Dynamic%20Material) _bloom 1e+02 :!class /Script/Engine.MaterialInstanceDynamic)
      (Rendering|Components|Light|SetLightColor (Variables|Default|GetSpotLight14) _light_color true)
      (Rendering|Material|SetVectorParameterValue (Variables|Default|GetLight%20Tower%20Dynamic%20Material) (Variables|Default|GetColor) _light_color :!class /Script/Engine.MaterialInstanceDynamic)
      (else
        (Rendering|Material|SetScalarParameterValue (Variables|Default|GetLight%20Tower%20Dynamic%20Material) _bloom 0.0 :!class /Script/Engine.MaterialInstanceDynamic)
        (Components|DestroyComponent (Variables|Default|GetSpotLight13))))
    (elif (not (Variables|Default|GetLights%20Enabled))
      (Rendering|Material|SetMaterial (Variables|Default|GetLightTower) 0 "/Game/PlanetSide_2/World/Materials/Props/LightTower_Off_Inst.LightTower_Off_Inst")
      (Components|DestroyComponent (Variables|Default|GetSpotLight13)))))