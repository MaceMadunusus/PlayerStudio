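; Straight oil pipeline prop that tiles a configurable number of segments into one placeable pipeline run.
; The construction script adds mesh instances to OilPipelineStraight along local X, spaced by TileLength, with the loop starting at the second tile.
; When Hollow is set, it swaps in the hollow mesh and adds a point light per segment, offsetting those on repeated tiles along the pipe.
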(fn ConstructionScript
  (if (Variables|Default|GetHollow)
    (Components|StaticMesh|SetStaticMesh (Variables|Default|GetOilPipeline_Straight) "/Game/PlanetSide_2/World/Meshes/Props/OilPipeline_Straight_Hollow.OilPipeline_Straight_Hollow")
    (AddComponent|AddPointLightComponent false))
  (for _index (range 1 (- (Variables|Default|GetTiling%20Count) 1))
    (Components|InstancedStaticMesh|AddInstance (Variables|Default|GetOilPipeline_Straight) (Math|Transform|MakeTransform (Math|Vector|MakeVector (* _index (Variables|Default|GetTile%20Length)) 0.0 0.0)))
    (if (Variables|Default|GetHollow)
      (AddComponent|AddPointLightComponent false (Math|Transform|MakeTransform (Math|Vector|MakeVector (+ (* _index (Variables|Default|GetTile%20Length)) 2915.0) 0.0 0.0))))))