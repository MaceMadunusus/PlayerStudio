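; BP_CeilingLight2 is a placeable ceiling light fixture prop with a configurable main light.
; Its construction script gives the fixture mesh a dynamic material instance built from CeilingLightFixtures_Inst.
; When LightsEnabled is set, it applies the exposed radius, intensity and outer cone angle to MainLight.
; Otherwise it hides the light and zeroes the material's Bloom parameter so the fixture appears switched off.
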(fn ConstructionScript
  (bind _main_light (Variables|Lights|GetMain%20Light))
  (bind _returnvalue (Rendering|Material|CreateDynamicMaterialInstance "/Game/PlanetSide_2/World/Materials/Props/CeilingLightFixtures_Inst.CeilingLightFixtures_Inst" :!class /Script/Engine.KismetMaterialLibrary))
  (bind _output_get (Variables|Default|SetCeiling%20Light%20Dyn%20Material _returnvalue))
  (Rendering|Material|SetMaterial (Variables|Meshes|GetCeilingLight2) 0 _output_get)
  (if (Variables|Lights|GetLights%20Enabled)
    (Rendering|Lighting|SetAttenuationRadius _main_light (Variables|Lights|GetRadius))
    (Rendering|Components|Light|SetIntensity _main_light (Variables|Lights|GetIntensity))
    (Rendering|Lighting|SetOuterConeAngle _main_light (Variables|Lights|GetOuter%20Cone%20Angle))
    (else
      (Rendering|SetVisibility (Variables|Lights|GetMain%20Light) false true)
      (Rendering|Material|SetScalarParameterValue (Variables|Default|GetCeiling%20Light%20Dyn%20Material) "Bloom" 0.0 :!class /Script/Engine.MaterialInstanceDynamic))))