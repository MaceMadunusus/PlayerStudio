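; Tripod work-light prop for the world that switches on and off with either the interior or exterior lighting group.
; The construction script puts a dynamic material instance on the tripod mesh and applies the off state when lights start disabled.
; Separate interior and exterior events store the new state, but only the one matching IsInteriorLight applies it, toggling the Lights component's visibility and the material's Bloom glow together.
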(event Custom|Interior%20Lights%20On/Off
  (params (Lights :type Boolean))
  (bind _tripod_light_dynamic_material (Variables|Default|GetTripod%20Light%20Dynamic%20Material))
  (Variables|Lights|SetLights%20Enabled Lights)
  (if (Variables|Lights|GetIs%20Interior%20Light)
    (if (Variables|Lights|GetLights%20Enabled)
      (Rendering|SetVisibility (Variables|Lights|GetLights) true true)
      (Rendering|Material|SetScalarParameterValue _tripod_light_dynamic_material "Bloom" 1e+02 :!class /Script/Engine.MaterialInstanceDynamic)
      (else
        (Rendering|SetVisibility (Variables|Lights|GetLights) false true)
        (Rendering|Material|SetScalarParameterValue _tripod_light_dynamic_material "Bloom" 0.0 :!class /Script/Engine.MaterialInstanceDynamic)))))

(event Custom|Exterior%20Lights%20On/Off
  (params (Lights :type Boolean))
  (bind _tripod_light_dynamic_material (Variables|Default|GetTripod%20Light%20Dynamic%20Material))
  (Variables|Lights|SetLights%20Enabled Lights)
  (if (not (Variables|Lights|GetIs%20Interior%20Light))
    (if (Variables|Lights|GetLights%20Enabled)
      (Rendering|SetVisibility (Variables|Lights|GetLights) true true)
      (Rendering|Material|SetScalarParameterValue _tripod_light_dynamic_material "Bloom" 1e+02 :!class /Script/Engine.MaterialInstanceDynamic)
      (else
        (Rendering|SetVisibility (Variables|Lights|GetLights) false true)
        (Rendering|Material|SetScalarParameterValue _tripod_light_dynamic_material "Bloom" 0.0 :!class /Script/Engine.MaterialInstanceDynamic)))))

(fn ConstructionScript
  (bind _returnvalue (Rendering|Material|CreateDynamicMaterialInstance "/Game/PlanetSide_2/World/Materials/Mining_Atlas_Inst.Mining_Atlas_Inst" :!class /Script/Engine.KismetMaterialLibrary))
  (Variables|Default|SetTripod%20Light%20Dynamic%20Material _returnvalue)
  (Rendering|Material|SetMaterial (Variables|Meshes|GetLight_Tripod) 0 (Variables|Default|GetTripod%20Light%20Dynamic%20Material))
  (if (not (Variables|Lights|GetLights%20Enabled))
    (Rendering|SetVisibility (Variables|Lights|GetLights) false true)
    (Rendering|Material|SetScalarParameterValue (Variables|Default|GetTripod%20Light%20Dynamic%20Material) "Bloom" 0.0 :!class /Script/Engine.MaterialInstanceDynamic)))