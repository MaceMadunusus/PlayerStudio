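; Ceiling light prop that switches on and off as part of either the interior or exterior lighting group.
; Separate interior and exterior events store the requested state in LightsEnabled, but only the one matching IsInteriorLight updates the fixture.
; Updates toggle MainLight visibility and drive the Bloom parameter on a dynamic material instance.
; The construction script creates that material and applies the off look when LightsEnabled is false.
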(event Custom|Interior%20Lights%20On/Off
  (params (Lights :type Boolean))
  (bind _ceiling_light_dyn_material (Variables|Default|GetCeiling%20Light%20Dyn%20Material))
  (bind _main_light (Variables|Lights|GetMain%20Light))
  (Variables|Lights|SetLights%20Enabled Lights)
  (if (Variables|Lights|GetIs%20Interior%20Light)
    (if (Variables|Lights|GetLights%20Enabled)
      (Rendering|SetVisibility _main_light true true)
      (Rendering|Material|SetScalarParameterValue _ceiling_light_dyn_material "Bloom" 1e+02 :!class /Script/Engine.MaterialInstanceDynamic)
      (else
        (Rendering|SetVisibility _main_light false true)
        (Rendering|Material|SetScalarParameterValue _ceiling_light_dyn_material "Bloom" 0.0 :!class /Script/Engine.MaterialInstanceDynamic)))))

(event Custom|Exterior%20Lights%20On/Off
  (params (Lights :type Boolean))
  (bind _ceiling_light_dyn_material (Variables|Default|GetCeiling%20Light%20Dyn%20Material))
  (bind _main_light (Variables|Lights|GetMain%20Light))
  (Variables|Lights|SetLights%20Enabled Lights)
  (if (not (Variables|Lights|GetIs%20Interior%20Light))
    (if (Variables|Lights|GetLights%20Enabled)
      (Rendering|SetVisibility _main_light true true)
      (Rendering|Material|SetScalarParameterValue _ceiling_light_dyn_material "Bloom" 1e+02 :!class /Script/Engine.MaterialInstanceDynamic)
      (else
        (Rendering|SetVisibility _main_light false true)
        (Rendering|Material|SetScalarParameterValue _ceiling_light_dyn_material "Bloom" 0.0 :!class /Script/Engine.MaterialInstanceDynamic)))))

(fn ConstructionScript
  (bind _returnvalue (Rendering|Material|CreateDynamicMaterialInstance "/Game/PlanetSide_2/World/Materials/Props/CeilingLightFixtures_Inst.CeilingLightFixtures_Inst" :!class /Script/Engine.KismetMaterialLibrary))
  (bind _output_get (Variables|Default|SetCeiling%20Light%20Dyn%20Material _returnvalue))
  (Rendering|Material|SetMaterial (Variables|Meshes|GetCeilingLight3) 0 _output_get)
  (if (not (Variables|Lights|GetLights%20Enabled))
    (Rendering|SetVisibility (Variables|Lights|GetMain%20Light) false true)
    (Rendering|Material|SetScalarParameterValue (Variables|Default|GetCeiling%20Light%20Dyn%20Material) "Bloom" 0.0 :!class /Script/Engine.MaterialInstanceDynamic)))