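; Ceiling light prop Blueprint that can be switched on and off as either an interior or exterior light.
; Separate interior and exterior toggle events store the enabled state, but only the one matching the IsInteriorLight flag updates the fixture.
; Switching changes the Lights component's visibility and the Bloom parameter on a dynamic material instance.
; The construction script creates that material instance and applies the off state when lights start disabled.
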(event Custom|Interior%20Lights%20On/Off
  (params (Lights%20Enabled :type Boolean))
  (bind _lights (Variables|Lights|GetLights))
  (bind _ceiling_light_dyn_material (Variables|Default|GetCeiling%20Light%20Dyn%20Material))
  (Variables|Lights|SetLights%20Enabled Lights%20Enabled)
  (if (Variables|Lights|GetIs%20Interior%20Light)
    (if (Variables|Lights|GetLights%20Enabled)
      (Rendering|SetVisibility _lights true true)
      (Rendering|Material|SetScalarParameterValue _ceiling_light_dyn_material "Bloom" 1e+02 :!class /Script/Engine.MaterialInstanceDynamic)
      (else
        (Rendering|SetVisibility _lights false true)
        (Rendering|Material|SetScalarParameterValue _ceiling_light_dyn_material "Bloom" 0.0 :!class /Script/Engine.MaterialInstanceDynamic)))))

(event Custom|Exterior%20Lights%20On/Off
  (params (Lights%20Enabled :type Boolean))
  (bind _lights (Variables|Lights|GetLights))
  (bind _ceiling_light_dyn_material (Variables|Default|GetCeiling%20Light%20Dyn%20Material))
  (Variables|Lights|SetLights%20Enabled Lights%20Enabled)
  (if (not (Variables|Lights|GetIs%20Interior%20Light))
    (if (Variables|Lights|GetLights%20Enabled)
      (Rendering|SetVisibility _lights true true)
      (Rendering|Material|SetScalarParameterValue _ceiling_light_dyn_material "Bloom" 1e+02 :!class /Script/Engine.MaterialInstanceDynamic)
      (else
        (Rendering|SetVisibility _lights false true)
        (Rendering|Material|SetScalarParameterValue _ceiling_light_dyn_material "Bloom" 0.0 :!class /Script/Engine.MaterialInstanceDynamic)))))

(fn ConstructionScript
  (bind _returnvalue (Rendering|Material|CreateDynamicMaterialInstance "/Game/PlanetSide_2/World/Materials/Props/CeilingLightFixtures_Inst.CeilingLightFixtures_Inst" :!class /Script/Engine.KismetMaterialLibrary))
  (Variables|Default|SetCeiling%20Light%20Dyn%20Material _returnvalue)
  (Rendering|Material|SetMaterial (Variables|Meshes|GetCeilingLight1) 0 (Variables|Default|GetCeiling%20Light%20Dyn%20Material))
  (if (not (Variables|Lights|GetLights%20Enabled))
    (Rendering|SetVisibility (Variables|Lights|GetLights) false true)
    (Rendering|Material|SetScalarParameterValue (Variables|Default|GetCeiling%20Light%20Dyn%20Material) "Bloom" 0.0 :!class /Script/Engine.MaterialInstanceDynamic)))