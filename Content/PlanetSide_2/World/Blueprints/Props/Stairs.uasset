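; Stairs prop that builds a tileable staircase in its construction script from instanced static meshes.
; TilingCountX repeats tiles across the width, while TilingCountY repeats them along negative Y, stepping down by TileHeight per row.
; Optional railings follow the rows, with IncludeCenterRails adding them between columns.
; The Railings instanced component is created inside the first-row column loop, replacing the reference on each pass.
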(fn ConstructionScript
  (bind _has_railing (Variables|Default|GetHas%20Railing))
  (bind _has_railing_2 (Variables|Default|GetHas%20Railing))
  (Utilities|FlowControl|Sequence
    (:then_0
      (for _index (range 1 (- (Variables|Default|GetTiling%20Count%20X) 1))
        (Components|InstancedStaticMesh|AddInstance (Variables|Default|GetStairs) (Math|Transform|MakeTransform (Math|Vector|MakeVector (* _index (Variables|Default|GetTile%20Width)) 0.0 0.0)))
        (if _has_railing_2
          (bind _returnvalue (AddComponent|AddInstancedStaticMeshComponent false))
          (Variables|Default|SetRailings _returnvalue)
          (if (Variables|Default|GetInclude%20Center%20Rails)
            (Components|InstancedStaticMesh|AddInstance (Variables|Default|GetRailings) (Math|Transform|MakeTransform (Math|Vector|MakeVector (* _index (Variables|Default|GetTile%20Width)) 0.0 0.0))))))
      (if _has_railing_2
        (Components|InstancedStaticMesh|AddInstance (Variables|Default|GetRailings) (Math|Transform|MakeTransform (Math|Vector|MakeVector (* _index (Variables|Default|GetTile%20Width)) 0.0 0.0)))))
    (:then_1
      (for _index_2 (range 1 (- (Variables|Default|GetTiling%20Count%20Y) 1))
        (Components|InstancedStaticMesh|AddInstance (Variables|Default|GetStairs) (Math|Transform|MakeTransform (Math|Vector|MakeVector 0.0 (* (* _index_2 (Variables|Default|GetTile%20Length)) -1.0) (* (* _index_2 (Variables|Default|GetTile%20Height)) -1.0))))
        (if (Variables|Default|GetHas%20Railing)
          (Components|InstancedStaticMesh|AddInstance (Variables|Default|GetRailings) (Math|Transform|ComposeTransforms (Math|Transform|MakeTransform (Math|Vector|MakeVector 0.0 (* (* _index_2 (Variables|Default|GetTile%20Length)) -1.0) (* (* _index_2 (Variables|Default|GetTile%20Height)) -1.0))) (Math|Transform|MakeTransform "7.000000, 0, 0"))))
        (for _index_3 (range 1 (- (Variables|Default|GetTiling%20Count%20X) 1))
          (Components|InstancedStaticMesh|AddInstance (Variables|Default|GetStairs) (Math|Transform|MakeTransform (Math|Vector|MakeVector (* _index_3 (Variables|Default|GetTile%20Width)) (* (* _index_2 (Variables|Default|GetTile%20Length)) -1.0) (* (* _index_2 (Variables|Default|GetTile%20Height)) -1.0))))
          (if _has_railing
            (if (Variables|Default|GetInclude%20Center%20Rails)
              (Components|InstancedStaticMesh|AddInstance (Variables|Default|GetRailings) (Math|Transform|MakeTransform (Math|Vector|MakeVector (* _index_3 (Variables|Default|GetTile%20Width)) (* (* _index_2 (Variables|Default|GetTile%20Length)) -1.0) (* (* _index_2 (Variables|Default|GetTile%20Height)) -1.0)))))))
        (if _has_railing
          (Components|InstancedStaticMesh|AddInstance (Variables|Default|GetRailings) (Math|Transform|MakeTransform (Math|Vector|MakeVector (* _index_3 (Variables|Default|GetTile%20Width)) (* (* _index_2 (Variables|Default|GetTile%20Length)) -1.0) (* (* _index_2 (Variables|Default|GetTile%20Height)) -1.0)))))))))