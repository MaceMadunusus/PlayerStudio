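; Wall light prop with two spotlights and a glowing material that switches on and off as either an interior or exterior light.
; The construction script creates a dynamic material instance, then applies intensity to both spotlights and radius to SpotLight1 only, or starts dark if disabled.
; Interior and exterior events both store the new state, but only the one matching IsInteriorLight toggles light visibility and material Bloom.
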(event Custom|Interior%20Lights%20On/Off
  (params (Lights :type Boolean))
  (bind _wall_light_dynamic_material (Variables|Lights|GetWall%20Light%20Dynamic%20Material))
  (Variables|Lights|SetLights%20Enabled Lights)
  (if (Variables|Lights|GetIs%20Interior%20Light)
    (if (Variables|Lights|GetLights%20Enabled)
      (Rendering|SetVisibility (Variables|Default|GetLights) true true)
      (Rendering|Material|SetScalarParameterValue _wall_light_dynamic_material "Bloom" 1e+02 :!class /Script/Engine.MaterialInstanceDynamic)
      (else
        (Rendering|SetVisibility (Variables|Default|GetLights) false true)
        (Rendering|Material|SetScalarParameterValue _wall_light_dynamic_material "Bloom" 0.0 :!class /Script/Engine.MaterialInstanceDynamic)))))

(event Custom|Exterior%20Lights%20On/Off
  (params (Lights :type Boolean))
  (bind _wall_light_dynamic_material (Variables|Lights|GetWall%20Light%20Dynamic%20Material))
  (Variables|Lights|SetLights%20Enabled Lights)
  (if (not (Variables|Lights|GetIs%20Interior%20Light))
    (if (Variables|Lights|GetLights%20Enabled)
      (Rendering|SetVisibility (Variables|Default|GetLights) true true)
      (Rendering|Material|SetScalarParameterValue _wall_light_dynamic_material "Bloom" 1e+02 :!class /Script/Engine.MaterialInstanceDynamic)
      (else
        (Rendering|SetVisibility (Variables|Default|GetLights) false true)
        (Rendering|Material|SetScalarParameterValue _wall_light_dynamic_material "Bloom" 0.0 :!class /Script/Engine.MaterialInstanceDynamic)))))

(fn ConstructionScript
  (bind _spotlight1 (Variables|Lights|GetSpotLight1))
  (bind _returnvalue (Rendering|Material|CreateDynamicMaterialInstance "/Game/PlanetSide_2/World/Materials/Props/Mining_Atlas_Inst.Mining_Atlas_Inst" :!class /Script/Engine.KismetMaterialLibrary))
  (bind _output_get (Variables|Lights|SetWall%20Light%20Dynamic%20Material _returnvalue))
  (Rendering|Material|SetMaterial (Variables|Meshes|GetLight_Wall) 0 _output_get)
  (if (Variables|Lights|GetLights%20Enabled)
    (Rendering|Components|Light|SetIntensity _spotlight1 (Variables|Lights|GetLight%20Intensity))
    (Rendering|Lighting|SetAttenuationRadius _spotlight1 (Variables|Lights|GetLight%20Radius))
    (else
      (Rendering|SetVisibility (Variables|Default|GetLights) false true)
      (Rendering|Material|SetScalarParameterValue (Variables|Lights|GetWall%20Light%20Dynamic%20Material) "Bloom" 0.0 :!class /Script/Engine.MaterialInstanceDynamic))))