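; Pillar Blueprint for a world prop whose attached lights and emissive glow switch on or off together.
; The construction script creates a dynamic instance of the mining atlas material, applies it to the pillar mesh and sets the initial state from the LightsEnabled flag.
; A LightsOn/Off event updates that flag at runtime, toggling the Lights component with its children and driving the material's Bloom parameter to match.
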(event Custom|Lights%20On/Off
  (params (Lights%20Enabled :type Boolean))
  (bind _bloom (Variables|Default|GetBloom))
  (bind _pillar_dynamic_material (Variables|Default|GetPillar%20Dynamic%20Material))
  (Variables|Default|SetLights%20Enabled Lights%20Enabled)
  (Rendering|Material|SetMaterial (Variables|Default|GetPillar) 0 (Variables|Default|GetPillar%20Dynamic%20Material))
  (Rendering|SetVisibility (Variables|Default|GetLights) (Variables|Default|GetLights%20Enabled) true)
  (if (Variables|Default|GetLights%20Enabled)
    (Rendering|Material|SetScalarParameterValue _pillar_dynamic_material _bloom 1e+02 :!class /Script/Engine.MaterialInstanceDynamic)
    (else
      (Rendering|Material|SetScalarParameterValue _pillar_dynamic_material _bloom 0.0 :!class /Script/Engine.MaterialInstanceDynamic))))

(fn ConstructionScript
  (bind _lights_enabled (Variables|Default|GetLights%20Enabled))
  (bind _bloom (Variables|Default|GetBloom))
  (bind _returnvalue (Rendering|Material|CreateDynamicMaterialInstance "/Game/PlanetSide_2/World/Materials/Mining_Atlas_Inst.Mining_Atlas_Inst" :!class /Script/Engine.KismetMaterialLibrary))
  (Variables|Default|SetPillar%20Dynamic%20Material _returnvalue)
  (Rendering|Material|SetMaterial (Variables|Default|GetPillar) 0 _returnvalue)
  (Rendering|SetVisibility (Variables|Default|GetLights) _lights_enabled true)
  (if _lights_enabled
    (Rendering|Material|SetScalarParameterValue _returnvalue _bloom 1e+02 :!class /Script/Engine.MaterialInstanceDynamic)
    (else
      (Rendering|Material|SetScalarParameterValue _returnvalue _bloom 0.0 :!class /Script/Engine.MaterialInstanceDynamic))))