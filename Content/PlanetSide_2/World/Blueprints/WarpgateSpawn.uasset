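; Warpgate spawn building actor that recolors itself for the owning faction and toggles its lighting.
; The construction script creates dynamic material instances for the six respawn arrays, the interior and the exterior.
; FactionSwitch sets the array light color and the interior and exterior primary color on those instances for NS, NC, TR or VS.
; Separate events show or hide the interior spot and wall lights and the exterior lights.
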(event Custom|Interior%20Lights%20On/Off
  (params (Lights%20Enabled :type Boolean))
  (Rendering|SetVisibility (Variables|Default|GetSpotLights) Lights%20Enabled true))

(event Custom|Faction%20Switch
  (params (Faction :type Name))
  (bind _respawn_array_dynamic_material (Variables|Default|GetRespawn%20Array%20Dynamic%20Material))
  (bind _interior_dynamic_material (Variables|Default|GetInterior%20Dynamic%20Material))
  (Variables|Default|SetFAction Faction)
  (switch name (Variables|Default|GetFAction)
    (:NS
      (Rendering|Material|SetVectorParameterValue _respawn_array_dynamic_material "Color 2" (Variables|Default|GetLight%20Color) :!class /Script/Engine.MaterialInstanceDynamic)
      (Rendering|Material|SetVectorParameterValue _interior_dynamic_material "Faction Primary Color" "(R=0.383775,G=0.325037,B=0.157281,A=1.000000)" :!class /Script/Engine.MaterialInstanceDynamic))
    (:NC
      (Rendering|Material|SetVectorParameterValue _respawn_array_dynamic_material "Color 2" (Variables|Default|GetLight%20Color%20NC) :!class /Script/Engine.MaterialInstanceDynamic)
      (Rendering|Material|SetVectorParameterValue _interior_dynamic_material "Faction Primary Color" "(R=0.025000,G=0.025000,B=0.250000,A=1.000000)" :!class /Script/Engine.MaterialInstanceDynamic))
    (:TR
      (Rendering|Material|SetVectorParameterValue _respawn_array_dynamic_material "Color 2" (Variables|Default|GetLight%20Color%20TR) :!class /Script/Engine.MaterialInstanceDynamic)
      (Rendering|Material|SetVectorParameterValue _interior_dynamic_material "Faction Primary Color" "(R=0.250000,G=0.025000,B=0.025000,A=1.000000)" :!class /Script/Engine.MaterialInstanceDynamic))
    (:VS
      (Rendering|Material|SetVectorParameterValue _respawn_array_dynamic_material "Color 2" (Variables|Default|GetLight%20Color%20VS) :!class /Script/Engine.MaterialInstanceDynamic)
      (Rendering|Material|SetVectorParameterValue _interior_dynamic_material "Faction Primary Color" "(R=0.250000,G=0.025000,B=0.250000,A=1.000000)" :!class /Script/Engine.MaterialInstanceDynamic))))

(event Custom|Exterior%20Lights%20On/Off
  (params (Lights%20Enabled :type Boolean))
  (Rendering|SetVisibility (Variables|Default|GetExterior%20Lights) Lights%20Enabled true))

(fn ConstructionScript
  (Utilities|FlowControl|Sequence
    (:then_0
      (bind _returnvalue (Rendering|Material|CreateDynamicMaterialInstance "/Game/PlanetSide_2/World/Materials/RespawnArray_Inst.RespawnArray_Inst" :!class /Script/Engine.KismetMaterialLibrary))
      (Variables|Default|SetRespawn%20Array%20Dynamic%20Material _returnvalue)
      (Rendering|Material|SetMaterial (Variables|Default|Getrespawn%20Array%203) 0 (Variables|Default|GetRespawn%20Array%20Dynamic%20Material)))
    (:then_1
      (bind _returnvalue_2 (Rendering|Material|CreateDynamicMaterialInstance "/Game/PlanetSide_2/World/Materials/FacilityBuildings_Interior_Inst.FacilityBuildings_Interior_Inst" :!class /Script/Engine.KismetMaterialLibrary))
      (Variables|Default|SetInterior%20Dynamic%20Material _returnvalue_2)
      (Rendering|Material|SetMaterial (Variables|Default|GetInterior) 0 (Variables|Default|GetInterior%20Dynamic%20Material)))
    (:then_2
      (bind _returnvalue_3 (Rendering|Material|CreateDynamicMaterialInstance "/Game/PlanetSide_2/World/Materials/FacilityBuildings_Inst.FacilityBuildings_Inst" :!class /Script/Engine.KismetMaterialLibrary))
      (Variables|Default|SetExterior%20Dynamic%20Material _returnvalue_3)
      (Rendering|Material|SetMaterial (Variables|Default|GetExterior) 0 (Variables|Default|GetExterior%20Dynamic%20Material)))))