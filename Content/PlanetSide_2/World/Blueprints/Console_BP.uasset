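; Faction-themed console prop whose ConsoleType selects one of eight icons (aircraft, infantry, vehicles, warpgate and others) and a matching screen material.
; The construction script shows the icon, then applies the material, light color and icon color for the current faction (NS, NC, TR, VS).
; FactionSwitch stores a new faction and repeats that styling.
; Icon color is written to the shared Icon_Parameters collection, so it is not per console.
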(event Custom|Faction%20Switch
  (params (Faction%20Name :type Name))
  (bind _console (Variables|Default|GetConsole))
  (bind _light_color_nc (Variables|Default|GetLight%20Color%20NC))
  (bind _light_color (Variables|Default|GetLight%20Color))
  (bind _console_type (Variables|Default|GetConsole%20Type))
  (bind _console_2 (Variables|Default|GetConsole))
  (bind _console_3 (Variables|Default|GetConsole))
  (bind _console_4 (Variables|Default|GetConsole))
  (bind _light_color_vs (Variables|Default|GetLight%20Color%20VS))
  (bind _light_color_tr (Variables|Default|GetLight%20Color%20TR))
  (Variables|Default|SetFAction Faction%20Name)
  (switch name (Variables|Default|GetFAction)
    (:NS
      (Utilities|FlowControl|Sequence
        (:then_0
          (switch int _console_type
            (:0
              (Rendering|Material|SetMaterial _console_3 1 "/Game/PlanetSide_2/World/Materials/Console/Console_NS1.Console_NS1"))
            (:1
              (Rendering|Material|SetMaterial _console_3 1 "/Game/PlanetSide_2/World/Materials/Console/Console_NS2.Console_NS2"))
            (:2
              (Rendering|Material|SetMaterial _console_3 1 "/Game/PlanetSide_2/World/Materials/Console/Console_NS3.Console_NS3"))
            (:3
              (Rendering|Material|SetMaterial _console_3 1 "/Game/PlanetSide_2/World/Materials/Console/Console_NS4.Console_NS4"))
            (:4
              (Rendering|Material|SetMaterial _console_3 1 "/Game/PlanetSide_2/World/Materials/Console/Console_NS5.Console_NS5"))
            (:5
              (Rendering|Material|SetMaterial _console_3 1 "/Game/PlanetSide_2/World/Materials/Console/Console_NS6.Console_NS6"))
            (:6
              (Rendering|Material|SetMaterial _console_3 1 "/Game/PlanetSide_2/World/Materials/Console/Console_NS7.Console_NS7"))
            (:7
              (Rendering|Material|SetMaterial _console_3 1 "/Game/PlanetSide_2/World/Materials/Console/Console_NS8.Console_NS8"))))
        (:then_1
          (Rendering|Components|Light|SetLightColor (Variables|Default|GetLight) _light_color)
          (Rendering|Material|SetVectorParameterValue "/Game/PlanetSide_2/Icons/Icon_Parameters.Icon_Parameters" "Color" _light_color :!class /Script/Engine.KismetMaterialLibrary))))
    (:NC
      (Utilities|FlowControl|Sequence
        (:then_0
          (switch int _console_type
            (:0
              (Rendering|Material|SetMaterial _console 1 "/Game/PlanetSide_2/World/Materials/Console/Console_NC1.Console_NC1"))
            (:1
              (Rendering|Material|SetMaterial _console 1 "/Game/PlanetSide_2/World/Materials/Console/Console_NC2.Console_NC2"))
            (:2
              (Rendering|Material|SetMaterial _console 1 "/Game/PlanetSide_2/World/Materials/Console/Console_NC3.Console_NC3"))
            (:3
              (Rendering|Material|SetMaterial _console 1 "/Game/PlanetSide_2/World/Materials/Console/Console_NC4.Console_NC4"))
            (:4
              (Rendering|Material|SetMaterial _console 1 "/Game/PlanetSide_2/World/Materials/Console/Console_NC5.Console_NC5"))
            (:5
              (Rendering|Material|SetMaterial _console 1 "/Game/PlanetSide_2/World/Materials/Console/Console_NC6.Console_NC6"))
            (:6
              (Rendering|Material|SetMaterial _console 1 "/Game/PlanetSide_2/World/Materials/Console/Console_NC7.Console_NC7"))
            (:7
              (Rendering|Material|SetMaterial _console 1 "/Game/PlanetSide_2/World/Materials/Console/Console_NC8.Console_NC8"))))
        (:then_1
          (Rendering|Components|Light|SetLightColor (Variables|Default|GetLight) _light_color_nc)
          (Rendering|Material|SetVectorParameterValue "/Game/PlanetSide_2/Icons/Icon_Parameters.Icon_Parameters" "Color" _light_color_nc :!class /Script/Engine.KismetMaterialLibrary))))
    (:TR
      (Utilities|FlowControl|Sequence
        (:then_0
          (switch int _console_type
            (:0
              (Rendering|Material|SetMaterial _console_4 1 "/Game/PlanetSide_2/World/Materials/Console/Console_TR1.Console_TR1"))
            (:1
              (Rendering|Material|SetMaterial _console_4 1 "/Game/PlanetSide_2/World/Materials/Console/Console_TR2.Console_TR2"))
            (:2
              (Rendering|Material|SetMaterial _console_4 1 "/Game/PlanetSide_2/World/Materials/Console/Console_TR3.Console_TR3"))
            (:3
              (Rendering|Material|SetMaterial _console_4 1 "/Game/PlanetSide_2/World/Materials/Console/Console_TR4.Console_TR4"))
            (:4
              (Rendering|Material|SetMaterial _console_4 1 "/Game/PlanetSide_2/World/Materials/Console/Console_TR5.Console_TR5"))
            (:5
              (Rendering|Material|SetMaterial _console_4 1 "/Game/PlanetSide_2/World/Materials/Console/Console_TR6.Console_TR6"))
            (:6
              (Rendering|Material|SetMaterial _console_4 1 "/Game/PlanetSide_2/World/Materials/Console/Console_TR7.Console_TR7"))
            (:7
              (Rendering|Material|SetMaterial _console_4 1 "/Game/PlanetSide_2/World/Materials/Console/Console_TR8.Console_TR8"))))
        (:then_1
          (Rendering|Components|Light|SetLightColor (Variables|Default|GetLight) _light_color_tr)
          (Rendering|Material|SetVectorParameterValue "/Game/PlanetSide_2/Icons/Icon_Parameters.Icon_Parameters" "Color" _light_color_tr :!class /Script/Engine.KismetMaterialLibrary))))
    (:VS
      (Utilities|FlowControl|Sequence
        (:then_0
          (switch int _console_type
            (:0
              (Rendering|Material|SetMaterial _console_2 1 "/Game/PlanetSide_2/World/Materials/Console/Console_VS1.Console_VS1"))
            (:1
              (Rendering|Material|SetMaterial _console_2 1 "/Game/PlanetSide_2/World/Materials/Console/Console_VS2.Console_VS2"))
            (:2
              (Rendering|Material|SetMaterial _console_2 1 "/Game/PlanetSide_2/World/Materials/Console/Console_VS3.Console_VS3"))
            (:3
              (Rendering|Material|SetMaterial _console_2 1 "/Game/PlanetSide_2/World/Materials/Console/Console_VS4.Console_VS4"))
            (:4
              (Rendering|Material|SetMaterial _console_2 1 "/Game/PlanetSide_2/World/Materials/Console/Console_VS5.Console_VS5"))
            (:5
              (Rendering|Material|SetMaterial _console_2 1 "/Game/PlanetSide_2/World/Materials/Console/Console_VS6.Console_VS6"))
            (:6
              (Rendering|Material|SetMaterial _console_2 1 "/Game/PlanetSide_2/World/Materials/Console/Console_VS7.Console_VS7"))
            (:7
              (Rendering|Material|SetMaterial _console_2 1 "/Game/PlanetSide_2/World/Materials/Console/Console_VS8.Console_VS8"))))
        (:then_1
          (Rendering|Components|Light|SetLightColor (Variables|Default|GetLight) _light_color_vs)
          (Rendering|Material|SetVectorParameterValue "/Game/PlanetSide_2/Icons/Icon_Parameters.Icon_Parameters" "Color" _light_color_vs :!class /Script/Engine.KismetMaterialLibrary))))))

(fn ConstructionScript
  (bind _console (Variables|Default|GetConsole))
  (bind _light_color_nc (Variables|Default|GetLight%20Color%20NC))
  (bind _light_color (Variables|Default|GetLight%20Color))
  (bind _console_2 (Variables|Default|GetConsole))
  (bind _console_type (Variables|Default|GetConsole%20Type))
  (bind _console_3 (Variables|Default|GetConsole))
  (bind _console_4 (Variables|Default|GetConsole))
  (bind _light_color_vs (Variables|Default|GetLight%20Color%20VS))
  (bind _light_color_tr (Variables|Default|GetLight%20Color%20TR))
  (Utilities|FlowControl|Sequence
    (:then_0
      (switch int (Variables|Default|GetConsole%20Type)
        (:0
          (Rendering|SetVisibility (Variables|Icon|GetIcon%20Aircraft) true false))
        (:1
          (Rendering|SetVisibility (Variables|Icon|GetIcon%20Galaxy) true false))
        (:2
          (Rendering|SetVisibility (Variables|Icon|GetIcon%20Infantry) true false))
        (:3
          (Rendering|SetVisibility (Variables|Icon|GetIcon%20Vehicle) true false))
        (:4
          (Rendering|SetVisibility (Variables|Icon|GetIcon%20Lightning) true false))
        (:5
          (Rendering|SetVisibility (Variables|Icon|GetIcon%20Flash) true false))
        (:6
          (Rendering|SetVisibility (Variables|Icon|GetIcon%20Sunderer) true false))
        (:7
          (Rendering|SetVisibility (Variables|Icon|GetIcon%20Warpgate) true false))))
    (:then_1
      (switch name (Variables|Default|GetFAction)
        (:NS
          (Utilities|FlowControl|Sequence
            (:then_0
              (switch int _console_type
                (:0
                  (Rendering|Material|SetMaterial _console_3 1 "/Game/PlanetSide_2/World/Materials/Console/Console_NS1.Console_NS1"))
                (:1
                  (Rendering|Material|SetMaterial _console_3 1 "/Game/PlanetSide_2/World/Materials/Console/Console_NS2.Console_NS2"))
                (:2
                  (Rendering|Material|SetMaterial _console_3 1 "/Game/PlanetSide_2/World/Materials/Console/Console_NS3.Console_NS3"))
                (:3
                  (Rendering|Material|SetMaterial _console_3 1 "/Game/PlanetSide_2/World/Materials/Console/Console_NS4.Console_NS4"))
                (:4
                  (Rendering|Material|SetMaterial _console_3 1 "/Game/PlanetSide_2/World/Materials/Console/Console_NS5.Console_NS5"))
                (:5
                  (Rendering|Material|SetMaterial _console_3 1 "/Game/PlanetSide_2/World/Materials/Console/Console_NS6.Console_NS6"))
                (:6
                  (Rendering|Material|SetMaterial _console_3 1 "/Game/PlanetSide_2/World/Materials/Console/Console_NS7.Console_NS7"))
                (:7
                  (Rendering|Material|SetMaterial _console_3 1 "/Game/PlanetSide_2/World/Materials/Console/Console_NS8.Console_NS8"))))
            (:then_1
              (Rendering|Components|Light|SetLightColor (Variables|Default|GetLight) _light_color)
              (Rendering|Material|SetVectorParameterValue "/Game/PlanetSide_2/Icons/Icon_Parameters.Icon_Parameters" "Color" _light_color :!class /Script/Engine.KismetMaterialLibrary))))
        (:NC
          (Utilities|FlowControl|Sequence
            (:then_0
              (switch int _console_type
                (:0
                  (Rendering|Material|SetMaterial _console 1 "/Game/PlanetSide_2/World/Materials/Console/Console_NC1.Console_NC1"))
                (:1
                  (Rendering|Material|SetMaterial _console 1 "/Game/PlanetSide_2/World/Materials/Console/Console_NC2.Console_NC2"))
                (:2
                  (Rendering|Material|SetMaterial _console 1 "/Game/PlanetSide_2/World/Materials/Console/Console_NC3.Console_NC3"))
                (:3
                  (Rendering|Material|SetMaterial _console 1 "/Game/PlanetSide_2/World/Materials/Console/Console_NC4.Console_NC4"))
                (:4
                  (Rendering|Material|SetMaterial _console 1 "/Game/PlanetSide_2/World/Materials/Console/Console_NC5.Console_NC5"))
                (:5
                  (Rendering|Material|SetMaterial _console 1 "/Game/PlanetSide_2/World/Materials/Console/Console_NC6.Console_NC6"))
                (:6
                  (Rendering|Material|SetMaterial _console 1 "/Game/PlanetSide_2/World/Materials/Console/Console_NC7.Console_NC7"))
                (:7
                  (Rendering|Material|SetMaterial _console 1 "/Game/PlanetSide_2/World/Materials/Console/Console_NC8.Console_NC8"))))
            (:then_1
              (Rendering|Components|Light|SetLightColor (Variables|Default|GetLight) _light_color_nc)
              (Rendering|Material|SetVectorParameterValue "/Game/PlanetSide_2/Icons/Icon_Parameters.Icon_Parameters" "Color" _light_color_nc :!class /Script/Engine.KismetMaterialLibrary))))
        (:TR
          (Utilities|FlowControl|Sequence
            (:then_0
              (switch int _console_type
                (:0
                  (Rendering|Material|SetMaterial _console_4 1 "/Game/PlanetSide_2/World/Materials/Console/Console_TR1.Console_TR1"))
                (:1
                  (Rendering|Material|SetMaterial _console_4 1 "/Game/PlanetSide_2/World/Materials/Console/Console_TR2.Console_TR2"))
                (:2
                  (Rendering|Material|SetMaterial _console_4 1 "/Game/PlanetSide_2/World/Materials/Console/Console_TR3.Console_TR3"))
                (:3
                  (Rendering|Material|SetMaterial _console_4 1 "/Game/PlanetSide_2/World/Materials/Console/Console_TR4.Console_TR4"))
                (:4
                  (Rendering|Material|SetMaterial _console_4 1 "/Game/PlanetSide_2/World/Materials/Console/Console_TR5.Console_TR5"))
                (:5
                  (Rendering|Material|SetMaterial _console_4 1 "/Game/PlanetSide_2/World/Materials/Console/Console_TR6.Console_TR6"))
                (:6
                  (Rendering|Material|SetMaterial _console_4 1 "/Game/PlanetSide_2/World/Materials/Console/Console_TR7.Console_TR7"))
                (:7
                  (Rendering|Material|SetMaterial _console_4 1 "/Game/PlanetSide_2/World/Materials/Console/Console_TR8.Console_TR8"))))
            (:then_1
              (Rendering|Components|Light|SetLightColor (Variables|Default|GetLight) _light_color_tr)
              (Rendering|Material|SetVectorParameterValue "/Game/PlanetSide_2/Icons/Icon_Parameters.Icon_Parameters" "Color" _light_color_tr :!class /Script/Engine.KismetMaterialLibrary))))
        (:VS
          (Utilities|FlowControl|Sequence
            (:then_0
              (switch int _console_type
                (:0
                  (Rendering|Material|SetMaterial _console_2 1 "/Game/PlanetSide_2/World/Materials/Console/Console_VS1.Console_VS1"))
                (:1
                  (Rendering|Material|SetMaterial _console_2 1 "/Game/PlanetSide_2/World/Materials/Console/Console_VS2.Console_VS2"))
                (:2
                  (Rendering|Material|SetMaterial _console_2 1 "/Game/PlanetSide_2/World/Materials/Console/Console_VS3.Console_VS3"))
                (:3
                  (Rendering|Material|SetMaterial _console_2 1 "/Game/PlanetSide_2/World/Materials/Console/Console_VS4.Console_VS4"))
                (:4
                  (Rendering|Material|SetMaterial _console_2 1 "/Game/PlanetSide_2/World/Materials/Console/Console_VS5.Console_VS5"))
                (:5
                  (Rendering|Material|SetMaterial _console_2 1 "/Game/PlanetSide_2/World/Materials/Console/Console_VS6.Console_VS6"))
                (:6
                  (Rendering|Material|SetMaterial _console_2 1 "/Game/PlanetSide_2/World/Materials/Console/Console_VS7.Console_VS7"))
                (:7
                  (Rendering|Material|SetMaterial _console_2 1 "/Game/PlanetSide_2/World/Materials/Console/Console_VS8.Console_VS8"))))
            (:then_1
              (Rendering|Components|Light|SetLightColor (Variables|Default|GetLight) _light_color_vs)
              (Rendering|Material|SetVectorParameterValue "/Game/PlanetSide_2/Icons/Icon_Parameters.Icon_Parameters" "Color" _light_color_vs :!class /Script/Engine.KismetMaterialLibrary))))))))