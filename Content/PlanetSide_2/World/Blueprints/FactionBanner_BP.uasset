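; Faction banner prop with a light that shows NS, NC, TR or VS branding in the world.
; The construction script picks a wall or standing mesh, lit or off, moves the light for wall mounts, and hides it when disabled.
; It applies a faction material and tints the light and a dynamic base material with the faction color.
; The FactionSwitch event repeats that material and color setup to change faction at runtime, leaving mesh and visibility untouched.
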(event Custom|Faction%20Switch
  (params (Faction%20Name :type Name))
  (bind _banner (Variables|Default|GetBanner))
  (bind _light_color_vs (Variables|Default|GetLight%20Color%20VS))
  (bind _light_color_tr (Variables|Default|GetLight%20Color%20TR))
  (bind _light_color_nc (Variables|Default|GetLight%20Color%20NC))
  (bind _light_color (Variables|Default|GetLight%20Color))
  (bind _light (Variables|Default|GetLight))
  (Variables|Default|SetFAction Faction%20Name)
  (bind _returnvalue (Rendering|Material|CreateDynamicMaterialInstance "/Game/PlanetSide_2/World/Materials/Faction_Banner_Inst.Faction_Banner_Inst" :!class /Script/Engine.KismetMaterialLibrary))
  (Variables|Default|SetBanner%20Base%20Material _returnvalue)
  (Rendering|Material|SetMaterial (Variables|Default|GetBanner) 0 _returnvalue)
  (switch name (Variables|Default|GetFAction)
    (:NS
      (Utilities|FlowControl|Sequence
        (:then_0
          (Rendering|Material|SetMaterial _banner 1 "/Game/PlanetSide_2/World/Materials/Banners/FactionBanner.FactionBanner"))
        (:then_1
          (Rendering|Components|Light|SetLightColor _light _light_color))
        (:then_2
          (Rendering|Material|SetVectorParameterValue (Variables|Default|GetBanner%20Base%20Material) "Color" _light_color :!class /Script/Engine.MaterialInstanceDynamic))))
    (:NC
      (Utilities|FlowControl|Sequence
        (:then_0
          (Rendering|Material|SetMaterial _banner 1 "/Game/PlanetSide_2/World/Materials/Banners/FactionBanner_NC_Inst.FactionBanner_NC_Inst"))
        (:then_1
          (Rendering|Components|Light|SetLightColor _light _light_color_nc))
        (:then_2
          (Rendering|Material|SetVectorParameterValue (Variables|Default|GetBanner%20Base%20Material) "Color" _light_color_nc :!class /Script/Engine.MaterialInstanceDynamic))))
    (:TR
      (Utilities|FlowControl|Sequence
        (:then_0
          (Rendering|Material|SetMaterial _banner 1 "/Game/PlanetSide_2/World/Materials/Banners/FactionBanner_TR_Inst.FactionBanner_TR_Inst"))
        (:then_1
          (Rendering|Components|Light|SetLightColor _light _light_color_tr))
        (:then_2
          (Rendering|Material|SetVectorParameterValue (Variables|Default|GetBanner%20Base%20Material) "Color" _light_color_tr :!class /Script/Engine.MaterialInstanceDynamic))))
    (:VS
      (Utilities|FlowControl|Sequence
        (:then_0
          (Rendering|Material|SetMaterial _banner 1 "/Game/PlanetSide_2/World/Materials/Banners/FactionBanner_VS_Inst.FactionBanner_VS_Inst"))
        (:then_1
          (Rendering|Components|Light|SetLightColor _light _light_color_vs))
        (:then_2
          (Rendering|Material|SetVectorParameterValue (Variables|Default|GetBanner%20Base%20Material) "Color" _light_color_vs :!class /Script/Engine.MaterialInstanceDynamic))))))

(fn ConstructionScript
  (bind _banner (Variables|Default|GetBanner))
  (bind _banner_2 (Variables|Default|GetBanner))
  (bind _light_color_vs (Variables|Default|GetLight%20Color%20VS))
  (bind _light_color_tr (Variables|Default|GetLight%20Color%20TR))
  (bind _light_color_nc (Variables|Default|GetLight%20Color%20NC))
  (bind _light_color (Variables|Default|GetLight%20Color))
  (bind _banner_enabled (Variables|Default|GetBanner%20Enabled))
  (bind _light (Variables|Default|GetLight))
  (if (Variables|Default|GetWall%20Mounted)
    (Transformation|SetRelativeLocation (Variables|Default|GetLight) "0, 0,-290.000000" false)
    (if _banner_enabled
      (Components|StaticMesh|SetStaticMesh _banner_2 "/Game/PlanetSide_2/World/Meshes/Gameplay/Banner_Wall.Banner_Wall")
      (bind _returnvalue (Rendering|Material|CreateDynamicMaterialInstance "/Game/PlanetSide_2/World/Materials/Faction_Banner_Inst.Faction_Banner_Inst" :!class /Script/Engine.KismetMaterialLibrary :!label _label))
      (Variables|Default|SetBanner%20Base%20Material _returnvalue)
      (Rendering|Material|SetMaterial (Variables|Default|GetBanner) 0 _returnvalue)
      (switch name (Variables|Default|GetFAction)
        (:NS
          (Utilities|FlowControl|Sequence
            (:then_0
              (Rendering|Material|SetMaterial _banner 1 "/Game/PlanetSide_2/World/Materials/Banners/FactionBanner.FactionBanner"))
            (:then_1
              (Rendering|Components|Light|SetLightColor _light _light_color))
            (:then_2
              (Rendering|Material|SetVectorParameterValue (Variables|Default|GetBanner%20Base%20Material) "Color" _light_color :!class /Script/Engine.MaterialInstanceDynamic))))
        (:NC
          (Utilities|FlowControl|Sequence
            (:then_0
              (Rendering|Material|SetMaterial _banner 1 "/Game/PlanetSide_2/World/Materials/Banners/FactionBanner_NC_Inst.FactionBanner_NC_Inst"))
            (:then_1
              (Rendering|Components|Light|SetLightColor _light _light_color_nc))
            (:then_2
              (Rendering|Material|SetVectorParameterValue (Variables|Default|GetBanner%20Base%20Material) "Color" _light_color_nc :!class /Script/Engine.MaterialInstanceDynamic))))
        (:TR
          (Utilities|FlowControl|Sequence
            (:then_0
              (Rendering|Material|SetMaterial _banner 1 "/Game/PlanetSide_2/World/Materials/Banners/FactionBanner_TR_Inst.FactionBanner_TR_Inst"))
            (:then_1
              (Rendering|Components|Light|SetLightColor _light _light_color_tr))
            (:then_2
              (Rendering|Material|SetVectorParameterValue (Variables|Default|GetBanner%20Base%20Material) "Color" _light_color_tr :!class /Script/Engine.MaterialInstanceDynamic))))
        (:VS
          (Utilities|FlowControl|Sequence
            (:then_0
              (Rendering|Material|SetMaterial _banner 1 "/Game/PlanetSide_2/World/Materials/Banners/FactionBanner_VS_Inst.FactionBanner_VS_Inst"))
            (:then_1
              (Rendering|Components|Light|SetLightColor _light _light_color_vs))
            (:then_2
              (Rendering|Material|SetVectorParameterValue (Variables|Default|GetBanner%20Base%20Material) "Color" _light_color_vs :!class /Script/Engine.MaterialInstanceDynamic)))))
      (else
        (Components|StaticMesh|SetStaticMesh _banner_2 "/Game/PlanetSide_2/World/Meshes/Gameplay/Banner_Wall_Off.Banner_Wall_Off")
        (bind _returnvalue_2 (Rendering|Material|CreateDynamicMaterialInstance "/Game/PlanetSide_2/World/Materials/Faction_Banner_Inst.Faction_Banner_Inst" :!class /Script/Engine.KismetMaterialLibrary :!label _label_2))
        (Variables|Default|SetBanner%20Base%20Material _returnvalue_2)
        (Rendering|Material|SetMaterial (Variables|Default|GetBanner) 0 _returnvalue_2)
        (Rendering|SetVisibility (Variables|Default|GetLight) false false)))
    (elif _banner_enabled
      (Components|StaticMesh|SetStaticMesh _banner_2 "/Game/PlanetSide_2/World/Meshes/Gameplay/Banner_Standing.Banner_Standing")
      (goto _label)
      (else
        (Components|StaticMesh|SetStaticMesh _banner_2 "/Game/PlanetSide_2/World/Meshes/Gameplay/Banner_Standing_Off.Banner_Standing_Off")
        (goto _label_2)))))