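; Configurable PlanetSide 2 facility tower with a faction banner, optional shields and turret mounts.
; The construction script creates the banner's dynamic material, removes components when shields or turrets are disabled, and, unless platforms-only, adds up to four lower and two upper turret meshes.
; A Turret Type macro picks each mesh: chaingun, tank cannon, flak cannon or missile launcher.
; Events swap banner material and color for NS, NC, TR or VS, and toggle shield visibility.
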(event Custom|Faction%20Switch
  (params (Faction%20Name :type Name :default "None"))
  (bind _banner_base_material (Variables|Default|GetBanner%20Base%20Material))
  (bind _banner (Variables|Default|GetBanner))
  (switch name Faction%20Name
    (:NS
      (Rendering|Material|SetMaterial _banner 1 "/Game/PlanetSide_2/World/Materials/Gameplay_Objects/Banners/M_FactionBanner.M_FactionBanner")
      (Rendering|Material|SetVectorParameterValue _banner_base_material "Color" "(R=1.000000,G=1.000000,B=1.000000,A=1.000000)" :!class /Script/Engine.MaterialInstanceDynamic))
    (:NC
      (Rendering|Material|SetMaterial _banner 1 "/Game/PlanetSide_2/World/Materials/Gameplay_Objects/Banners/MI_FactionBanner_NC.MI_FactionBanner_NC")
      (Rendering|Material|SetVectorParameterValue _banner_base_material "Color" "(R=0.000000,G=0.000000,B=1.000000,A=1.000000)" :!class /Script/Engine.MaterialInstanceDynamic))
    (:TR
      (Rendering|Material|SetMaterial _banner 1 "/Game/PlanetSide_2/World/Materials/Gameplay_Objects/Banners/MI_FactionBanner_TR.MI_FactionBanner_TR")
      (Rendering|Material|SetVectorParameterValue _banner_base_material "Color" "(R=1.000000,G=0.000000,B=0.000000,A=1.000000)" :!class /Script/Engine.MaterialInstanceDynamic))
    (:VS
      (Rendering|Material|SetMaterial _banner 1 "/Game/PlanetSide_2/World/Materials/Gameplay_Objects/Banners/MI_FactionBanner_VS.MI_FactionBanner_VS")
      (Rendering|Material|SetVectorParameterValue _banner_base_material "Color" "(R=0.305000,G=0.000000,B=0.305000,A=1.000000)" :!class /Script/Engine.MaterialInstanceDynamic))))

(event Custom|Shield%20Enable/Disable
  (params (Shield%20Enabled :type Boolean :default false))
  (Rendering|SetVisibility Shield%20Enabled true))

(fn ConstructionScript
  (bind _returnvalue (Rendering|Material|CreateDynamicMaterialInstance "/Game/PlanetSide_2/World/Materials/Gameplay_Objects/MI_FactionBanner.MI_FactionBanner" :!class /Script/Engine.KismetMaterialLibrary))
  (bind _output_get (Variables|Default|SetBanner%20Base%20Material _returnvalue))
  (Rendering|Material|SetMaterial (Variables|Default|GetBanner) 0 _output_get)
  (if (Variables|Default|GetShields%20Enabled)
    _
    (else
      (Components|DestroyComponent)))
  (if (Variables|Turrets|GetTurrets%20Enabled)
    (if (not (Variables|Turrets|GetPlatforms%20Only))
      (Utilities|FlowControl|Sequence
        (:then_0
          (if (Variables|Turrets|GetLower%20Turret%201%20Enabled)
            (bind _returnvalue_2 (AddComponent|AddStaticMeshComponent false))
            (Utilities|TurretType _returnvalue_2 (Variables|Turrets|GetLower%20Turret%201%20Type))))
        (:then_1
          (if (Variables|Turrets|GetLower%20Turret%202%20Enabled)
            (bind _returnvalue_3 (AddComponent|AddStaticMeshComponent false))
            (Utilities|TurretType _returnvalue_3 (Variables|Turrets|GetLower%20Turret%202%20Type))))
        (:then_2
          (if (Variables|Turrets|GetLower%20Turret%203%20Enabled)
            (bind _returnvalue_4 (AddComponent|AddStaticMeshComponent false))
            (Utilities|TurretType _returnvalue_4 (Variables|Turrets|GetLower%20Turret%203%20Type))))
        (:then_3
          (if (Variables|Turrets|GetLower%20Turret%204%20Enabled)
            (bind _returnvalue_5 (AddComponent|AddStaticMeshComponent false))
            (Utilities|TurretType _returnvalue_5 (Variables|Turrets|GetLower%20Turret%204%20Type))))
        (:then_4
          (if (Variables|Turrets|GetUpper%20Turret%201%20Enabled)
            (bind _returnvalue_6 (AddComponent|AddStaticMeshComponent false))
            (Utilities|TurretType _returnvalue_6 (Variables|Turrets|GetUpper%20Turret%201%20Type))))
        (:then_5
          (if (Variables|Turrets|GetUpper%20Turret%202%20Enabled)
            (bind _returnvalue_7 (AddComponent|AddStaticMeshComponent false))
            (Utilities|TurretType _returnvalue_7 (Variables|Turrets|GetUpper%20Turret%202%20Type))))))
    (else
      (Components|DestroyComponent))))