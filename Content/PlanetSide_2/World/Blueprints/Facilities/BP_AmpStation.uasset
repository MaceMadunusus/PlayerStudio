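; BP_AmpStation is the Amp Station facility Blueprint for a PlanetSide 2 world.
; Its events set the visibility of the SCU and vehicle bay shields, including their child components, from a Shield flag, and play capture audio when the facility is captured.
; When AlternateStyle is set, the construction script swaps in alternate interior meshes and destroys two components.
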(event Custom|SCU%20Shield%20Disable
  (params (Shield :type Boolean))
  (Rendering|SetVisibility (Variables|Default|GetSCU%20Shields) Shield true))

(event Custom|Vehicle%20Shield%20Dsiable
  (params (Shield :type Boolean))
  (Rendering|SetVisibility (Variables|Default|GetVehicle%20Bay%20Shields) Shield true))

(event Custom|Facility%20Captured
  (params (Captured%20By :type Name))
  (Audio|Components|Audio|Play (Variables|Default|GetCapture%20Audio) 0.0))

(fn ConstructionScript
  (if (Variables|Default|GetAlternate%20Style)
    (Components|StaticMesh|SetStaticMesh "/Game/PlanetSide_2/World/Meshes/LargeFacilities/AmpStation/AmpStation_BaseInterior_Alternative.AmpStation_BaseInterior_Alternative")
    (Components|StaticMesh|SetStaticMesh "/Game/PlanetSide_2/World/Meshes/LargeFacilities/AmpStation/AmpStation_Interior_Alternate.AmpStation_Interior_Alternate")
    (Components|StaticMesh|SetStaticMesh "/Game/PlanetSide_2/World/Meshes/LargeFacilities/AmpStation/AmpStation_Interior_CCRoom2_Alternate.AmpStation_Interior_CCRoom2_Alternate")
    (Components|StaticMesh|SetStaticMesh "/Game/PlanetSide_2/World/Meshes/LargeFacilities/AmpStation/AmpStation_Interior_CCRoom_Tunnel_Alternate.AmpStation_Interior_CCRoom_Tunnel_Alternate")
    (Components|DestroyComponent)
    (Components|DestroyComponent)))