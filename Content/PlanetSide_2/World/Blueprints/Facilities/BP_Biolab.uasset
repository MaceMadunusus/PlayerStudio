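; Biolab facility Blueprint that manages the facility's shields and capture sound.
; The construction script adds the main shield as a static mesh component, which an event later re-creates or destroys.
; Separate events toggle visibility of the SCU and vehicle bay shields, including their child components.
; The capture event plays the capture audio regardless of its Captured flag.
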(event Custom|SCU%20Shield%20Disable
  (params (Shield :type Boolean :default false))
  (Rendering|SetVisibility (Variables|Default|GetSCU%20Shields) Shield true))

(event Custom|Vehicle%20Shield%20Dsiable
  (params (Shield :type Boolean :default false))
  (Rendering|SetVisibility (Variables|Default|GetVehicle%20Bay%20Shields) Shield true))

(event Custom|Shield%20Enable/Disable
  (params (Shield :type Boolean :default false))
  (if Shield
    (bind _returnvalue (AddComponent|AddStaticMeshComponent false))
    (Variables|Default|SetShield _returnvalue)
    (else
      (Components|DestroyComponent (Variables|Default|GetShield)))))

(event Custom|Facility%20Captured
  (params (Captured :type Name))
  (Audio|Components|Audio|Play (Variables|Default|GetCapture%20Audio) 0.0))

(fn ConstructionScript
  (bind _returnvalue (AddComponent|AddStaticMeshComponent false))
  (Variables|Default|SetShield _returnvalue))