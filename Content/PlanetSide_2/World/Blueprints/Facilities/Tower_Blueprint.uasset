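; Tower facility Blueprint that shows its owning faction (NS, NC, TR or VS) on a banner.
; The construction script creates a dynamic material instance for the banner base, then applies the current faction's banner material and tints the base's Color parameter.
; The FactionSwitch event stores a new faction and repeats the same material swap and tint, duplicating the construction script's switch rather than sharing it.
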(event Custom|Faction%20Switch
  (params (Faction%20Name :type Name))
  (bind _banner_base_material (Variables|Default|GetBanner%20Base%20Material))
  (bind _banner (Variables|Default|GetBanner))
  (Variables|Default|SetFAction Faction%20Name)
  (switch name (Variables|Default|GetFAction)
    (:NS
      (Utilities|FlowControl|Sequence
        (:then_0
          (Rendering|Material|SetMaterial _banner 1 "/Game/PlanetSide_2/World/Materials/Gameplay_Objects/Banners/FactionBanner.FactionBanner"))
        (:then_2
          (Rendering|Material|SetVectorParameterValue _banner_base_material "Color" "(R=1.000000,G=1.000000,B=1.000000,A=1.000000)" :!class /Script/Engine.MaterialInstanceDynamic))))
    (:NC
      (Utilities|FlowControl|Sequence
        (:then_0
          (Rendering|Material|SetMaterial _banner 1 "/Game/PlanetSide_2/World/Materials/Gameplay_Objects/Banners/FactionBanner_NC_Inst.FactionBanner_NC_Inst"))
        (:then_2
          (Rendering|Material|SetVectorParameterValue _banner_base_material "Color" "(R=0.000000,G=0.000000,B=1.000000,A=1.000000)" :!class /Script/Engine.MaterialInstanceDynamic))))
    (:TR
      (Utilities|FlowControl|Sequence
        (:then_0
          (Rendering|Material|SetMaterial _banner 1 "/Game/PlanetSide_2/World/Materials/Gameplay_Objects/Banners/FactionBanner_TR_Inst.FactionBanner_TR_Inst"))
        (:then_2
          (Rendering|Material|SetVectorParameterValue _banner_base_material "Color" "(R=1.000000,G=0.000000,B=0.000000,A=1.000000)" :!class /Script/Engine.MaterialInstanceDynamic))))
    (:VS
      (Utilities|FlowControl|Sequence
        (:then_0
          (Rendering|Material|SetMaterial _banner 1 "/Game/PlanetSide_2/World/Materials/Gameplay_Objects/Banners/FactionBanner_VS_Inst.FactionBanner_VS_Inst"))
        (:then_2
          (Rendering|Material|SetVectorParameterValue _banner_base_material "Color" "(R=0.305000,G=0.000000,B=0.305000,A=1.000000)" :!class /Script/Engine.MaterialInstanceDynamic))))))

(fn ConstructionScript
  (bind _banner (Variables|Default|GetBanner))
  (bind _returnvalue (Rendering|Material|CreateDynamicMaterialInstance "/Game/PlanetSide_2/World/Materials/Gameplay_Objects/Faction_Banner_Inst.Faction_Banner_Inst" :!class /Script/Engine.KismetMaterialLibrary))
  (Variables|Default|SetBanner%20Base%20Material _returnvalue)
  (Rendering|Material|SetMaterial (Variables|Default|GetBanner) 0 _returnvalue)
  (switch name (Variables|Default|GetFAction)
    (:NS
      (Utilities|FlowControl|Sequence
        (:then_0
          (Rendering|Material|SetMaterial _banner 1 "/Game/PlanetSide_2/World/Materials/Gameplay_Objects/Banners/FactionBanner.FactionBanner"))
        (:then_2
          (Rendering|Material|SetVectorParameterValue (Variables|Default|GetBanner%20Base%20Material) "Color" "(R=1.000000,G=1.000000,B=1.000000,A=1.000000)" :!class /Script/Engine.MaterialInstanceDynamic))))
    (:NC
      (Utilities|FlowControl|Sequence
        (:then_0
          (Rendering|Material|SetMaterial _banner 1 "/Game/PlanetSide_2/World/Materials/Gameplay_Objects/Banners/FactionBanner_NC_Inst.FactionBanner_NC_Inst"))
        (:then_2
          (Rendering|Material|SetVectorParameterValue (Variables|Default|GetBanner%20Base%20Material) "Color" "(R=0.000000,G=0.000000,B=1.000000,A=1.000000)" :!class /Script/Engine.MaterialInstanceDynamic))))
    (:TR
      (Utilities|FlowControl|Sequence
        (:then_0
          (Rendering|Material|SetMaterial _banner 1 "/Game/PlanetSide_2/World/Materials/Gameplay_Objects/Banners/FactionBanner_TR_Inst.FactionBanner_TR_Inst"))
        (:then_2
          (Rendering|Material|SetVectorParameterValue (Variables|Default|GetBanner%20Base%20Material) "Color" "(R=1.000000,G=0.000000,B=0.000000,A=1.000000)" :!class /Script/Engine.MaterialInstanceDynamic))))
    (:VS
      (Utilities|FlowControl|Sequence
        (:then_0
          (Rendering|Material|SetMaterial _banner 1 "/Game/PlanetSide_2/World/Materials/Gameplay_Objects/Banners/FactionBanner_VS_Inst.FactionBanner_VS_Inst"))
        (:then_2
          (Rendering|Material|SetVectorParameterValue (Variables|Default|GetBanner%20Base%20Material) "Color" "(R=0.305000,G=0.000000,B=0.305000,A=1.000000)" :!class /Script/Engine.MaterialInstanceDynamic))))))