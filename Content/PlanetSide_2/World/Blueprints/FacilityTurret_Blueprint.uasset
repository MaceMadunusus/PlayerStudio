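; Configurable PlanetSide 2 facility turret made of a base mesh and a turret mesh, skinned by owning faction.
; The construction script picks the chaingun, AT, flak or missile mesh from TurretType, and WallTurret selects an offset wall-platform layout over the standard base.
; FactionSwitch updates FAction and repeats the construction script's material logic at runtime.
; Wall turrets recolor only the turret mesh, and NS reuses the NC material.
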(event Custom|Faction%20Switch
  (params (Faction%20Name :type Name))
  (bind _facilityturret (Variables|Default|GetFacilityTurret))
  (bind _facilityturret_base (Variables|Default|GetFacilityTurret_Base))
  (Variables|Turret|SetFAction Faction%20Name)
  (if (Variables|Turret|GetWall%20Turret)
    (switch name (Variables|Turret|GetFAction)
      (:NS
        (Rendering|Material|SetMaterial _facilityturret 0 "/Game/PlanetSide_2/World/Materials/Turrets/TurretBase_NC.TurretBase_NC"))
      (:NC
        (Rendering|Material|SetMaterial _facilityturret 0 "/Game/PlanetSide_2/World/Materials/Turrets/TurretBase_NC.TurretBase_NC"))
      (:TR
        (Rendering|Material|SetMaterial _facilityturret 0 "/Game/PlanetSide_2/World/Materials/Turrets/TurretBase_TR.TurretBase_TR"))
      (:VS
        (Rendering|Material|SetMaterial _facilityturret 0 "/Game/PlanetSide_2/World/Materials/Turrets/TurretBase_VS.TurretBase_VS")))
    (else
      (switch name (Variables|Turret|GetFAction)
        (:NS
          (Rendering|Material|SetMaterial _facilityturret_base 0 "/Game/PlanetSide_2/World/Materials/Turrets/TurretBase_NC.TurretBase_NC"))
        (:NC
          (Rendering|Material|SetMaterial _facilityturret_base 0 "/Game/PlanetSide_2/World/Materials/Turrets/TurretBase_NC.TurretBase_NC"))
        (:TR
          (Rendering|Material|SetMaterial _facilityturret_base 0 "/Game/PlanetSide_2/World/Materials/Turrets/TurretBase_TR.TurretBase_TR"))
        (:VS
          (Rendering|Material|SetMaterial _facilityturret_base 0 "/Game/PlanetSide_2/World/Materials/Turrets/TurretBase_VS.TurretBase_VS"))))))

(fn ConstructionScript
  (bind _facilityturret (Variables|Default|GetFacilityTurret))
  (bind _facilityturret_2 (Variables|Default|GetFacilityTurret))
  (bind _facilityturret_base (Variables|Default|GetFacilityTurret_Base))
  (bind _facilityturret_base_2 (Variables|Default|GetFacilityTurret_Base))
  (Utilities|FlowControl|Sequence
    (:then_0
      (switch int (Variables|Turret|GetTurret%20Type)
        (:1
          (Components|StaticMesh|SetStaticMesh _facilityturret "/Game/PlanetSide_2/World/Meshes/Gameplay/FacilityTurret_Chaingun.FacilityTurret_Chaingun"))
        (:2
          (Components|StaticMesh|SetStaticMesh _facilityturret "/Game/PlanetSide_2/World/Meshes/Gameplay/FacilityTurret_AT.FacilityTurret_AT"))
        (:3
          (Components|StaticMesh|SetStaticMesh _facilityturret "/Game/PlanetSide_2/World/Meshes/Gameplay/FacilityTurret_Flak.FacilityTurret_Flak"))
        (:4
          (Components|StaticMesh|SetStaticMesh _facilityturret "/Game/PlanetSide_2/World/Meshes/Gameplay/FacilityTurret_Missile.FacilityTurret_Missile"))))
    (:then_1
      (if (Variables|Turret|GetWall%20Turret)
        (Components|StaticMesh|SetStaticMesh _facilityturret_base "/Game/PlanetSide_2/World/Meshes/Gameplay/FacilityTurret_Platform.FacilityTurret_Platform")
        (Transformation|SetRelativeRotation _facilityturret_base "0,90.000000, 0" false)
        (Transformation|SetRelativeLocation (Variables|Default|GetFacilityTurret) "0,610.000000,20.000000" false)
        (switch name (Variables|Turret|GetFAction)
          (:NS
            (Rendering|Material|SetMaterial _facilityturret_2 0 "/Game/PlanetSide_2/World/Materials/Turrets/TurretBase_NC.TurretBase_NC"))
          (:NC
            (Rendering|Material|SetMaterial _facilityturret_2 0 "/Game/PlanetSide_2/World/Materials/Turrets/TurretBase_NC.TurretBase_NC"))
          (:TR
            (Rendering|Material|SetMaterial _facilityturret_2 0 "/Game/PlanetSide_2/World/Materials/Turrets/TurretBase_TR.TurretBase_TR"))
          (:VS
            (Rendering|Material|SetMaterial _facilityturret_2 0 "/Game/PlanetSide_2/World/Materials/Turrets/TurretBase_VS.TurretBase_VS")))
        (else
          (Components|StaticMesh|SetStaticMesh _facilityturret_base "/Game/PlanetSide_2/World/Meshes/Gameplay/FacilityTurret_Base.FacilityTurret_Base")
          (switch name (Variables|Turret|GetFAction)
            (:NS
              (Rendering|Material|SetMaterial _facilityturret_base_2 0 "/Game/PlanetSide_2/World/Materials/Turrets/TurretBase_NC.TurretBase_NC"))
            (:NC
              (Rendering|Material|SetMaterial _facilityturret_base_2 0 "/Game/PlanetSide_2/World/Materials/Turrets/TurretBase_NC.TurretBase_NC"))
            (:TR
              (Rendering|Material|SetMaterial _facilityturret_base_2 0 "/Game/PlanetSide_2/World/Materials/Turrets/TurretBase_TR.TurretBase_TR"))
            (:VS
              (Rendering|Material|SetMaterial _facilityturret_base_2 0 "/Game/PlanetSide_2/World/Materials/Turrets/TurretBase_VS.TurretBase_VS"))))))))