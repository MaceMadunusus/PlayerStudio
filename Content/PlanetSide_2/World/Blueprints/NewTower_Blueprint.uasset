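; Configurable PlanetSide 2 tower Blueprint with seven lower and eight upper turret mounts, eight blast shields, and faction-based turret skins.
; The construction script runs a shared helper per mount that, when enabled, shows the platform and swaps the turret mesh by type.
; It also applies the faction material (NS reuses NC's) and toggles shield visibility.
; Events switch faction and toggle interior or exterior lights.
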(event Custom|Exterior%20Lights%20On/Off
  (params (Lights%20Enabled :type Boolean))
  (Rendering|SetVisibility (Variables|Default|GetExterior%20Lights) Lights%20Enabled true))

(event Custom|Faction%20Switch
  (params (Faction%20Name :type Name))
  (bind _lower_turret (Variables|Turret|GetLower%20Turret))
  (Variables|Turret|SetFAction Faction%20Name)
  (switch name (Variables|Turret|GetFAction)
    (:NS
      (Rendering|Material|SetMaterial _lower_turret 0 "/Game/PlanetSide_2/World/Materials/Turrets/TurretBase_NC.TurretBase_NC"))
    (:NC
      (Rendering|Material|SetMaterial _lower_turret 0 "/Game/PlanetSide_2/World/Materials/Turrets/TurretBase_NC.TurretBase_NC"))
    (:TR
      (Rendering|Material|SetMaterial _lower_turret 0 "/Game/PlanetSide_2/World/Materials/Turrets/TurretBase_TR.TurretBase_TR"))
    (:VS
      (Rendering|Material|SetMaterial _lower_turret 0 "/Game/PlanetSide_2/World/Materials/Turrets/TurretBase_VS.TurretBase_VS"))))

(event Custom|Interior%20Lights%20On/Off
  (params (Lights%20Enabled :type Boolean))
  (Rendering|SetVisibility (Variables|Default|GetInterior%20Lights) Lights%20Enabled true))

(fn ConstructionScript
  (bind _lower_turret (Variables|Turret|GetLower%20Turret))
  (Utilities|FlowControl|Sequence
    (:then_0
      ;[1 1 1] Lower Turret Type Selection
      (Utilities|FlowControl|Sequence
        (:then_0
          (PlanetSide2|TurretTypeSelectionforTowers (Variables|LowerTurrets|GetLower%20Turret%201%20Type) (Variables|Turret|GetLower%20Turret) (Variables|Turret|GetLower%20Platform%201) (Variables|LowerTurrets|GetLower%20Turret%201%20Enabled)))
        (:then_1
          (PlanetSide2|TurretTypeSelectionforTowers (Variables|LowerTurrets|GetLower%20Turret%202%20Type) (Variables|Turret|GetLower%20Turret%202) (Variables|Turret|GetLower%20Platform%202) (Variables|LowerTurrets|GetLower%20Turret%202%20Enabled)))
        (:then_2
          (PlanetSide2|TurretTypeSelectionforTowers (Variables|LowerTurrets|GetLower%20Turret%203%20Type) (Variables|Turret|GetLower%20Turret%203) (Variables|Turret|GetLower%20Platform%203) (Variables|LowerTurrets|GetLower%20Turret%203%20Enabled)))
        (:then_3
          (PlanetSide2|TurretTypeSelectionforTowers (Variables|LowerTurrets|GetLower%20Turret%204%20Type) (Variables|Turret|GetLower%20Turret%204) (Variables|Turret|GetLower%20Platform%204) (Variables|LowerTurrets|GetLower%20Turret%204%20Enabled)))
        (:then_4
          (PlanetSide2|TurretTypeSelectionforTowers (Variables|LowerTurrets|GetLower%20Turret%205%20Type) (Variables|Turret|GetLower%20Turret%205) (Variables|Turret|GetLower%20Platform%205) (Variables|LowerTurrets|GetLower%20Turret%205%20Enabled)))
        (:then_5
          (PlanetSide2|TurretTypeSelectionforTowers (Variables|LowerTurrets|GetLower%20Turret%206%20Type) (Variables|Turret|GetLower%20Turret%206) (Variables|Turret|GetLower%20Platform%206) (Variables|LowerTurrets|GetLower%20Turret%206%20Enabled)))
        (:then_6
          (PlanetSide2|TurretTypeSelectionforTowers (Variables|LowerTurrets|GetLower%20Turret%207%20Type) (Variables|Turret|GetLower%20Turret%207) (Variables|Turret|GetLower%20Platform%207) (Variables|LowerTurrets|GetLower%20Turret%207%20Enabled)))))
    (:then_1
      ;[1 1 1] Upper Turret Type Selection
      (Utilities|FlowControl|Sequence
        (:then_0
          (PlanetSide2|TurretTypeSelectionforTowers (Variables|UpperTurrets|GetUpper%20Turret%201%20Type) (Variables|Turret|GetUpper%20Turret%201) (Variables|Turret|GetTop%20Platform%201) (Variables|UpperTurrets|GetUpper%20Turret%201%20Enabled)))
        (:then_1
          (PlanetSide2|TurretTypeSelectionforTowers (Variables|UpperTurrets|GetUpper%20Turret%202%20Type) (Variables|Turret|GetUpper%20Turret%202) (Variables|Turret|GetTop%20Platform%202) (Variables|UpperTurrets|GetUpper%20Turret%202%20Enabled)))
        (:then_2
          (PlanetSide2|TurretTypeSelectionforTowers (Variables|UpperTurrets|Getupper%20Turret%203%20Type) (Variables|Turret|GetUpper%20Turret%203) (Variables|Turret|GetTop%20Platform%203) (Variables|UpperTurrets|GetUpper%20Turret%203%20Enabled)))
        (:then_3
          (PlanetSide2|TurretTypeSelectionforTowers (Variables|UpperTurrets|Getupper%20Turret%204%20Type) (Variables|Turret|GetUpper%20Turret%204) (Variables|Turret|GetTop%20Platform%204) (Variables|UpperTurrets|GetUpper%20Turret%204%20Enabled)))
        (:then_4
          (PlanetSide2|TurretTypeSelectionforTowers (Variables|UpperTurrets|GetUpper%20Turret%205%20Type) (Variables|Turret|GetUpper%20Turret%205) (Variables|Turret|GetTop%20Platform%205) (Variables|UpperTurrets|GetUpper%20Turret%205%20Enabled)))
        (:then_5
          (PlanetSide2|TurretTypeSelectionforTowers (Variables|UpperTurrets|GetUpper%20Turret%206%20Type) (Variables|Turret|GetUpper%20Turret%206) (Variables|Turret|GetTop%20Platform%206) (Variables|UpperTurrets|GetUpper%20Turret%206%20Enabled)))
        (:then_6
          (PlanetSide2|TurretTypeSelectionforTowers (Variables|UpperTurrets|GetUpper%20Turret%207%20Type) (Variables|Turret|GetUpper%20Turret%207) (Variables|Turret|GetTop%20Platform%207) (Variables|UpperTurrets|GetUpper%20Turret%207%20Enabled)))
        (:then_7
          (PlanetSide2|TurretTypeSelectionforTowers (Variables|UpperTurrets|GetUpper%20Turret%208%20Type) (Variables|Turret|Getupper%20Turret%208) (Variables|Turret|GetTop%20Platform%208) (Variables|UpperTurrets|GetUpper%20Turret%208%20Enabled)))))
    (:then_2
      ;[1 1 1] Faction Selection
      (switch name (Variables|Turret|GetFAction)
        (:NS
          (Rendering|Material|SetMaterial _lower_turret 0 "/Game/PlanetSide_2/World/Materials/Turrets/TurretBase_NC.TurretBase_NC"))
        (:NC
          (Rendering|Material|SetMaterial _lower_turret 0 "/Game/PlanetSide_2/World/Materials/Turrets/TurretBase_NC.TurretBase_NC"))
        (:TR
          (Rendering|Material|SetMaterial _lower_turret 0 "/Game/PlanetSide_2/World/Materials/Turrets/TurretBase_TR.TurretBase_TR"))
        (:VS
          (Rendering|Material|SetMaterial _lower_turret 0 "/Game/PlanetSide_2/World/Materials/Turrets/TurretBase_VS.TurretBase_VS"))))
    (:then_3
      ;[1 1 1] Blastshields
      (Utilities|FlowControl|Sequence
        (:then_0
          (Rendering|SetVisibility (Variables|Blastshield|GetBlastshield1) (Variables|Blastshield|GetBlastshield%201%20Enable) false))
        (:then_1
          (Rendering|SetVisibility (Variables|Blastshield|GetBlastShield2) (Variables|Blastshield|GetBlastshield%202%20Enable) false))
        (:then_2
          (Rendering|SetVisibility (Variables|Blastshield|GetBlastShield3) (Variables|Blastshield|GetBlastshield%203%20enable) false))
        (:then_3
          (Rendering|SetVisibility (Variables|Blastshield|GetBlastShield4) (Variables|Blastshield|GetBlastshield%204%20Enable) false))
        (:then_4
          (Rendering|SetVisibility (Variables|Blastshield|GetBlastShield5) (Variables|Blastshield|GetBlastshield%205%20Enable) false))
        (:then_5
          (Rendering|SetVisibility (Variables|Blastshield|GetBlastShield6) (Variables|Blastshield|GetBlastshield%206%20Enable) false))
        (:then_6
          (Rendering|SetVisibility (Variables|Blastshield|GetBlastShield7) (Variables|Blastshield|GetBlastshield%207%20Enable) false))
        (:then_7
          (Rendering|SetVisibility (Variables|Blastshield|GetBlastShield8) (Variables|Blastshield|GetBlastshield%208%20Enable) false))))))

(fn TurretTypeSelectionforTowers
  (params (Turret%20Type :type Integer) (Turret%20Selection :type Static%20Mesh%20Component%20Object%20Reference) (Platform%20Mesh%20Target :type Scene%20Component%20Object%20Reference) (Turret%20On/Off :type Boolean))
  (if Turret%20On/Off
    (Rendering|SetVisibility Platform%20Mesh%20Target true true)
    (Variables|Default|SetTurret%20Select Turret%20Selection)
    (switch int Turret%20Type
      (:1
        (Components|StaticMesh|SetStaticMesh (Variables|Default|GetTurret%20Select) "/Game/PlanetSide_2/World/Meshes/Gameplay/FacilityTurret_Chaingun.FacilityTurret_Chaingun"))
      (:2
        (Components|StaticMesh|SetStaticMesh (Variables|Default|GetTurret%20Select) "/Game/PlanetSide_2/World/Meshes/Gameplay/FacilityTurret_AT.FacilityTurret_AT"))
      (:3
        (Components|StaticMesh|SetStaticMesh (Variables|Default|GetTurret%20Select) "/Game/PlanetSide_2/World/Meshes/Gameplay/FacilityTurret_Flak.FacilityTurret_Flak"))
      (:4
        (Components|StaticMesh|SetStaticMesh (Variables|Default|GetTurret%20Select) "/Game/PlanetSide_2/World/Meshes/Gameplay/FacilityTurret_Missile.FacilityTurret_Missile"))))
  (return))