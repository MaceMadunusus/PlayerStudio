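; MiningPlatform Blueprint builds a tiled mining platform whose style and grid size are configurable.
; Its construction script optionally swaps in a second mesh for PlatformStyle 2, then adds mesh instances spaced by TileLength.
; Nested loops extend the grid along positive X and negative Y, and do not add the origin tile.
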(fn ConstructionScript
  (switch int (Variables|Platform|GetPlatform%20Style)
    (:1
      _)
    (:2
      (Components|StaticMesh|SetStaticMesh (Variables|Default|GetMiningPlatform) "/Game/PlanetSide_2/World/Meshes/MiningPlatform2.MiningPlatform2")))
  (Utilities|FlowControl|Sequence
    (:then_0
      (for _index (range 1 (- (Variables|Platform|GetTiling%20Count%20X) 1))
        (Components|InstancedStaticMesh|AddInstance (Variables|Default|GetMiningPlatform) (Math|Transform|MakeTransform (Math|Vector|MakeVector (* _index (Variables|Platform|GetTile%20Length)) 0.0 0.0)))))
    (:then_1
      (for _index_2 (range 1 (- (Variables|Platform|GetTiling%20Count%20Y) 1))
        (Components|InstancedStaticMesh|AddInstance (Variables|Default|GetMiningPlatform) (Math|Transform|MakeTransform (Math|Vector|MakeVector 0.0 (* (* _index_2 (Variables|Platform|GetTile%20Length)) -1.0) 0.0)))
        (for _index_3 (range 1 (- (Variables|Platform|GetTiling%20Count%20X) 1))
          (Components|InstancedStaticMesh|AddInstance (Variables|Default|GetMiningPlatform) (Math|Transform|MakeTransform (Math|Vector|MakeVector (* _index_3 (Variables|Platform|GetTile%20Length)) (* (* _index_2 (Variables|Platform|GetTile%20Length)) -1.0) 0.0))))))))