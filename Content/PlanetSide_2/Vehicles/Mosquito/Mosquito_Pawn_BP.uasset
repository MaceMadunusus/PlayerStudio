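; Player-flown Mosquito aircraft pawn from a PlanetSide 2 project, with physics flight, afterburner, chaingun and switchable cockpit/chase cameras.
; Tick adds forward-only and vertical velocity from input and applies local rotations.
; Speed along the actor's right vector, its nose axis, selects flight or hover mode, aiming the fuel-limited afterburner forward or up.
; Held fire loops through a gate and retriggerable delay, spawning Needler bullets at an offset.
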(event EventBeginPlay
  ;[1 1 1] Calculate speed
  (Variables|Default|SetOld%20Position (Transformation|GetActorLocation (Game|Player|GetPlayerPawn 0))))

(event EventActorBeginOverlap
  (params (OtherActor :type Actor%20Object%20Reference)))

(event EventTick
  (params (DeltaSeconds :type Float%20%28single-precision%29))
  (Variables|Default|SetDelta%20Seconds DeltaSeconds)
  ;[1 1 1] Movement
  (Physics|SetPhysicsLinearVelocity (Variables|Default|GetMosquito) (* (* (Math|Vector|GetRightVector (Transformation|GetActorRotation)) (* (Math|Float|Clamp(Float) 0.0 (Input|AxisValues|GetMoveForward)) (Variables|Movement|GetSpeedForward))) (Variables|Default|GetDelta%20Seconds)) true "None")
  (Physics|SetPhysicsLinearVelocity (Variables|Default|GetMosquito) (* (* (Math|Vector|GetUpVector (Transformation|GetActorRotation)) (* (Input|AxisValues|GetMoveUp) (Variables|Movement|GetAscend%20Speed))) (Variables|Default|GetDelta%20Seconds)) true "None")
  (Transformation|AddActorLocalRotation (Class|KismetMathLibrary|MakeRot 0.0 0.0 (* (Input|AxisValues|GetPitch) (Variables|Movement|GetPitch%20Speed))) false)
  (Transformation|AddActorLocalRotation (Class|KismetMathLibrary|MakeRot 0.0 (* (Input|AxisValues|GetYaw/moveRight) (Variables|Movement|GetYaw%20speed)) 0.0) false)
  (Transformation|AddActorLocalRotation (Class|KismetMathLibrary|MakeRot (* (Input|AxisValues|GetRoll/turn) (Variables|Movement|GetRoll%20Speed)) 0.0 0.0) false)
  ;[1 1 1] Calculates speed along local x-axis. Sets flightmode/hovermode
  (bind _returnvalue (Physics|GetPhysicsLinearVelocity (Variables|Default|GetMosquito) "None"))
  (Variables|Default|SetIs%20in%20flightmode? (>= (* (Math|Vector|VectorLength (Math|Vector|MakeVector (Math|Float|Max(Float) (.X (Math|Vector|BreakVector (* _returnvalue (Math|Vector|GetRightVector (Transformation|GetActorRotation))))) 0.0) (Math|Float|Max(Float) (.Y (Math|Vector|BreakVector (* _returnvalue (Math|Vector|GetRightVector (Transformation|GetActorRotation))))) 0.0) (Math|Float|Max(Float) (.Z (Math|Vector|BreakVector (* _returnvalue (Math|Vector|GetRightVector (Transformation|GetActorRotation))))) 0.0))) 0.036) 8e+01))
  ;[1 1 1] AfterBurner
  (if (Variables|Default|GetAfterBurner%20On?)
    (if (Variables|Default|GetIs%20in%20flightmode?)
      (Class|PrimitiveComponent|SetAllPhysicsLinearVelocity (Variables|Default|GetMosquito) (* (Math|Vector|GetRightVector (Transformation|GetActorRotation)) (Variables|Afterburner|GetAfterBurner%20speed)) true)
      (Utilities|FlowControl|Delay 0.1)
      (Variables|Afterburner|SetCurrent%20AB (Math|Float|Clamp(Float) (- (Variables|Afterburner|GetCurrent%20AB) 4.0) 0.0 (Variables|Afterburner|GetMax%20AB)))
      (if (<= (Variables|Afterburner|GetCurrent%20AB) 1e+01)
        (Variables|Afterburner|SetAfterBurner%20speed 0.0)
        (else
          (Variables|Afterburner|SetAfterBurner%20speed 1e+02)))
      (else
        (Class|PrimitiveComponent|SetAllPhysicsLinearVelocity (Variables|Default|GetMosquito) (* (Math|Vector|GetUpVector (Transformation|GetActorRotation)) (Variables|Afterburner|GetAfterBurner%20speed)) true)
        (Utilities|FlowControl|Delay 0.1)
        (Variables|Afterburner|SetCurrent%20AB (Math|Float|Clamp(Float) (- (Variables|Afterburner|GetCurrent%20AB) 4.0) 0.0 (Variables|Afterburner|GetMax%20AB)))
        (if (<= (Variables|Afterburner|GetCurrent%20AB) 1e+01)
          (Variables|Afterburner|SetAfterBurner%20speed 0.0)
          (else
            (Variables|Afterburner|SetAfterBurner%20speed 1e+02)))))
    (else
      (Utilities|FlowControl|Delay 1.0)
      (Variables|Afterburner|SetCurrent%20AB (Math|Float|Clamp(Float) (+ (Variables|Afterburner|GetCurrent%20AB) 1e+01) 0.0 (Variables|Afterburner|GetMax%20AB))))))

(event Input|ActionEvents|InputActionChangeView
  ;[1 1 1] Change view
  (:Pressed
    (CallFunction|EnableInternalView (not (Variables|Default|GetIs%20in%20Vehicle?)))))

(event Input|ActionEvents|InputActionFire
  (bind _returnvalue (Transformation|GetActorRotation))
  (bind _gun_audio (Variables|Default|GetGun%20Audio))
  ;[1 1 1] Fire weapon
  (:Pressed
    (Audio|Components|Audio|Play _gun_audio 0.0)
    (Utilities|FlowControl|Sequence
      (:then_0
        (goto _label Open))
      (:then_1
        (Utilities|FlowControl|Gate true :!label _label
          (:Exit
            (Utilities|FlowControl|Sequence
              (:then_0
                (Game|SpawnActorfromClass "/Game/PlanetSide_2/Vehicles/Mosquito/Needler_Bullet_BP.Needler_Bullet_BP_C" (Math|Transform|MakeTransform (+ (Transformation|GetActorLocation) (Math|Vector|RotateVector (Variables|Gun|GetGunOffSet) _returnvalue)) _returnvalue) false 3.0 0) ; Spawn projectile
              )
              (:then_1
                (Utilities|FlowControl|RetriggerableDelay (Variables|Gun|GetFire%20Rate))
                (goto _label))))))))
  (:Released
    (Audio|Components|Audio|Stop _gun_audio)
    (Class|GameplayStatics|PlaySoundAttached "/Game/PlanetSide_2/Audio/Weapons/WPN_VEH_12MM_MOSQUITO_CHAINGUN_2D_SHOOT_END_Cue.WPN_VEH_12MM_MOSQUITO_CHAINGUN_2D_SHOOT_END_Cue" _gun_audio)
    (goto _label Close)))

(event Input|ActionEvents|InputActionAfterBurner/Run
  (bind _engine (Variables|Default|GetEngine))
  ;[1 1 1] AfterBurner
  (:Pressed
    (Variables|Default|SetAfterBurner%20On? true)
    (Class|GameplayStatics|PlaySoundAttached "/Game/PlanetSide_2/Audio/Vehicle/Mosquito/VEH_MOSQUITO_ENG_BOOST_ON_Cue.VEH_MOSQUITO_ENG_BOOST_ON_Cue" _engine))
  (:Released
    (Variables|Default|SetAfterBurner%20On? false)
    (Class|GameplayStatics|PlaySoundAttached "/Game/PlanetSide_2/Audio/Vehicle/Mosquito/VEH_MOSQUITO_ENG_BOOST_OFF_Cue.VEH_MOSQUITO_ENG_BOOST_OFF_Cue" _engine)))

(fn ConstructionScript)

(fn EnableInternalView
  (params (State :type Boolean :default false))
  (bind _internal_camera (Variables|Default|GetInternal%20camera))
  (bind _chase_camera (Variables|Default|GetChase%20Camera))
  (Variables|Default|SetIs%20in%20Vehicle? State)
  (if (Variables|Default|GetIs%20in%20Vehicle?)
    (Components|Activation|Activate _internal_camera false)
    (Components|Activation|Deactivate _chase_camera)
    (else
      (Components|Activation|Deactivate _internal_camera)
      (Components|Activation|Activate _chase_camera false))))