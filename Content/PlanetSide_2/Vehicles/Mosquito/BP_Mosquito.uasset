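; Player-flyable Mosquito aircraft from a PlanetSide 2 project, with afterburner, switchable cockpit/chase cameras, enter/exit and a loadout options menu.
; Construction script attaches the weapon child actor, optional fins, utility mesh and glass material.
; Tick runs shared flight, hover and afterburner-fuel helpers, feeding HUD and panel widgets.
; Input drives the primary weapon; secondary only updates selection, and the flare ability only plays sound and cooldown.
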(event OnComponentBeginOverlap(Capsule)
  (params (OtherActor :type Actor%20Object%20Reference) (OtherComp :type Primitive%20Component%20Object%20Reference) (OtherBodyIndex :type Integer) (bFromSweep :type Boolean) (SweepResult :type Hit%20Result%20Structure%20%28by%20ref%29))
  ;[1 1 1] Player in enterable range.
  (CallFunction|SetVehicleTarget OtherActor self))

(event OnComponentEndOverlap(Capsule)
  (params (OtherActor :type Actor%20Object%20Reference) (OtherComp :type Primitive%20Component%20Object%20Reference) (OtherBodyIndex :type Integer))
  ;[1 1 1] Player in enterable range.
  (CallFunction|SetVehicleTarget OtherActor))

(event Custom|Updated%20Weapon
  (bind _weapon_component (Variables|Vehicle|GetWeapon%20Component))
  (Class|SceneComponent|Attachto _weapon_component (Variables|Default|GetVehicle) "Primary Weapon" "SnapToTarget" true)
  (bind _asbp_weapon_base (Utilities|Casting|CastToBP_Weapon_Base (Variables|/Script/Engine.ChildActorComponent|GetChildActor _weapon_component)))
  (Variables|Gun|SetWeapon%20Base _asbp_weapon_base))

(event EventPossessed
  (params (NewController :type Controller%20Object%20Reference))
  (bind _returnvalue (Game|GetPlayerController 0))
  ;[1 1 1] Create HUD
  (bind _returnvalue_2 (UserInterface|CreateWidget "/Game/PlanetSide_2/UI/HUD_Mosquito.HUD_Mosquito_C" _returnvalue))
  (Variables|Default|SetVehicle%20HUD _returnvalue_2)
  (bind _asbp_weapon_base (Utilities|Casting|CastToBP_Weapon_Base (Variables|/Script/Engine.ChildActorComponent|GetChildActor (Variables|Vehicle|GetWeapon%20Component))))
  (Variables|/Game/PlanetSide_2/Weapons/BP_Weapon_Base.BP_Weapon_Base_C|SetPanel%20Widget _asbp_weapon_base (Variables|HUD|GetPanelWidget))
  (Variables|Gun|SetWeapon%20Base _asbp_weapon_base)
  (bind _returnvalue_3 (UserInterface|CreateWidget "/Game/PlanetSide_2/UI/MosquitoOptions.MosquitoOptions_C" _returnvalue self))
  (Variables|Default|SetOptions _returnvalue_3))

(event EventTick
  (params (DeltaSeconds :type Float%20%28single-precision%29))
  (bind _self self)
  (bind _afterburner_max_fuel (Variables|Default|GetAfterburner%20Max%20Fuel))
  (bind _panelwidget (Variables|HUD|GetPanelWidget))
  ;[1 1 1] Movement
  (bind _output_get (Variables|Default|SetDelta%20Seconds DeltaSeconds))
  (Default|MovementAircraft self _output_get (Variables|Default|GetForward%20Speed) (Variables|Default|GetAscend%20Speed) (Variables|Default|GetPitch%20Rate) (Variables|Default|GetYaw%20Rate) (Variables|Default|GetRoll%20Rate))
  ;[1 1 1] Calculates speed along local x-axis. Sets flightmode/hovermode and displays it on HUD
  (bind (_camera_rotation _speed) (CallFunction|CalculateFlightSpeed&SetHoverMode (Variables|Default|GetHover%20Speed) (Variables|Default|GetEngine) (Utilities|Array|MakeArray (Variables|Default|GetTrail%20FL) (Variables|Default|GetTrail%20FR) (Variables|Default|GetTrail%20RL) (Variables|Default|GetTrail%20RR))))
  (bind _ashud_mosquito (Utilities|Casting|CastToHUD_Mosquito (Variables|Default|GetVehicle%20HUD)))
  (Default|HUDCurrentRotation _ashud_mosquito _camera_rotation)
  (Class|BPIAircraftInterface|HUDCurrentSpeed(Message) (UserInterface|GetUserWidgetObject (Variables|HUD|GetSpeedWidget)) _speed)
  ;[1 1 1] AfterBurner
  (if (Variables|Default|GetIsAfterburnerOn)
    (Default|Afterburneron _self _self (Variables|Default|GetEngine) (Variables|Default|GetAfterburner%20Fuel%20Drain) _afterburner_max_fuel (Variables|Default|GetAfterburner%20Min%20Fuel) (Variables|Default|GetAfterburner%20Max%20Speed) _panelwidget)
    (else
      (Utilities|FlowControl|Delay (Variables|Default|GetAfterburner%20Fuel%20Regen%20Delay))
      (CallFunction|AfterburnerOff _afterburner_max_fuel (Variables|Default|GetAfterburner%20Fuel%20Regen) _panelwidget))))

(event Input|ActionEvents|InputActionChangeView
  (params (Key :type Key%20Structure :default "AnyKey"))
  ;[1 1 1] Change view
  (:Pressed
    (CallFunction|SwitchCamera (Variables|Default|GetIsInVehicle) (Variables|Default|GetInternal%20camera) (Variables|Default|GetChase%20Camera) (Variables|Default|GetMosquito_Cockpit) (Variables|Default|GetVehicle) (Variables|Default|GetEngine))))

(event Input|ActionEvents|InputActionAbility
  (params (Key :type Key%20Structure :default "AnyKey"))
  (bind _panelwidget (Variables|HUD|GetPanelWidget))
  (bind _returnvalue (UserInterface|GetUserWidgetObject _panelwidget))
  ;[1 1 1] Use Ability
  (:Pressed
    (if (not (Variables|Default|GetIsAbilityOnCooldown))
      (Class|BPIAircraftInterface|AbilityonCooldown(Message) _returnvalue)
      (Variables|Default|SetIsAbilityOnCooldown true)
      (Audio|SpawnSoundAttached "/Game/PlanetSide_2/Audio/Item/Flare_Launcher.Flare_Launcher" (Variables|Vehicle|GetUtility%20Mesh%20Component))
      (Utilities|FlowControl|Delay (Variables|Default|GetAbility%20Cooldown))
      (Class|BPIAircraftInterface|AbilityOffCooldown(Message) _returnvalue)
      (Variables|Default|SetIsAbilityOnCooldown false))))

(event Input|ActionEvents|InputActionFire
  (params (Key :type Key%20Structure :default "AnyKey"))
  (bind _active_weapon_slot (Variables|Gun|GetActive%20Weapon%20Slot))
  (bind _weapon_base (Variables|Gun|GetWeapon%20Base))
  ;[1 1 1] Fire weapon
  (:Pressed
    (switch Utilities|FlowControl|Switch|SwitchonEAircraftWeaponSlot _active_weapon_slot
      (:NewEnumerator0
        (Default|Fire _weapon_base))))
  (:Released
    (switch Utilities|FlowControl|Switch|SwitchonEAircraftWeaponSlot _active_weapon_slot
      (:NewEnumerator0
        (Default|StopFiring _weapon_base)))))

(event Input|ActionEvents|InputActionReload
  (params (Key :type Key%20Structure :default "AnyKey"))
  ;[1 1 1] Reload
  (:Pressed
    (switch Utilities|FlowControl|Switch|SwitchonEAircraftWeaponSlot (Variables|Gun|GetActive%20Weapon%20Slot)
      (:NewEnumerator0
        (Default|Reload (Variables|Gun|GetWeapon%20Base))))))

(event Input|ActionEvents|InputActionAfterBurner/Run
  (params (Key :type Key%20Structure :default "AnyKey"))
  (bind _engine (Variables|Default|GetEngine))
  ;[1 1 1] AfterBurner
  (:Pressed
    (Variables|Default|SetIsAfterburnerOn true)
    (bind _returnvalue (Audio|SpawnSoundAttached "/Game/PlanetSide_2/Audio/Vehicle/Mosquito/VEH_MOSQUITO_ENG_BOOST_ON_Cue.VEH_MOSQUITO_ENG_BOOST_ON_Cue" _engine))
    (Effects|Components|ParticleSystem|SetBoolParameter _returnvalue "Inside" false :!label _label))
  (:Released
    (Variables|Default|SetIsAfterburnerOn false)
    (bind _returnvalue_2 (Audio|SpawnSoundAttached "/Game/PlanetSide_2/Audio/Vehicle/Mosquito/VEH_MOSQUITO_ENG_BOOST_OFF_Cue.VEH_MOSQUITO_ENG_BOOST_OFF_Cue" _engine))
    (goto _label)))

(event Input|KeyboardEvents|U
  (params (Key :type Key%20Structure :default "AnyKey"))
  (bind _returnvalue (Game|GetPlayerController 0))
  (bind _options (Variables|Default|GetOptions))
  (:Pressed
    (Utilities|FlowControl|FlipFlop
      (:A
        (UserInterface|Viewport|AddtoViewport _options 0)
        (Input|SetInputModeGameandUI _returnvalue _options true true)
        (Components|Activation|Activate (Variables|Default|GetWeaponCam1) false)
        (Components|Activation|Deactivate (Variables|Default|GetInternal%20camera)))
      (:B
        (Widget|RemovefromParent _options)
        (Input|SetInputModeGameOnly _returnvalue)
        (if (Variables|Default|GetIsInVehicle)
          (Components|Activation|Activate (Variables|Default|GetInternal%20camera) false)
          (else
            (Components|Activation|Activate (Variables|Default|GetChase%20Camera) false)))
        (Components|Activation|Deactivate (Variables|Default|GetWeaponCam1))))))

(event Input|KeyboardEvents|1
  (params (Key :type Key%20Structure :default "AnyKey"))
  ;[1 1 1] Switch Weapons
  (:Pressed
    (Class|BPIAircraftInterface|SetWeaponPrimary(Message) (UserInterface|GetUserWidgetObject (Variables|HUD|GetPanelWidget)) "NewEnumerator0")
    (Default|SetWeaponPrimary (Variables|HUD|GetMosquitoHUD) "NewEnumerator0")
    (Variables|Gun|SetActive%20Weapon%20Slot "NewEnumerator0")))

(event Input|KeyboardEvents|2
  (params (Key :type Key%20Structure :default "AnyKey"))
  (bind _weapon_base (Variables|Gun|GetWeapon%20Base))
  ;[1 1 1] Switch Weapons
  (:Pressed
    (Class|BPIAircraftInterface|SetWeaponSecondary(Message) (UserInterface|GetUserWidgetObject (Variables|HUD|GetPanelWidget)) "NewEnumerator1")
    (Default|SetWeaponSecondary (Variables|HUD|GetMosquitoHUD) "NewEnumerator1")
    (Variables|Gun|SetActive%20Weapon%20Slot "NewEnumerator1")
    (if (Variables|/Game/PlanetSide_2/Weapons/BP_Weapon_Base.BP_Weapon_Base_C|GetIsFiring _weapon_base)
      (Default|StopFiring _weapon_base))))

(event Input|KeyboardEvents|E
  (params (Key :type Key%20Structure :default "AnyKey"))
  ;[1 1 1] Exit Vehicle
  (:Pressed
    (CallFunction|ExitVehicle (Variables|Default|GetPlayer) (Variables|Default|GetSpawn%20Location))))

(fn ConstructionScript
  (Utilities|FlowControl|Sequence
    (:then_0
      (switch Utilities|FlowControl|Switch|SwitchonEMosquitoSlotUtility (Variables|Vehicle|GetUtility%20Item)
        (:NewEnumerator0
          (bind _returnvalue (AddComponent|AddStaticMeshComponent true))
          (bind _output_get (Variables|Vehicle|SetUtility%20Mesh%20Component _returnvalue))
          (Class|SceneComponent|Attachto _output_get (Variables|Default|GetVehicle) "Flare Launcher" "SnapToTarget" true))))
    (:then_1
      (if (Variables|Cosmetics|GetHasFins)
        (bind _returnvalue_2 (AddComponent|AddStaticMeshComponent true))
        (bind _output_get_2 (Variables|Cosmetics|SetFin%20Mesh%20Component _returnvalue_2))
        (Components|StaticMesh|SetStaticMesh _output_get_2 (Variables|Cosmetics|GetFin%20Mesh))
        (Class|SceneComponent|Attachto _output_get_2 (Variables|Default|GetVehicle) "Attachments" "SnapToTarget" true)))
    (:then_2
      (Rendering|Material|SetMaterial (Variables|Cosmetics|GetGlass) 0 (Variables|Cosmetics|GetGlass%20Material)))
    (:then_3
      (bind _returnvalue_3 (AddComponent|AddChildActorComponent false))
      (bind _output_get_3 (Variables|Vehicle|SetWeapon%20Component _returnvalue_3))
      (Class|SceneComponent|Attachto _output_get_3 (Variables|Default|GetVehicle) "Primary Weapon" "SnapToTarget" true)
      (ChildActorComponent|SetChildActorClass _output_get_3 0))))

(fn Movement
  (params (Mesh :type Primitive%20Component%20Object%20Reference) (Delta%20Seconds :type Float%20%28single-precision%29) (Forward%20Speed :type Float%20%28single-precision%29) (Ascend%20Speed :type Float%20%28single-precision%29) (Pitch%20Rate :type Float%20%28single-precision%29) (Yaw%20Rate :type Float%20%28single-precision%29) (Roll%20Rate :type Float%20%28single-precision%29))
  (Physics|SetPhysicsLinearVelocity Mesh (* (* (Math|Vector|GetForwardVector (Transformation|GetActorRotation)) (* (Input|AxisValues|GetMoveForward) Forward%20Speed)) Delta%20Seconds) true "None")
  (Physics|SetPhysicsLinearVelocity Mesh (* (* (Math|Vector|GetUpVector (Transformation|GetActorRotation)) (* (Input|AxisValues|GetMoveUp) Ascend%20Speed)) Delta%20Seconds) true "None")
  (Transformation|AddActorLocalRotation (Math|Rotator|MakeRotator 0.0 (* (Input|AxisValues|GetPitch) Pitch%20Rate) 0.0) false false)
  (Transformation|AddActorLocalRotation (Math|Rotator|MakeRotator 0.0 0.0 (* (Input|AxisValues|GetYaw/moveRight) Yaw%20Rate)) false false)
  (Transformation|AddActorLocalRotation (Math|Rotator|MakeRotator (* (Input|AxisValues|GetRoll/turn) Roll%20Rate) 0.0 0.0) false false))