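; Base aircraft vehicle for a PlanetSide 2 project, providing flight, hover and afterburner functions with no active event logic of its own.
; Movement adds physics velocity along right (used as forward) and up vectors, plus local rotation from input.
; A speed threshold selects flight or hover, switching engine audio and trails.
; Afterburner thrusts forward in flight or upward in hover, draining regenerable fuel reported to a UI widget.
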(event EventBeginPlay)

(event Collision|EventActorBeginOverlap
  (params (OtherActor :type Actor%20Object%20Reference)))

(event EventTick
  (params (DeltaSeconds :type Float%20%28single-precision%29)))

(fn ConstructionScript)

(fn MovementAircraft
  (params (Delta%20Seconds :type Float%20%28single-precision%29) (Forward%20Speed :type Float%20%28single-precision%29) (Ascend%20Speed :type Float%20%28single-precision%29) (Pitch%20Rate :type Float%20%28single-precision%29) (Yaw%20Rate :type Float%20%28single-precision%29) (Roll%20Rate :type Float%20%28single-precision%29))
  (bind _vehicle (Variables|Default|GetVehicle))
  (Physics|SetPhysicsLinearVelocity _vehicle (* (* (Math|Vector|GetRightVector (Transformation|GetActorRotation)) (* (Input|AxisValues|GetMoveForward) Forward%20Speed)) Delta%20Seconds) true "None")
  (Physics|SetPhysicsLinearVelocity _vehicle (* (* (Math|Vector|GetUpVector (Transformation|GetActorRotation)) (* (Input|AxisValues|GetMoveUp) Ascend%20Speed)) Delta%20Seconds) true "None")
  (Transformation|AddLocalRotation (Variables|Default|GetVehicle) (Class|KismetMathLibrary|MakeRot (* (Input|AxisValues|GetRoll/turn) Roll%20Rate) (* (Input|AxisValues|GetYaw/moveRight) Yaw%20Rate) (* (Input|AxisValues|GetPitch) Pitch%20Rate)) false))

(fn CalculateFlightSpeed&SetHoverMode
  (params (Hover%20Speed :type Float%20%28single-precision%29) (Engine%20Audio :type Audio%20Component%20Object%20Reference) (Trail%20Component :type Array%20of%20Scene%20Component%20Object%20References))
  (bind _returnvalue (Physics|GetPhysicsLinearVelocity (Variables|Default|GetVehicle) "None"))
  (bind _output_get (Variables|Aircraft|SetIsInFlightMode (>= (* (Math|Vector|VectorLength (Math|Vector|MakeVector (Math|Float|Max(Float) (.X (Math|Vector|BreakVector (* _returnvalue (Math|Vector|GetRightVector (Transformation|GetActorRotation))))) 0.0) (Math|Float|Max(Float) (.Y (Math|Vector|BreakVector (* _returnvalue (Math|Vector|GetRightVector (Transformation|GetActorRotation))))) 0.0) (Math|Float|Max(Float) (.Z (Math|Vector|BreakVector (* _returnvalue (Math|Vector|GetRightVector (Transformation|GetActorRotation))))) 0.0))) 0.036) Hover%20Speed)))
  (if _output_get
    (Effects|Components|ParticleSystem|SetIntParameter Engine%20Audio "Low / High / Boost" 1)
    (for _array_element Trail%20Component
      (Rendering|SetVisibility _array_element true true))
    (else
      (Effects|Components|ParticleSystem|SetIntParameter Engine%20Audio "Low / High / Boost" 0)
      (for _array_element_2 Trail%20Component
        (Rendering|SetVisibility _array_element_2 false true))))
  (return (Camera|GetCameraRotation (Game|GetPlayerCameraManager 0)) (Math|Float|Floor (* (Math|Vector|VectorLength (Math|Vector|MakeVector (Math|Float|Max(Float) (.X (Math|Vector|BreakVector (* _returnvalue (Math|Vector|GetRightVector (Transformation|GetActorRotation))))) 0.0) (Math|Float|Max(Float) (.Y (Math|Vector|BreakVector (* _returnvalue (Math|Vector|GetRightVector (Transformation|GetActorRotation))))) 0.0) (Math|Float|Max(Float) (.Z (Math|Vector|BreakVector (* _returnvalue (Math|Vector|GetRightVector (Transformation|GetActorRotation))))) 0.0))) 0.036))))

(fn Afterburneron
  (params (Actor :type Actor%20Object%20Reference) (Engine%20Audio%20Component :type Audio%20Component%20Object%20Reference) (Afterburner%20Fuel%20Drain :type Float%20%28single-precision%29) (Afterburner%20Max%20Fuel :type Float%20%28single-precision%29) (Afterburner%20Minimum%20Fuel :type Float%20%28single-precision%29) (Afterburner%20Max%20Speed :type Float%20%28single-precision%29) (Afterburner%20UI%20Panel :type Widget%20Component%20Object%20Reference))
  (bind _returnvalue (Transformation|GetActorRotation Actor))
  (bind _vehicle (Variables|Default|GetVehicle))
  (Effects|Components|ParticleSystem|SetIntParameter Engine%20Audio%20Component "Low / High / Boost" 2)
  (if (Variables|Aircraft|GetIsInFlightMode)
    (Class|PrimitiveComponent|SetAllPhysicsLinearVelocity _vehicle (* (Math|Vector|GetRightVector _returnvalue) (Variables|Afterburner|GetAfterburner%20Speed)) true)
    (else
      (Class|PrimitiveComponent|SetAllPhysicsLinearVelocity _vehicle (* (Math|Vector|GetUpVector _returnvalue) (Variables|Afterburner|GetAfterburner%20Speed)) true)))
  (bind _output_get (Variables|Afterburner|SetAfterburner%20Fuel (Math|Float|Clamp(Float) (- (Variables|Afterburner|GetAfterburner%20Fuel) Afterburner%20Fuel%20Drain) 0.0 Afterburner%20Max%20Fuel)))
  (if (<= _output_get Afterburner%20Minimum%20Fuel)
    (Variables|Afterburner|SetAfterburner%20Speed 0.0)
    (else
      (Variables|Afterburner|SetAfterburner%20Speed Afterburner%20Max%20Speed)))
  (Class|AircraftInterface|RemainingFuel(Message) (UserInterface|GetUserWidgetObject Afterburner%20UI%20Panel) (Variables|Afterburner|GetAfterburner%20Fuel) Afterburner%20Max%20Fuel))

(fn AfterburnerOff
  (params (Afterburner%20Max%20Fuel :type Float%20%28single-precision%29) (Fuel%20Regeneration%20Speed :type Float%20%28single-precision%29) (Afterburner%20UI%20Panel :type Widget%20Component%20Object%20Reference))
  (bind _output_get (Variables|Afterburner|SetAfterburner%20Fuel (Math|Float|Clamp(Float) (+ (Variables|Afterburner|GetAfterburner%20Fuel) Fuel%20Regeneration%20Speed) 0.0 Afterburner%20Max%20Fuel)))
  (Class|AircraftInterface|RemainingFuel(Message) (UserInterface|GetUserWidgetObject Afterburner%20UI%20Panel) _output_get Afterburner%20Max%20Fuel))