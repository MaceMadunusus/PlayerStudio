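; Base weapon actor that handles automatic fire, ammo and reloading, with mesh, sound, muzzle flash and fire delay set in the construction script.
; Fire runs a Gate and RetriggerableDelay loop, spawning BP_Projectile at the Muzzle socket with damage falloff parameters and updating the ammo panel widget.
; An empty magazine triggers a timed reload that resumes fire if still firing.
; An overlap sphere, kept only for ManualFiring, toggles player input.
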(event OnComponentBeginOverlap(Sphere)
  (params (OverlappedComponent :type Primitive%20Component%20Object%20Reference) (OtherActor :type Actor%20Object%20Reference) (OtherComp :type Primitive%20Component%20Object%20Reference) (OtherBodyIndex :type Integer) (bFromSweep :type Boolean) (SweepResult :type Hit%20Result%20Structure%20%28by%20ref%29))
  (Input|EnableInput (Game|GetPlayerController 0)))

(event OnComponentEndOverlap(Sphere)
  (params (OverlappedComponent :type Primitive%20Component%20Object%20Reference) (OtherActor :type Actor%20Object%20Reference) (OtherComp :type Primitive%20Component%20Object%20Reference) (OtherBodyIndex :type Integer))
  (Input|DisableInput (Game|GetPlayerController 0)))

(event Custom|Stop%20Firing
  (bind _weapon_audio (Variables|Default|GetWeapon%20Audio))
  ;[1 1 1] Fire Weapon
  (Variables|Internal|SetIsFiring false)
  (if (not (Variables|Internal|GetIsReloading))
    (Audio|Components|Audio|Stop _weapon_audio)
    (Audio|SpawnSoundAttached (Variables|Default|GetFire%20Stop%20Sound) _weapon_audio "None" "0, 0, 0" "0, 0, 0" "KeepRelativeOffset" false 1.0 1.0 0.0 0 0)
    (Utilities|FlowControl|Gate true) ; enters at Close
  ))

(event Custom|Fire
  ;[1 1 1] Fire Weapon
  (Variables|Internal|SetIsFiring true)
  (if (not (Variables|Internal|GetIsReloading))
    (Audio|Components|Audio|Play (Variables|Default|GetWeapon%20Audio) 0.0)
    (Utilities|FlowControl|Sequence
      (:then_0
        (goto _label Open))
      (:then_1
        (Utilities|FlowControl|Gate true :!label _label
          (:Exit
            (Utilities|FlowControl|Sequence
              (:then_0
                (Utilities|FlowControl|RetriggerableDelay (Variables|Internal|GetFire%20Delay))
                (goto _label))
              (:then_1
                (if (> (Variables|Stats|GetRounds) 0)
                  (Game|SpawnActorfromClass "/Game/PlanetSide_2/Weapons/BP_Projectile.BP_Projectile_C" (Transformation|GetSocketTransform (Variables|Default|GetWeapon) "Muzzle" "RTS_World") "AdjustIfPossibleButDontSpawnIfColliding" 0 (Variables|Stats|GetMax%20Damage) (Variables|Stats|GetMax%20Damage%20Range) (Variables|Stats|GetMin%20Damage) (Variables|Stats|GetMin%20Damage%20Range) 0 self (Variables|Stats|GetMuzzle%20Velocity) (Game|GetPlayerCharacter 0)) ; Spawn projectile
                  (bind _output_get (Variables|Stats|SetRounds (- (Variables|Stats|GetRounds) 1)))
                  (Class|BPIAircraftInterface|SetWeaponAmmo(Message) (UserInterface|GetUserWidgetObject (Variables|Internal|GetPanel%20Widget)) _output_get (Variables|Stats|GetAmmo%20Pool) (Variables|Default|GetWeapon%20Slot))
                  (else
                    (CallFunction|StopFiring)
                    (Variables|Internal|SetIsFiring true)
                    (CallFunction|Reload)))))))))))

(event Custom|Reload
  (bind _magazine_size (Variables|Stats|GetMagazine%20Size))
  ;[1 1 1] Reload Weapon
  (Variables|Internal|SetIsReloading true)
  (if (and (== (Variables|Stats|GetRounds) 0) (> (Variables|Stats|GetAmmo%20Pool) 0))
    (Utilities|FlowControl|Delay (Variables|Stats|GetLong%20Reload%20Time))
    (else
      (Utilities|FlowControl|Delay (Variables|Stats|GetShort%20Reload%20Time))))
  (bind _output_get (Variables|Stats|SetRounds _magazine_size))
  (bind _output_get_2 (Variables|Stats|SetAmmo%20Pool (- (Variables|Stats|GetAmmo%20Pool) _magazine_size)))
  (Class|BPIAircraftInterface|SetWeaponAmmo(Message) (UserInterface|GetUserWidgetObject (Variables|Internal|GetPanel%20Widget)) _output_get _output_get_2 (Variables|Default|GetWeapon%20Slot))
  (Variables|Internal|SetIsReloading false)
  (if (Variables|Internal|GetIsFiring)
    (CallFunction|Fire)))

(fn ConstructionScript
  (bind _weapon (Variables|Default|GetWeapon))
  (bind _weapon_audio (Variables|Default|GetWeapon%20Audio))
  (bind _muzzle_flash (Variables|Default|GetMuzzle%20Flash))
  (Variables|Internal|SetFire%20Delay (/ 1.0 (/ (Math|Conversions|ToFloat(Integer) (Variables|Stats|GetFire%20Rate)) 6e+01)))
  (Components|StaticMesh|SetStaticMesh _weapon (Variables|Default|GetWeapon%20Mesh))
  (Audio|Components|Audio|SetSound _weapon_audio (Variables|Default|GetFire%20Sound))
  (Class|SceneComponent|Attachto _weapon_audio _weapon "Muzzle" "SnapToTarget" true)
  (Effects|Components|ParticleSystem|SetTemplate _muzzle_flash (Variables|Default|GetMuzzle%20Flash%20FX))
  (Class|SceneComponent|Attachto _muzzle_flash (Variables|Default|GetWeapon) "Muzzle" "SnapToTarget" true)
  (if (not (Variables|Default|GetManual%20Firing))
    (Components|DestroyComponent (Variables|Default|GetSphere))))