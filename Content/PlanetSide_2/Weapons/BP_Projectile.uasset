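; Projectile Blueprint for weapon fire with distance-based damage falloff, setting its speed from MuzzleVelocity on BeginPlay.
; Tick holds MaxDamage up to MaxDamageRange, then applies a trig-derived linear slope, without offsetting distance by MaxDamageRange, until locking MinDamage beyond MinDamageRange.
; Hit calls ApplyDamage with the current Damage but no damaged actor wired, then destroys the projectile.
; An impact spark emitter is present but never runs.
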(event EventBeginPlay
  (bind _projectilemovement (Variables|Default|GetProjectileMovement))
  (bind _output_get (Variables|/Script/Engine.ProjectileMovementComponent|SetInitialSpeed _projectilemovement (* (Variables|Default|GetMuzzle%20Velocity) 1e+02)))
  (Variables|/Script/Engine.ProjectileMovementComponent|SetMaxSpeed _projectilemovement _output_get))

(event Collision|EventActorBeginOverlap
  (params (OtherActor :type Actor%20Object%20Reference)))

(event EventTick
  (params (DeltaSeconds :type Float%20%28single-precision%29))
  (bind _min_damage_range (Variables|Default|GetMin%20Damage%20Range))
  (bind _max_damage_range (Variables|Default|GetMax%20Damage%20Range))
  (bind _fired_from (Variables|Default|GetFired%20From))
  (bind _bullet (Variables|Default|GetBullet))
  (bind _returnvalue (- _min_damage_range _max_damage_range))
  (bind _returnvalue_2 (Transformation|GetWorldLocation _bullet))
  (bind _returnvalue_3 (- _returnvalue_2 _fired_from))
  (bind _returnvalue_4 (Math|Vector|VectorLength _returnvalue_3))
  (if (not (Variables|Default|GetExceeded%20Falloff%20Distance))
    (Math|Float|CompareFloat _returnvalue_4 (Variables|Default|GetMax%20Damage%20Range)
      (:>
        (Math|Float|CompareFloat _returnvalue_4 (Variables|Default|GetMin%20Damage%20Range)
          (:>
            (Variables|Default|SetDamage (Variables|Default|GetMin%20Damage) :!label _label)
            (Variables|Default|SetExceeded%20Falloff%20Distance true))
          (:==
            (goto _label))
          (:<
            (Variables|Default|SetDamage (+ (* (Math|Trig|Tan(Degrees) (Class|KismetMathLibrary|DegAtan2 (- (Variables|Default|GetMax%20Damage) (Variables|Default|GetMin%20Damage)) _returnvalue)) (- _returnvalue _returnvalue_4)) (Variables|Default|GetMin%20Damage))))))
      (:==
        (Variables|Default|SetDamage (Variables|Default|GetMax%20Damage) :!label _label_2))
      (:<
        (goto _label_2)))))

(event Collision|EventHit
  (params (MyComp :type Primitive%20Component%20Object%20Reference) (Other :type Actor%20Object%20Reference) (OtherComp :type Primitive%20Component%20Object%20Reference) (bSelfMoved :type Boolean) (HitLocation :type Vector) (HitNormal :type Vector :default "0, 0, 0") (NormalImpulse :type Vector :default "0, 0, 0") (Hit :type Hit%20Result%20Structure%20%28by%20ref%29))
  (Game|Damage|ApplyDamage 0 (Variables|Default|GetDamage) 0 (Variables|Default|GetSource) (Variables|Default|GetDamage%20Type))
  (Actor|DestroyActor))

(fn ConstructionScript)